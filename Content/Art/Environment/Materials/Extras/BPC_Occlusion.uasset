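; Actor component that makes its owner's static mesh see-through, apparently for occlusion, through TransparentStart and TransparentEnd.
; Start caches dynamic instances of FadeMaterial and swaps them onto the mesh, enabling Tick.
; Tick advances a constant-speed fade, easing Opacity toward Transparency, then disables itself when finished.
; As wired, the fade always targets 1, so TransparentEnd never reaches the branch restoring the materials saved at BeginPlay.
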(event EventTick
  (params (DeltaSeconds :type Float%20%28single-precision%29))
  (bind _fadein_outamount (CallFunction|TpinorOut))
  (Variables|Default|SetFadeIn/OutAmount (.FadeIn/OutAmount (CallFunction|TpinorOut)))
  (for _array_element (Variables|Default|GetFadeMaterialPerMesh)
    (Rendering|Material|SetScalarParameterValue _array_element "Opacity" (Class|KismetMathLibrary|FInterpEaseinOut 0.0 (Variables|Default|GetTransparency) (.FadeIn/OutAmount (CallFunction|TpinorOut)) 2.0) :!class /Script/Engine.MaterialInstanceDynamic))
  (if true
    (if (>= _fadein_outamount 1.0)
      (Components|Tick|SetComponentTickEnabled false))
    (elif (<= _fadein_outamount 0.0)
      (Components|Tick|SetComponentTickEnabled false)
      (CallFunction|ResetMeshMaterial))))

(event EventBeginPlay
  (Variables|Default|SetStaticMesh (Actor|GetComponentbyClass (Components|GetOwner) "/Script/Engine.StaticMeshComponent"))
  (bind _staticmesh (Variables|Default|GetStaticMesh)
    (:then
      (Variables|Default|SetStaticMeshMaterial (Rendering|Material|GetMaterials _staticmesh)))
    (:else)))

(fn ReplaceMeshbyTpMaterials
  (params (CurrentMesh :type Primitive%20Component%20Object%20Reference) (CurrentTpMaterials :type Array%20of%20Material%20Instance%20Object%20References))
  (for (_array_element _array_index) CurrentTpMaterials
    (Rendering|Material|SetMaterial CurrentMesh _array_index _array_element))
  (Variables|Default|SetIsMeshSemiTP? true)
  (Components|Tick|SetComponentTickEnabled true))

(fn ResetMeshMaterial
  (bind _staticmeshmaterial (Variables|Default|GetStaticMeshMaterial))
  (Utilities|IsStaticMeshVaild? (Variables|Default|GetStaticMesh) _staticmeshmaterial
    (:True
      (for (_array_element _array_index) _staticmeshmaterial
        (Rendering|Material|SetMaterial (Variables|Default|GetStaticMesh) _array_index _array_element)))))

(fn TransparentStart
  (bind _staticmesh (Variables|Default|GetStaticMesh))
  (bind _fadematerialpermesh (Variables|Default|GetFadeMaterialPerMesh))
  (Utilities|IsStaticMeshVaild? _staticmesh (Variables|Default|GetFadeMaterial)
    (:True
      (if (> (Utilities|Array|Length _fadematerialpermesh) 0)
        (CallFunction|ReplaceMeshbyTpMaterials _staticmesh _fadematerialpermesh)
        (else
          (for _array_element (Variables|Default|GetFadeMaterial)
            (bind _returnvalue (Rendering|Material|CreateDynamicMaterialInstance _array_element "None" "None" :!class /Script/Engine.KismetMaterialLibrary))
            (Utilities|Array|Add (Variables|Default|GetFadeMaterialPerMesh) _returnvalue))
          (CallFunction|ReplaceMeshbyTpMaterials _staticmesh _fadematerialpermesh))))))

(fn TpinorOut
  (LocalVariables|SetFadeTarget 1.0)
  (return (Math|Interpolation|FInterptoConstant (Variables|Default|GetFadeIn/OutAmount) (LocalVariables|GetFadeTarget) (Utilities|Time|GetWorldDeltaSeconds) (Variables|Default|GetFadeSpeed)) false))

(fn TransparentEnd
  (Utilities|IsStaticMeshVaild? (Variables|Default|GetStaticMesh) (Variables|Default|GetStaticMeshMaterial)
    (:True
      (if (> (Utilities|Array|Length (Variables|Default|GetFadeMaterialPerMesh)) 0)
        (Variables|Default|SetIsMeshSemiTP? false)
        (Components|Tick|SetComponentTickEnabled true)))))