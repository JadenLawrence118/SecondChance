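; Character component that, on trigger, soft-locks onto a nearby pawn and snaps the owner toward it.
; It tries a primary target mode, then a secondary, using area or facing-direction sphere traces to pick the nearest eligible BPI_Softlock actor.
; MoveComponentTo turns the capsule's yaw and optionally closes distance, respecting move, height and per-target spacing limits.
; The target is notified, an event reports the lock, and settings are swappable at runtime.
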(event Custom|CE_TriggerSoftlock
  (if (General|IsSoftlockAllowed?) ; Check if the softlock is allowed
    ;[1 1 1] Handles Primary Target Type
    (bind (_foundtarget_ _softlock_selectedactor) (FindTarget|ChooseTargetbyCurrentTargetType (Variables|Options|General|GetPrimaryTargetType))) ; Choose the softlock target based of the\n"PrimaryTargetType" (enum)
    (if _foundtarget_ ; Check if trace can find a target
      (Utilities|IsValid _softlock_selectedactor ; check if target is valid
        (:Is%20Valid
          (Class|BPISoftlock|BIonSelectedTarget(Message) _softlock_selectedactor) ; Sends a message to the selected\ntarget
          (Variables|CameraRotation|SetCamera_ConditionMet? true)
          (Components|MoveComponentTo (Variables|/Script/Engine.Character|GetCapsuleComponent (Variables|Privat|GetCharacterReference)) (Handling|GetMovetoLocation _softlock_selectedactor (Variables|Options|Movement|GetMaxMoveDistance)) (Handling|GetMovetoRotation _softlock_selectedactor) false false 0.2 true) ; rotates / moves the owner to the softlock target
          (Default|CallOnSoftlockTargetFound _softlock_selectedactor true false))
        (:Is%20Not%20Valid
          ;[1 1 1] Handels Secondary Target Type
          (bind (_foundtarget__2 _softlock_selectedactor_2) (FindTarget|ChooseTargetbyCurrentTargetType (Variables|Options|General|GetSecondaryTargetType) :!label _label)) ; Choose the softlock target based of the\n"SecondaryTargetType" (enum)
          (if _foundtarget__2
            (Utilities|IsValid _softlock_selectedactor_2 ; check if target is valid
              (:Is%20Valid
                (Class|BPISoftlock|BIonSelectedTarget(Message) _softlock_selectedactor_2) ; Sends a message to the selected\ntarget
                (Variables|CameraRotation|SetCamera_ConditionMet? true)
                (Components|MoveComponentTo (Variables|/Script/Engine.Character|GetCapsuleComponent (Variables|Privat|GetCharacterReference)) (Handling|GetMovetoLocation _softlock_selectedactor_2 (Variables|Options|Movement|GetMaxMoveDistance)) (Handling|GetMovetoRotation _softlock_selectedactor_2) false false 0.2 true) ; rotates / moves the owner to the softlock target
                (Default|CallOnSoftlockTargetFound _softlock_selectedactor_2 false true))))))
      (else
        (goto _label)))))

(event EventBeginPlay
  ;[1 1 1] Create character reference from owner
  (bind _ascharacter (Utilities|Casting|CastToCharacter (Components|GetOwner))) ; Cast to owner character
  (Variables|Privat|SetCharacterReference _ascharacter) ; Store reference into a variable
  ;[1 1 1] Setup Timer Tick
  (Utilities|Time|SetTimerbyFunctionName 0 "CE_UpdateTick" 0.01 true) ; Set a looping timer, to avoid the default tick usage \n(performance)
)

(fn FindSoftlockTargetArea
  (bind _returnvalue (Components|GetOwner))
  (bind _l_possibletargets (LocalVariables|GetL_PossibleTargets))
  (bind _nearesttarget (FindTarget|GetNearestTarget _l_possibletargets))
  (bind _returnvalue_2 (Transformation|GetActorLocation _returnvalue))
  ;[1 1 1] Sphere Enemy Check // Search for nearest Target in Range
  (bind (_outhits _returnvalue_3) (Collision|MultiSphereTraceForObjects _returnvalue_2 _returnvalue_2 (Variables|Options|TargetTypeSettings|Area|GetArea_TraceDistance) (Utilities|Array|MakeArray "ObjectTypeQuery3") false (Utilities|Array|MakeArray (Components|GetOwner)) "None")) ; Create a sphere tracer to find targets in range
  (if _returnvalue_3
    (bind _array_element (Utilities|Array|ForEachLoopwithBreak _outhits)
      (:LoopBody
        (bind _bi_canbetarget_ (Class|BPISoftlock|BICanbeTarget?(Message) (.HitActor (Collision|BreakHitResult _array_element))))
        (if (and _bi_canbetarget_ (Utilities|DoesObjectImplementInterface (.HitActor (Collision|BreakHitResult _array_element)) "/Game/SoftLock/Blueprints/Component/BPI_Softlock.BPI_Softlock_C")) ; Check if the hitted actor has\nthe softlock interface and the\ncanBeTarget function is true
          (Utilities|Array|Add (LocalVariables|GetL_PossibleTargets) (.HitActor (Collision|BreakHitResult _array_element)))))
      (:Completed
        (Utilities|IsValid _nearesttarget
          (:Is%20Valid
            (bind _output_get (Variables|Privat|SetSoftLock_SelectedActor _nearesttarget)) ; Set the current softlock actor
            (return true _output_get))
          (:Is%20Not%20Valid
            (return false 0)))))
    (else
      (return false 0))))

(fn FindSoftlockTargetActorLookDir
  (bind _returnvalue (Components|GetOwner))
  (bind _l_possibletargets (LocalVariables|GetL_PossibleTargets))
  (bind _nearesttarget (FindTarget|GetNearestTarget _l_possibletargets))
  (bind _returnvalue_2 (Transformation|GetActorRotation _returnvalue))
  (bind _returnvalue_3 (Transformation|GetActorLocation _returnvalue))
  (bind _returnvalue_4 (Math|Vector|GetForwardVector _returnvalue_2))
  ;[1 1 1] Owner Looking Direction Target Check // Search for nearest Target in the Owners Looking Direction
  (bind (_outhits _returnvalue_5) (Collision|MultiSphereTraceForObjects (+ _returnvalue_3 (* _returnvalue_4 1e+02)) (+ _returnvalue_3 (* _returnvalue_4 (Variables|Options|TargetTypeSettings|ActorLookingDirection|GetActorLookDir_TraceDistance))) (Variables|Options|TargetTypeSettings|ActorLookingDirection|GetActorLookDir_SphereRadius) (Utilities|Array|MakeArray "ObjectTypeQuery3") false (Utilities|Array|MakeArray (Components|GetOwner)) "None")) ; Create a Sphere Trace in looking direction\nof the owner
  (if _returnvalue_5
    (bind _array_element (Utilities|Array|ForEachLoopwithBreak _outhits)
      (:LoopBody
        (bind _bi_canbetarget_ (Class|BPISoftlock|BICanbeTarget?(Message) (.HitActor (Collision|BreakHitResult _array_element))))
        (if (and _bi_canbetarget_ (Utilities|DoesObjectImplementInterface (.HitActor (Collision|BreakHitResult _array_element)) "/Game/SoftLock/Blueprints/Component/BPI_Softlock.BPI_Softlock_C")) ; Check if the hit actor has\nthe softlock interface and the\ncanBeTarget function is true
          (Utilities|Array|Add (LocalVariables|GetL_PossibleTargets) (.HitActor (Collision|BreakHitResult _array_element)))))
      (:Completed
        (Utilities|IsValid _nearesttarget
          (:Is%20Valid
            (bind _output_get (Variables|Privat|SetSoftLock_SelectedActor _nearesttarget)) ; Set the current softlock actor
            (return true _output_get))
          (:Is%20Not%20Valid
            (return false 0)))))
    (else
      (return false 0))))

(fn GetNearestTarget
  (params (Array :type Array%20of%20Actor%20Object%20References))
  (for _array_element Array ; Loops all targets and search for the \nclosest one
    (if (or (< (Transformation|GetDistanceTo (Components|GetOwner) _array_element) (LocalVariables|GetL_NearestDistance)) (== (LocalVariables|GetL_NearestDistance) 0.0)) ; if the current array element actor\nis closer to the owner, than the \nnearest target before, than true
      (LocalVariables|SetL_NearestDistance (Transformation|GetDistanceTo (Components|GetOwner) _array_element)) ; Set new nearest distance
      (LocalVariables|SetL_NearestTarget _array_element) ; Set nearest Target
    ))
  (return (LocalVariables|GetL_NearestTarget) (LocalVariables|GetL_NearestDistance)) ; After the loop the nearest target\nand the nearest distance will be\nstored in the output
)

(fn IsSoftlockAllowed?
  (return (Variables|Privat|GetAllowSoftLock?)))

(fn ChooseTargetbyCurrentTargetType
  (params (TargetType :type E_SoftlockTargetTypes%20Enum :default "NewEnumerator0"))
  (switch Utilities|FlowControl|Switch|SwitchonE_SoftlockTargetTypes TargetType ; Switch on the current target type
    (:NewEnumerator6
      (return false 0))
    (:NewEnumerator0
      (bind (_foundtarget_ _softlock_selectedactor) (FindTarget|FindSoftlockTargetArea))
      (return _foundtarget_ _softlock_selectedactor))
    (:NewEnumerator1
      (bind (_foundtarget__2 _softlock_selectedactor_2) (FindTarget|FindSoftlockTargetActorLookDir))
      (return _foundtarget__2 _softlock_selectedactor_2))))

(fn ChangeSoftlockSettings
  (params (Settings :type S%20Softlock%20Main%20Settings%20Structure))
  (bind (_primary_targettype _secondary_targettype _targettype_settings _movement_settings) (Utilities|Struct|BreakS_Softlock_Main_Settings Settings))
  (bind (_area_tracedistance _actorlookdir_tracedistance _actorlookdir_sphereradius) (Utilities|Struct|BreakS_Softlock_TargetType_Settings _targettype_settings))
  (bind (_movestowardtarget_ _maxmovedistance _mintargetdistance _maxheightdifference) (Utilities|Struct|BreakS_Softlock_Movement_Settings _movement_settings))
  (Variables|Options|General|SetPrimaryTargetType _primary_targettype)
  (Variables|Options|General|SetSecondaryTargetType _secondary_targettype)
  (Utilities|FlowControl|Sequence
    (:then_0
      (Variables|Options|TargetTypeSettings|Area|SetArea_TraceDistance _area_tracedistance)
      (Variables|Options|TargetTypeSettings|ActorLookingDirection|SetActorLookDir_TraceDistance _actorlookdir_tracedistance)
      (Variables|Options|TargetTypeSettings|ActorLookingDirection|SetActorLookDir_SphereRadius _actorlookdir_sphereradius))
    (:then_1
      (Variables|Options|Movement|SetMovesTowardTarget? _movestowardtarget_)
      (Variables|Options|Movement|SetMaxMoveDistance _maxmovedistance)
      (Variables|Options|Movement|SetMinTargetDistance _mintargetdistance)
      (Variables|Options|Movement|SetMaxHeightDifference _maxheightdifference))))

(fn GetMovetoLocation
  (params (TargetActor :type Actor%20Object%20Reference) (MaxMoveDistance :type Float%20%28double-precision%29))
  (bind _characterreference (Variables|Privat|GetCharacterReference))
  (bind _returnvalue (Transformation|GetActorLocation _characterreference))
  (return (select (and (Variables|Options|Movement|GetMovesTowardTarget?) (< (Math|Float|Absolute(Float) (- (.z (Transformation|GetActorLocation TargetActor)) (.z (Transformation|GetActorLocation (Variables|Privat|GetCharacterReference))))) (Variables|Options|Movement|GetMaxHeightDifference))) (select (== MaxMoveDistance 0.0) (+ (Transformation|GetActorLocation TargetActor) (* (Math|Vector|GetUnitDirection(Vector) (Transformation|GetActorLocation TargetActor) (Transformation|GetActorLocation (Variables|Privat|GetCharacterReference))) (Handling|GetMinimumTargetDistance TargetActor))) (+ _returnvalue (* (Math|Vector|GetUnitDirection(Vector) (Transformation|GetActorLocation TargetActor) _returnvalue) (* (select (> MaxMoveDistance (Handling|CurrentDistanceBetweenActors TargetActor (Variables|Privat|GetCharacterReference))) (Handling|CurrentDistanceBetweenActors TargetActor (Variables|Privat|GetCharacterReference)) MaxMoveDistance) -1.0)))) (Transformation|GetActorLocation (Variables|Privat|GetCharacterReference)))))

(fn GetMovetoRotation
  (params (Target :type Actor%20Object%20Reference))
  (bind _characterreference (Variables|Privat|GetCharacterReference))
  (bind _returnvalue (Transformation|GetActorRotation _characterreference))
  (return (Math|Rotator|MakeRotator (.roll _returnvalue) (.pitch _returnvalue) (.yaw (Math|Rotator|FindLookatRotation (Transformation|GetActorLocation (Variables|Privat|GetCharacterReference)) (Transformation|GetActorLocation Target))))))

(fn GetMinimumTargetDistance
  (params (Target :type Object%20Object%20Reference))
  (bind (_bi_usecustomdistance_ _bi_newmindistance) (Class|BPISoftlock|BIMinDistance(Message) Target)) ; Trys to get custom minimum distance from the current\ntarget, if false use default MinTargetDistance
  (return (select _bi_usecustomdistance_ _bi_newmindistance (Variables|Options|Movement|GetMinTargetDistance))))

(fn CurrentDistanceBetweenActors
  (params (Target :type Actor%20Object%20Reference) (OtherActor%28Owner%29 :type Actor%20Object%20Reference))
  (return (- (Transformation|GetDistanceTo Target OtherActor%28Owner%29) (Handling|GetMinimumTargetDistance Target))))