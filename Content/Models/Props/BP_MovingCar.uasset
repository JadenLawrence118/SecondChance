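; BP_MovingCar is a looping prop car that drives along the spline of its referenced BP_CarRoute.
; Each run picks a random car mesh, then plays a timeline scaled to CompletionTime.
; InstanceRef selects one of five movement tracks, whose alpha sets the car's distance and rotation along the spline.
; On finish it waits TimeBeforeReplay, reset to 1 if a randomly varied check is non-positive, then runs again.
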(event Custom|Move
  (bind _routeref (Variables|Default|GetRouteRef))
  (bind _timebeforereplayvariation (Variables|Default|GetTimeBeforeReplayVariation))
  (bind _spline (Variables|/Game/Models/Props/BP_CarRoute.BP_CarRoute_C|GetSpline _routeref))
  ;[0.551 0.4543 0.9882] Randomize Car Colour
  (Components|StaticMesh|SetStaticMesh (Variables|Default|GetCar) (.OutItem (Utilities|Array|Random (Variables|Default|GetCarModels))))
  ;[0.968 0.7524 1] Play All Timeline Tracks For Length of CompletionTime
  (Components|Timeline|SetPlayRate (Variables|Default|GetMoveTimeline) (/ 1.0 (Variables|Default|GetCompletionTime)))
  (bind (_direction _movetrack _movetrack2 _movetrack3 _movetrack4 _movetrack5) (Timeline|MoveTimeline PlayFromStart)
    (:Update
      ;[1 0.8539 0.6416] Get Corresponding Movement Track to the Relevant Car
      (bind _output_get (Variables|Default|SetMoveTracks (Utilities|Array|MakeArray _movetrack _movetrack2 _movetrack3 _movetrack4 _movetrack5)))
      ;[0.8477 1 0.6556] Move Car to Desired Position Along Corresponding BP_CarRoute Spline
      (Transformation|SetActorTransform (Math|Transform|MakeTransform (Spline|GetLocationatDistanceAlongSpline _spline (Math|Float|Lerp 0.0 (Spline|GetSplineLength _spline) (Utilities|Array|Get(acopy) _output_get (- (Variables|Default|GetInstanceRef) 1))) "World") (Spline|GetRotationatDistanceAlongSpline _spline (Math|Float|Lerp 0.0 (Spline|GetSplineLength _spline) (Utilities|Array|Get(acopy) _output_get (- (Variables|Default|GetInstanceRef) 1))) "World") "1.000000,1.000000,1.000000")))
    (:Finished
      ;[1 0.6131 0.5932] Replay After TimeBeforeReplay in Seconds (or similar value)
      (if (> (Math|Random|RandomIntegerinRange (- (Variables|Default|GetTimeBeforeReplay) _timebeforereplayvariation) (+ (Variables|Default|GetTimeBeforeReplay) _timebeforereplayvariation)) 0)
        _
        (else
          (Variables|Default|SetTimeBeforeReplay 1)))
      (Utilities|FlowControl|Delay (Math|Conversions|ToFloat(Integer) (Variables|Default|GetTimeBeforeReplay)))
      (CallFunction|Move))))

(event EventBeginPlay
  (CallFunction|Move))

(fn ConstructionScript)