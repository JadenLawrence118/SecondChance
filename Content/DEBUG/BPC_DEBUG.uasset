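; BPC_DEBUG is a component that provides a toggleable debug menu for the local player.
; On BeginPlay it waits one tick, then creates WB_DEBUG for player controller 0 and adds it to the viewport hidden.
; The IA_DebugMenu input flips an open flag that shows or hides the widget, switches between Game-and-UI and Game-only input modes, and toggles the mouse cursor.
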(event Input|EnhancedActionEvents|EnhancedInputActionIA_DebugMenu
  (params (ActionValue :type Vector%202D%20Structure) (ElapsedSeconds :type Float%20%28double-precision%29) (TriggeredSeconds :type Float%20%28double-precision%29) (InputAction :type Input%20Action%20Object%20Reference :default "/Game/DEBUG/IA_DebugMenu.IA_DebugMenu"))
  (bind _returnvalue (Game|GetPlayerController 0))
  ;[0 1 0.0655] DEBUG
  (:Started
    (if (not (Variables|Default|GetIsDebugOpen))
      (Variables|Default|SetIsDebugOpen true)
      (Widget|SetVisibility (Variables|Default|GetDebugMenuWidget) "Visible")
      (Input|SetInputModeGameandUI _returnvalue (Variables|Default|GetDebugMenuWidget) "DoNotLock" true false)
      (Variables|/Script/Engine.PlayerController|SetbShowMouseCursor (Game|GetPlayerController 0) true)
      (else
        (Variables|Default|SetIsDebugOpen false)
        (Widget|SetVisibility (Variables|Default|GetDebugMenuWidget) "Hidden")
        (Input|SetInputModeGameOnly _returnvalue false)
        (Variables|/Script/Engine.PlayerController|SetbShowMouseCursor (Game|GetPlayerController 0) false)))))

(event EventBeginPlay
  (Utilities|FlowControl|DelayUntilNextTick)
  (bind _returnvalue (UserInterface|CreateWidget "/Game/DEBUG/WB_DEBUG.WB_DEBUG_C" (Game|GetPlayerController 0)))
  (bind _output_get (Variables|Default|SetDebugMenuWidget _returnvalue))
  (UserInterface|Viewport|AddtoViewport _output_get 0)
  (Widget|SetVisibility _output_get "Hidden"))