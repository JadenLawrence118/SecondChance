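; Boss enemy component that handles sword hit detection and deals melee damage during an attack.
; StartMeleeTrace runs a looping timer that sphere-traces between the supplied start and end scene objects at the given radius and interval, with debug drawing on.
; A DoOnce limits damage to the first hit actor per trace window.
; StopMeleeTrace clears the timer and resets that gate for the next swing.
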(event Custom|Start%20Melee%20Trace
  (params (Trace%20Start%20Object :type Scene%20Component%20Object%20Reference) (Trace%20End%20Object :type Scene%20Component%20Object%20Reference) (Trace%20Radius :type Float%20%28single-precision%29) (Attack%20Damage :type Float%20%28double-precision%29) (TraceFrequency%28sec%29 :type Float%20%28double-precision%29))
  (bind _returnvalue (Utilities|Time|SetTimerbyEvent (delegate Custom|Melee%20Tarce) TraceFrequency%28sec%29 true))
  (Variables|Default|SetMelee%20Trace%20Loop _returnvalue))

(event Custom|Melee%20Tarce
  (bind (_outhit _returnvalue) (Collision|SphereTraceByChannel (Transformation|GetWorldLocation (stale Custom|Start%20Melee%20Trace Trace%20Start%20Object)) (Transformation|GetWorldLocation (stale Custom|Start%20Melee%20Trace Trace%20End%20Object)) (stale Custom|Start%20Melee%20Trace Trace%20Radius) "TraceTypeQuery4" false 0 "ForDuration"))
  (if _returnvalue
    (Utilities|FlowControl|DoOnce false
      (:Completed
        (Game|Damage|ApplyDamage (.HitActor (Collision|BreakHitResult _outhit)) (stale Custom|Start%20Melee%20Trace Attack%20Damage) 0 0)))))

(event Custom|StopMeleeTrace
  (Utilities|Time|ClearandInvalidateTimerbyHandle (Variables|Default|GetMelee%20Trace%20Loop))
  (Utilities|FlowControl|DoOnce false) ; enters at Reset
)

(event EventBeginPlay)

(event EventTick
  (params (DeltaSeconds :type Float%20%28single-precision%29)))