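; Final boss fight director that coordinates Orpheus and Orion with the player through a StateTree and bound events.
; Switching to the present halts both bosses; leaving it resumes them, starting the StateTree the first time.
; Half-health events set second-phase and Orpheus AOE flags.
; It also runs Orion's sword-clash QTE, swapping input contexts and using a timer-drained bar, refilled by presses, to pick success or failure montages.
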(event Custom|OnOrionHalfHealth_Event
  (if (not (Variables|Default|GetIsSecondPhase))
    (Variables|Default|SetIsSecondPhase true)))

(event Custom|OnOrpheusHalfHealth_Event
  (Variables|Default|SetCanUseOrpheusAOE true)
  (if (not (Variables|Default|GetIsSecondPhase))
    (Variables|Default|SetIsSecondPhase true)))

(event Custom|OnTimeChange_Event
  (params (InPresent :type Boolean))
  (bind _player_ref (Variables|Default|GetPlayer%20Ref))
  (bind _orion_ref (Variables|Default|GetOrion%20Ref))
  (bind _orpheus_ref (Variables|Default|GetOrpheus%20Ref))
  (if InPresent
    (Default|StopAction _orpheus_ref)
    (Default|Pause _orion_ref)
    (else
      (Utilities|FlowControl|Sequence
        (:then_0
          (Utilities|FlowControl|DoOnce false
            (:Completed
              (AI|Logic|StartLogic (Variables|Default|GetStateTree)))))
        (:then_1
          (Default|ContinueAction _orpheus_ref _player_ref)
          (Default|Continue _orion_ref _player_ref))))))

(event Custom|OnActionEnd_Event
  (Development|PrintString "ACTION END 
"))

(event Custom|QTE%20Start
  (bind _player_ref (Variables|Default|GetPlayer%20Ref))
  (bind _orion_ref (Variables|Default|GetOrion%20Ref))
  (bind _returnvalue (Transformation|GetActorRotation _player_ref))
  (bind _mesh (Variables|/Script/Engine.Character|GetMesh _player_ref))
  (Utilities|FlowControl|Sequence
    (:then_0
      (Utilities|FlowControl|DoOnce false) ; enters at Reset
    )
    (:then_1
      (Variables|/Game/ThirdPerson/Blueprints/BP_ThirdPersonCharacter.BP_ThirdPersonCharacter_C|SetInQTE? _player_ref true)
      (Components|Movement|StopMovementImmediately (Variables|/Script/Engine.Character|GetCharacterMovement _player_ref))
      (bind _asplayer_controller (Utilities|Casting|CastToPlayerController (Pawn|GetController _player_ref)))
      (Utilities|IsValid (PlayerController|LocalPlayerSubsystems|GetEnhancedInputLocalPlayerSubsystem _asplayer_controller)
        (:Is%20Valid
          (Input|RemoveMappingContext (PlayerController|LocalPlayerSubsystems|GetEnhancedInputLocalPlayerSubsystem _asplayer_controller) "/Game/ThirdPerson/Input/IMC_Default.IMC_Default" "(bIgnoreAllPressedKeysUntilRelease=True,bForceImmediately=False,bNotifyUserSettings=False)")
          (Input|AddMappingContext (PlayerController|LocalPlayerSubsystems|GetEnhancedInputLocalPlayerSubsystem _asplayer_controller) "/Game/ThirdPerson/Input/IMC_OrionQTE.IMC_OrionQTE" 0 "(bIgnoreAllPressedKeysUntilRelease=True,bForceImmediately=False,bNotifyUserSettings=False)")
          (Transformation|SetActorRotation _player_ref (Math|Rotator|MakeRotator (.roll _returnvalue) (.pitch _returnvalue) (+ (.yaw (Transformation|GetActorRotation _orion_ref)) 1.8e+02)))
          (Transformation|SetActorLocation _player_ref (Transformation|GetWorldLocation (Variables|/Game/Enemies/Boss/FinalBoss/Orion/BP_Orion.BP_Orion_C|GetQTE%20KaiaPos _orion_ref)) false false)
          (Animation|Montage|PlayMontage _mesh "/Game/Art/Characters/Kaia/Animations/Combo1/AM_SwordCrashQTEStart.AM_SwordCrashQTEStart" 0.2
            (:OnNotifyBegin
              (Animation|Montage|PlayMontage _mesh "/Game/Art/Characters/Kaia/Animations/Combo1/AM_InQTE.AM_InQTE"
                (:then
                  (Utilities|Time|SetTimerbyEvent (delegate Custom|EndQTE) 1e+01)
                  (Animation|Montage|MontageSetPlayRate (Components|SkeletalMesh|GetAnimInstance _mesh) "/Game/Art/Characters/Kaia/Animations/Combo1/AM_SwordCrashQTEStart.AM_SwordCrashQTEStart" 0.0)
                  (Utilities|FlowControl|Delay 1.0)
                  (bind _returnvalue_2 (UserInterface|CreateWidget "/Game/UI/Boss/WB_QTEBar.WB_QTEBar_C"))
                  (UserInterface|Viewport|AddtoViewport _returnvalue_2 0)
                  (Variables|Default|SetQTE%20Bar _returnvalue_2)
                  (bind _returnvalue_3 (Utilities|Time|SetTimerbyEvent (delegate Custom|BarDecrease) 0.05 true))
                  (Variables|Default|SetTimer _returnvalue_3))))))))))

(event Custom|OnQTEPress_Event
  (bind _qtebarmax (Variables|Default|GetQTEBarMax))
  (bind _output_get (Variables|Default|SetQTECurrentVar (Math|Float|Clamp(Float) (+ (Variables|Default|GetQTECurrentVar) 4.0) 0.0 1e+02)))
  (bind _qte_bar (Variables|Default|GetQTE%20Bar)
    (:then
      (Default|SetPercentage _qte_bar (/ _output_get _qtebarmax))
      (if (>= _output_get _qtebarmax)
        (CallFunction|EndQTE)))
    (:else)))

(event Custom|EndQTE
  (Variables|/Game/ThirdPerson/Blueprints/BP_ThirdPersonCharacter.BP_ThirdPersonCharacter_C|SetInQTE? (Variables|Default|GetPlayer%20Ref) false)
  (Utilities|Time|ClearandInvalidateTimerbyHandle (Variables|Default|GetTimer))
  (Widget|SetVisibility (Variables|Default|GetQTE%20Bar) "Hidden")
  (if (<= (Variables|Default|GetQTECurrentVar) (/ (Variables|Default|GetQTEBarMax) 2.0))
    (Animation|Montage|PlayMontage (Variables|/Script/Engine.Character|GetMesh (Variables|Default|GetPlayer%20Ref)) "/Game/Art/Characters/Kaia/Animations/Combo1/AM_QTEFailed.AM_QTEFailed" 0.2
      (:OnCompleted
        _))
    (else
      (Animation|Montage|PlayMontage (Variables|/Script/Engine.Character|GetMesh (Variables|Default|GetPlayer%20Ref)) "/Game/Art/Characters/Kaia/Animations/Combo1/AM_QTESuccess.AM_QTESuccess" 0.5
        (:OnCompleted
          _))))
  (bind _asplayer_controller (Utilities|Casting|CastToPlayerController (Pawn|GetController (Variables|Default|GetPlayer%20Ref))))
  (Utilities|IsValid (PlayerController|LocalPlayerSubsystems|GetEnhancedInputLocalPlayerSubsystem _asplayer_controller)
    (:Is%20Valid
      (Input|RemoveMappingContext (PlayerController|LocalPlayerSubsystems|GetEnhancedInputLocalPlayerSubsystem _asplayer_controller) "/Game/ThirdPerson/Input/IMC_OrionQTE.IMC_OrionQTE" "(bIgnoreAllPressedKeysUntilRelease=True,bForceImmediately=False,bNotifyUserSettings=False)")
      (Input|AddMappingContext (PlayerController|LocalPlayerSubsystems|GetEnhancedInputLocalPlayerSubsystem _asplayer_controller) "/Game/ThirdPerson/Input/IMC_Default.IMC_Default" 0 "(bIgnoreAllPressedKeysUntilRelease=True,bForceImmediately=False,bNotifyUserSettings=False)")
      (Default|FullCharacterReset (Variables|/Game/ThirdPerson/Blueprints/BP_ThirdPersonCharacter.BP_ThirdPersonCharacter_C|GetBPC_AttackSystem (Variables|Default|GetPlayer%20Ref)))
      (Variables|Default|SetQTECurrentVar 5e+01)
      (Utilities|FlowControl|DoOnce false
        (:Completed
          (Default|BlockEnd (Variables|Default|GetOrion%20Ref)))))))

(event Custom|BarDecrease
  (bind _output_get (Variables|Default|SetQTECurrentVar (Math|Float|Clamp(Float) (- (Variables|Default|GetQTECurrentVar) 1.0) 0.0 1e+02)))
  (Default|SetPercentage (Variables|Default|GetQTE%20Bar) (/ _output_get (Variables|Default|GetQTEBarMax)))
  (if (<= _output_get 0.0)
    (CallFunction|EndQTE)))

(event EventBeginPlay
  (Utilities|FlowControl|Sequence
    (:then_0
      (bind _returnvalue (Actor|GetActorOfClass "/Game/Enemies/Boss/FinalBoss/Orpheus/BP_Orpheus.BP_Orpheus_C"))
      (Variables|Default|SetOrpheus%20Ref _returnvalue)
      (EventDispatchers|AssignOnHalfHealth _returnvalue (EventDispatchers|CreateEvent :!event Custom|OnOrpheusHalfHealth_Event)))
    (:then_1
      (bind _returnvalue_2 (Actor|GetActorOfClass "/Game/Enemies/Boss/FinalBoss/Orion/BP_Orion.BP_Orion_C"))
      (bind _output_get (Variables|Default|SetOrion%20Ref _returnvalue_2))
      (EventDispatchers|AssignOnHalfHealth _output_get (EventDispatchers|CreateEvent :!event Custom|OnOrionHalfHealth_Event))
      (EventDispatchers|AssignOnQTE _output_get (EventDispatchers|CreateEvent :!event Custom|QTE%20Start))
      (EventDispatchers|AssignOnActionEnd _output_get (delegate Custom|OnActionEnd_Event)))
    (:then_2
      (bind _returnvalue_3 (Actor|GetActorOfClass "/Game/ThirdPerson/Blueprints/BP_ThirdPersonCharacter.BP_ThirdPersonCharacter_C"))
      (Variables|Default|SetPlayer%20Ref _returnvalue_3)
      (EventDispatchers|AssignOnTimeChange _returnvalue_3 (EventDispatchers|CreateEvent :!event Custom|OnTimeChange_Event))
      (EventDispatchers|AssignOnQTEPress _returnvalue_3 (EventDispatchers|CreateEvent :!event Custom|OnQTEPress_Event)))
    (:then_3
      (Default|Exit (Variables|Default|GetOrpheus%20Ref))
      (Default|Exit (Variables|Default|GetOrion%20Ref)))))

(event Collision|EventActorBeginOverlap
  (params (OtherActor :type Actor%20Object%20Reference)))

(event EventTick
  (params (DeltaSeconds :type Float%20%28single-precision%29)))

(fn ConstructionScript)

(fn AttackNumAdd
  (Math|Integer|IncrementInt (Variables|Default|GetCurrentAttackNum)))