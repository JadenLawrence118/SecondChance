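; BP_MegaElectrocute is a timed area attack in the Orpheus final boss's SafeZone set, with a warning phase followed by a damaging phase.
; Start plays the telegraph child actor for the warning time, then Activate passes Damage to the damage-area child actor and switches it on until Reset deactivates it and fires OnAttackEnd.
; A State enum and single timer handle let Stop and Continue pause and resume whichever phase is running.
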(event Custom|Start
  (params (WarningTime%28sec%29 :type Float%20%28double-precision%29))
  ;[1 1 1] Warning
  (Variables|Default|SetState "NewEnumerator0")
  (Class|BPITelegraph|Start(Message) (Variables|/Script/Engine.ChildActorComponent|GetChildActor (Variables|Default|GetDamageZoneTelegraph)) WarningTime%28sec%29)
  (bind _returnvalue (Utilities|Time|SetTimerbyEvent (delegate Custom|Activate) WarningTime%28sec%29))
  (Variables|Default|SetTimer _returnvalue))

(event Custom|Reset
  (Variables|Default|SetState "NewEnumerator2")
  (Class|BPIBossAreaAttack|Deactivate(Message) (Variables|/Script/Engine.ChildActorComponent|GetChildActor (Variables|Default|GetDamageArea)))
  (Utilities|Time|ClearandInvalidateTimerbyHandle (Variables|Default|GetTimer))
  (Default|CallOnAttackEnd))

(event Custom|Activate
  (bind _damage (Variables|Default|GetDamage))
  (Utilities|Time|ClearandInvalidateTimerbyHandle (Variables|Default|GetTimer))
  (Variables|Default|SetState "NewEnumerator1")
  (Development|PrintString (Utilities|String|ToString(Float) _damage))
  (Class|BPILaser|SetDamage(Message) (Variables|/Script/Engine.ChildActorComponent|GetChildActor (Variables|Default|GetDamageArea)) _damage)
  (Class|BPITelegraph|Reset(Message) (Variables|/Script/Engine.ChildActorComponent|GetChildActor (Variables|Default|GetDamageZoneTelegraph)))
  (Class|BPIBossAreaAttack|Activate(Message) (Variables|/Script/Engine.ChildActorComponent|GetChildActor (Variables|Default|GetDamageArea)))
  (bind _returnvalue (Utilities|Time|SetTimerbyEvent (delegate Custom|Reset) (Variables|Default|GetActivateTime)))
  (Variables|Default|SetTimer _returnvalue))

(event EventBeginPlay
  (Class|BPITelegraph|Reset(Message) (Variables|/Script/Engine.ChildActorComponent|GetChildActor (Variables|Default|GetDamageZoneTelegraph)))
  (Class|BPIBossAreaAttack|Deactivate(Message) (Variables|/Script/Engine.ChildActorComponent|GetChildActor (Variables|Default|GetDamageArea))))

(event Collision|EventActorBeginOverlap
  (params (OtherActor :type Actor%20Object%20Reference)))

(event EventTick
  (params (DeltaSeconds :type Float%20%28single-precision%29)))

(fn ConstructionScript)

(fn Stop
  (switch Utilities|FlowControl|Switch|SwitchonE_ElectrocuteState (Variables|Default|GetState)
    (:NewEnumerator0
      (Class|BPITelegraph|Pause(Message) (Variables|/Script/Engine.ChildActorComponent|GetChildActor (Variables|Default|GetDamageZoneTelegraph))))
    (:NewEnumerator1
      (Class|BPIBossAreaAttack|Pause(Message) (Variables|/Script/Engine.ChildActorComponent|GetChildActor (Variables|Default|GetDamageArea)))))
  (Utilities|Time|PauseTimerbyHandle (Variables|Default|GetTimer)))

(fn Continue
  (switch Utilities|FlowControl|Switch|SwitchonE_ElectrocuteState (Variables|Default|GetState)
    (:NewEnumerator0
      (Class|BPITelegraph|Continue(Message) (Variables|/Script/Engine.ChildActorComponent|GetChildActor (Variables|Default|GetDamageZoneTelegraph))))
    (:NewEnumerator1
      (Class|BPIBossAreaAttack|Continue(Message) (Variables|/Script/Engine.ChildActorComponent|GetChildActor (Variables|Default|GetDamageArea)))))
  (Utilities|Time|UnpauseTimerbyHandle (Variables|Default|GetTimer)))