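; BP_SafeZone is a safe area actor for the Orpheus final boss fight that shields the player from damage.
; It caches the player character on BeginPlay and toggles its Damageable flag when the PlayerHitBox-tagged component begins or ends overlapping the LaserShape.
; The construction script applies a configurable material and scale to LaserShape, and SetVisible shows or hides that shape.
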(event OnComponentBeginOverlap(LaserShape)
  (params (OverlappedComponent :type Primitive%20Component%20Object%20Reference) (OtherActor :type Actor%20Object%20Reference) (OtherComp :type Primitive%20Component%20Object%20Reference) (OtherBodyIndex :type Integer) (bFromSweep :type Boolean) (SweepResult :type Hit%20Result%20Structure%20%28by%20ref%29))
  (if (Components|ComponentHasTag OtherComp "PlayerHitBox")
    (Variables|/Game/ThirdPerson/Blueprints/BP_ThirdPersonCharacter.BP_ThirdPersonCharacter_C|SetDamageable (Variables|Private|GetPlayerRef) false)))

(event OnComponentEndOverlap(LaserShape)
  (params (OverlappedComponent :type Primitive%20Component%20Object%20Reference) (OtherActor :type Actor%20Object%20Reference) (OtherComp :type Primitive%20Component%20Object%20Reference) (OtherBodyIndex :type Integer))
  (if (Components|ComponentHasTag OtherComp "PlayerHitBox")
    (Variables|/Game/ThirdPerson/Blueprints/BP_ThirdPersonCharacter.BP_ThirdPersonCharacter_C|SetDamageable (Variables|Private|GetPlayerRef) true)))

(event EventTick
  (params (DeltaSeconds :type Float%20%28single-precision%29)))

(event EventBeginPlay
  (bind _asbp_third_person_character (Utilities|Casting|CastToBP_ThirdPersonCharacter (Game|GetPlayerCharacter 0)))
  (Variables|Private|SetPlayerRef _asbp_third_person_character))

(fn ConstructionScript
  (bind _lasershape (Variables|Default|GetLaserShape))
  (Rendering|Material|SetMaterial _lasershape 0 (Variables|Customisation|GetMaterial))
  (Transformation|SetRelativeScale3D _lasershape (Variables|Customisation|GetScaleMultiplyer))
  (if (Variables|Customisation|GetIsStatic)
    _))

(fn SetVisible
  (params (Visible :type Boolean))
  (Rendering|SetVisibility (Variables|Default|GetLaserShape) Visible false))