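; Destructible AOE charger for the Orpheus boss safe zone, with a present-time twin mesh placed PresentPastDis below it.
; A reversible timeline raises and lowers the main mesh, firing spawned or hidden events; Stop and Continue pause and resume it.
; Damage, enabled once first fully risen, goes through BPCPlayerStats with a brief invulnerability window after hits.
; At zero health it broadcasts destruction, stops Niagara effects and hides both meshes.
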(event Custom|Spawn
  (bind _returnvalue (Transformation|GetActorLocation))
  (bind _startpos_z (Variables|Default|GetStartPos_Z))
  (Variables|Default|SetIsSpawning true)
  (Components|Activation|Activate (Variables|Default|GetNiagara1) false)
  (bind (_direction _z_pos_alpha) (Timeline|StartEndTimeline PlayFromStart)
    (:Update
      (Transformation|SetWorldLocation (Variables|Default|GetMainCharger) (Math|Vector|MakeVector (.x _returnvalue) (.y _returnvalue) (Math|Float|Lerp _startpos_z (+ _startpos_z 1.7e+02) _z_pos_alpha)) false false))
    (:Finished
      (switch Utilities|FlowControl|Switch|SwitchonETimelineDirection _direction
        (:Forward
          (Default|CallOnSpawned)
          (Variables|/Game/ThirdPerson/Blueprints/BPC_PlayerStats.BPC_PlayerStats_C|SetCanTakeDamage (Variables|Default|GetBPC_PlayerStats) true)
          (Collision|SetCollisionEnabled (Variables|Default|GetMainCharger) "QueryAndProbe"))
        (:Backward
          (Default|CallOnHidden)
          (Collision|SetCollisionEnabled (Variables|Default|GetMainCharger) "NoCollision"))))))

(event Custom|ReturnToGround
  (bind _returnvalue (Transformation|GetActorLocation))
  (bind _startpos_z (Variables|Default|GetStartPos_Z))
  (Variables|Default|SetIsSpawning false)
  (Components|Activation|Deactivate (Variables|Default|GetNiagara1))
  (bind (_direction _z_pos_alpha) (Timeline|StartEndTimeline ReverseFromEnd)
    (:Update
      (Transformation|SetWorldLocation (Variables|Default|GetMainCharger) (Math|Vector|MakeVector (.x _returnvalue) (.y _returnvalue) (Math|Float|Lerp _startpos_z (+ _startpos_z 1.7e+02) _z_pos_alpha)) false false))
    (:Finished
      (switch Utilities|FlowControl|Switch|SwitchonETimelineDirection _direction
        (:Forward
          (Default|CallOnSpawned)
          (Variables|/Game/ThirdPerson/Blueprints/BPC_PlayerStats.BPC_PlayerStats_C|SetCanTakeDamage (Variables|Default|GetBPC_PlayerStats) true)
          (Collision|SetCollisionEnabled (Variables|Default|GetMainCharger) "QueryAndProbe"))
        (:Backward
          (Default|CallOnHidden)
          (Collision|SetCollisionEnabled (Variables|Default|GetMainCharger) "NoCollision"))))))

(event Custom|Destroyed
  (Default|CallOnDestroy)
  (Components|Activation|Deactivate (Variables|Default|GetNiagara1))
  (Rendering|SetVisibility (Variables|Default|GetMainCharger) false false)
  (Collision|SetCollisionEnabled (Variables|Default|GetMainCharger) "NoCollision"))

(event EventBeginPlay
  (bind _returnvalue (Transformation|GetActorLocation))
  (Variables|/Game/ThirdPerson/Blueprints/BPC_PlayerStats.BPC_PlayerStats_C|SetCanTakeDamage (Variables|Default|GetBPC_PlayerStats) false)
  (Variables|Default|SetStartPos_Z (.z _returnvalue))
  (Transformation|SetWorldLocation (Variables|Default|GetPresentCharger) (Math|Vector|MakeVector (.x _returnvalue) (.y _returnvalue) (- (.z _returnvalue) (Variables|Default|GetPresentPastDis))) false false)
  (Collision|SetCollisionEnabled (Variables|Default|GetMainCharger) "NoCollision")
  (Components|Activation|Deactivate (Variables|Default|GetNiagara1)))

(event Collision|EventActorBeginOverlap
  (params (OtherActor :type Actor%20Object%20Reference)))

(event EventTick
  (params (DeltaSeconds :type Float%20%28single-precision%29)))

(event Game|Damage|EventAnyDamage
  (params (Damage :type Float%20%28single-precision%29) (DamageType :type Damage%20Type%20Object%20Reference) (InstigatedBy :type Controller%20Object%20Reference) (DamageCauser :type Actor%20Object%20Reference))
  (bind _bpc_playerstats (Variables|Default|GetBPC_PlayerStats))
  (if (Variables|/Game/ThirdPerson/Blueprints/BPC_PlayerStats.BPC_PlayerStats_C|GetCanTakeDamage (Variables|Default|GetBPC_PlayerStats))
    (bind _isplayerdead (Default|DecreaseHealth (Variables|Default|GetBPC_playerStats) Damage))
    (if _isplayerdead
      (CallFunction|Destroyed)
      (else
        (Variables|/Game/ThirdPerson/Blueprints/BPC_PlayerStats.BPC_PlayerStats_C|SetCanTakeDamage _bpc_playerstats false)
        (Utilities|FlowControl|Delay 0.3)
        (Variables|/Game/ThirdPerson/Blueprints/BPC_PlayerStats.BPC_PlayerStats_C|SetCanTakeDamage _bpc_playerstats true)))))

(fn ConstructionScript)

(fn Stop
  (Audio|Components|Audio|Stop (Variables|Default|GetStartEndTimeline)))

(fn Continue
  (bind _startendtimeline (Variables|Default|GetStartEndTimeline))
  (if (Variables|Default|GetIsSpawning)
    (Audio|Components|Audio|Play _startendtimeline)
    (else
      (Utilities|String|Reverse _startendtimeline))))