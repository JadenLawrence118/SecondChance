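; Electrocution area for the Orpheus final boss's grenade, a child Blueprint that adds electric VFX and on/off control to its parent, which receives the damage value.
; BeginPlay sets the Niagara lifetime from AttackDuration.
; Activate and Deactivate toggle visibility, IsOn and a looping timer that re-activates the effect.
; Pause freezes effect and timer, Continue resumes only the effect, and DoDanageOnce just hides LaserShape.
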(event Custom|LoopVFX
  (Components|Activation|Activate (Variables|Default|GetNiagara) false))

(event Custom|DoDanageOnce
  (Rendering|SetVisibility (Variables|Default|GetLaserShape) false false))

(event EventBeginPlay
  (|CallParentFunction)
  (Niagara|SetNiagaraVariable(Float) (Variables|Default|GetNiagara) "Lifetime" (Variables|Default|GetAttackDuration)))

(event Collision|EventActorBeginOverlap
  (params (OtherActor :type Actor%20Object%20Reference)))

(event EventTick
  (params (DeltaSeconds :type Float%20%28single-precision%29))
  (|CallParentFunction DeltaSeconds) ; This node is disabled and will not be called.\nDrag off pins to build functionality.
)

(event EventContinue
  (Class|NiagaraComponent|SetPaused (Variables|Default|GetNiagara) false))

(event EventPause
  (Class|NiagaraComponent|SetPaused (Variables|Default|GetNiagara) true)
  (Utilities|Time|PauseTimerbyHandle (Variables|Default|GetTimer)))

(event EventActivate
  (Rendering|SetVisibility (Variables|Default|GetDefaultSceneRoot) true true)
  (Components|Activation|Activate (Variables|Default|GetNiagara) false)
  (Variables|Default|SetIsOn true)
  (bind _returnvalue (Utilities|Time|SetTimerbyEvent (delegate Custom|LoopVFX) 1.0 true))
  (Variables|Default|SetTimer _returnvalue))

(event EventDeactivate
  (Rendering|SetVisibility (Variables|Default|GetDefaultSceneRoot) false true)
  (Components|Activation|Deactivate (Variables|Default|GetNiagara))
  (Variables|Default|SetIsOn false)
  (Utilities|Time|ClearandInvalidateTimerbyHandle (Variables|Default|GetTimer)))

(event EventSetDamage
  (params (Damage :type Float%20%28double-precision%29))
  (|CallParentFunction Damage))

(fn ConstructionScript
  (|CallParentFunction))