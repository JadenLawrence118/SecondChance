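; Reusable grenade for the Orpheus final boss that flies to a target, explodes and leaves a timed electrocution area.
; TrajectoryToDestin moves the mesh by timelines as a quick throw, arced projectile or drop, scaling play rate by distance over speed and starting a telegraph circle at the destination.
; Landing activates the electrocute child actor until a timer frees the grenade.
; A state variable lets Stop and Continue pause and resume each phase.
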(event Custom|TrajectoryToDestin
  (params (Start%20Loc :type Vector) (Destination :type Vector) (ProjectileApex :type Float%20%28double-precision%29) (GrenadeType :type E_GrenadeType%20Enum :default "NewEnumerator0"))
  (bind _returnvalue (Math|Vector|Distance2D(Vector) Destination Start%20Loc))
  (bind (_x _y _z) (Math|Vector|BreakVector Start%20Loc))
  (bind (_x_2 _y_2 _z_2) (Math|Vector|BreakVector Destination))
  (bind (_x_3 _y_3 _z_3) (Math|Vector|BreakVector Start%20Loc))
  (bind (_x_4 _y_4 _z_4) (Math|Vector|BreakVector Start%20Loc))
  (bind (_x_5 _y_5 _z_5) (Math|Vector|BreakVector Destination))
  (bind (_x_6 _y_6 _z_6) (Math|Vector|BreakVector Destination))
  (bind _z_7 (Math|Vector|BreakVector Start%20Loc))
  (bind _z_8 (Math|Vector|BreakVector Destination))
  (bind _staticmesh (Variables|Default|GetStaticMesh))
  (bind _staticmesh_2 (Variables|Default|GetStaticMesh))
  (bind _telegraphcircle (Variables|Default|GetTelegraphCircle))
  (bind _qtmoving_speed_unit_per_sec_ (Variables|Default|GetQTMoving%20Speed%28Unit%20Per%20Sec%29))
  (bind _pmoving_speed_unit_per_sec_ (Variables|Default|GetPMoving%20Speed%28Unit%20Per%20Sec%29))
  (bind _dmoving_speed_unit_per_sec_ (Variables|Default|GetDMoving%20Speed%28Unit%20Per%20Sec%29))
  (bind _staticmesh_3 (Variables|Default|GetStaticMesh))
  (bind _returnvalue_2 (/ _returnvalue _qtmoving_speed_unit_per_sec_))
  (bind _returnvalue_3 (/ _returnvalue _pmoving_speed_unit_per_sec_))
  (bind _returnvalue_4 (- _z_7 _z_8))
  (bind _relativerotation (Variables|/Script/Engine.SceneComponent|GetRelativeRotation _staticmesh_2))
  (bind _relativerotation_2 (Variables|/Script/Engine.SceneComponent|GetRelativeRotation _staticmesh))
  (bind _relativerotation_3 (Variables|/Script/Engine.SceneComponent|GetRelativeRotation _staticmesh_3))
  (bind _returnvalue_5 (+ (.roll _relativerotation_2) 1.0))
  (bind _returnvalue_6 (/ _returnvalue_4 _dmoving_speed_unit_per_sec_))
  (bind _returnvalue_7 (+ (.roll _relativerotation_3) 1.0))
  (bind _returnvalue_8 (+ (.roll _relativerotation) 1.0))
  (bind _returnvalue_9 (Utilities|Select :Index GrenadeType :NewEnumerator0 _returnvalue_2 :NewEnumerator1 _returnvalue_3 :NewEnumerator2 _returnvalue_6))
  (bind _returnvalue_10 (/ 1.0 _returnvalue_9))
  (Variables|Default|SetGrenade%20Type GrenadeType)
  (Variables|Default|SetIsInUse true)
  (Rendering|SetVisibility (Variables|Default|GetStaticMesh) true false)
  ;[1 1 1] The time of grende projectile motion
  (switch Utilities|FlowControl|Switch|SwitchonE_GrenadeType (Variables|Default|GetGrenade%20Type)
    (:NewEnumerator0
      (Components|Timeline|SetPlayRate (Variables|Default|GetQTTimeline) _returnvalue_10))
    (:NewEnumerator1
      (Components|Timeline|SetPlayRate (Variables|Default|GetProjectileMotionZUp) _returnvalue_10))
    (:NewEnumerator2
      (Components|Timeline|SetPlayRate (Variables|Default|GetDropTimeline) _returnvalue_10)))
  ;[1 1 1] Start warning at destination
  (Transformation|SetWorldLocation _telegraphcircle Destination false false)
  (Class|BPITelegraph|Start(Message) (Variables|/Script/Engine.ChildActorComponent|GetChildActor _telegraphcircle) _returnvalue_9)
  (Variables|Default|SetState "NewEnumerator2")
  (switch Utilities|FlowControl|Switch|SwitchonE_GrenadeType (Variables|Default|GetGrenade%20Type)
    (:NewEnumerator0
      ;[1 1 1] Grenade QuickThrowMotion
      (bind (_direction _x_y_movement _z_movement) (Timeline|QTTimeline PlayFromStart)
        (:Update
          (Transformation|SetWorldLocation _staticmesh (Math|Vector|MakeVector (Math|Float|Lerp _x_4 _x_5 _x_y_movement) (Math|Float|Lerp _y_4 _y_5 _x_y_movement) (Math|Float|Lerp _z_4 _z_5 _z_movement)) false false)
          (Transformation|SetRelativeRotation _staticmesh (Math|Rotator|MakeRotator _returnvalue_5 _returnvalue_5 _returnvalue_5) false false))
        (:Finished
          (Components|Activation|Activate (Variables|Default|GetExplosion) false :!label _label)
          (Rendering|SetVisibility (Variables|Default|GetStaticMesh) false false)
          (Class|BPITelegraph|Reset(Message) (Variables|/Script/Engine.ChildActorComponent|GetChildActor (Variables|Default|GetTelegraphCircle)))
          (Class|BPIBossAreaAttack|Activate(Message) (Variables|/Script/Engine.ChildActorComponent|GetChildActor (Variables|Default|GetElectrocuteArea)))
          (bind _returnvalue_11 (Utilities|Time|SetTimerbyEvent (delegate Custom|ElectrocuteEnd) (Variables|Default|GetActivateTime)))
          (Variables|Default|SetTimer _returnvalue_11)
          (Variables|Default|SetState "NewEnumerator3")
          (Transformation|SetRelativeRotation (Variables|Default|GetStaticMesh) "0, 0, 0" false false))))
    (:NewEnumerator1
      ;[1 1 1] Grenade Projectile Motion
      (CallFunction|ProjectileZMove _z _z_2 ProjectileApex)
      (bind _x_y_movement_2 (Timeline|ProjectileMotionXY PlayFromStart)
        (:Update
          (Transformation|SetWorldLocation _staticmesh_2 (Math|Vector|MakeVector (Math|Float|Lerp _x _x_2 _x_y_movement_2) (Math|Float|Lerp _y _y_2 _x_y_movement_2) (.z (Transformation|GetWorldLocation (Variables|Default|GetStaticMesh)))) false false)
          (Transformation|SetRelativeRotation _staticmesh_2 (Math|Rotator|MakeRotator _returnvalue_8 _returnvalue_8 _returnvalue_8) false false))
        (:Finished
          (goto _label))))
    (:NewEnumerator2
      ;[1 1 1] Grenade Dropping Movment
      (bind _z_movement_2 (Timeline|DropTimeline PlayFromStart)
        (:Update
          (Transformation|SetWorldLocation _staticmesh_3 (Math|Vector|MakeVector (Math|Float|Lerp _x_3 _x_6 _z_movement_2) (Math|Float|Lerp _y_3 _y_6 _z_movement_2) (Math|Float|Lerp _z_3 _z_6 _z_movement_2)) false false)
          (Transformation|SetRelativeRotation _staticmesh_3 (Math|Rotator|MakeRotator _returnvalue_7 _returnvalue_7 _returnvalue_7) false false))
        (:Finished
          (goto _label))))))

(event Custom|ElectrocuteEnd
  (Class|BPIBossAreaAttack|Deactivate(Message) (Variables|/Script/Engine.ChildActorComponent|GetChildActor (Variables|Default|GetElectrocuteArea)))
  (Variables|Default|SetState "NewEnumerator0")
  (Variables|Default|SetIsInUse false)
  (Utilities|Time|ClearandInvalidateTimerbyHandle (Variables|Default|GetTimer)))

(event Custom|Projectile%20Z%20move
  (params (StartPosZ :type Float%20%28double-precision%29) (DesPosZ :type Float%20%28double-precision%29) (ProjectileApex :type Float%20%28double-precision%29))
  (bind _returnvalue (+ StartPosZ ProjectileApex))
  (bind _staticmesh (Variables|Default|GetStaticMesh))
  (bind _staticmesh_2 (Variables|Default|GetStaticMesh))
  (bind _returnvalue_2 (Transformation|GetWorldLocation _staticmesh))
  (bind _returnvalue_3 (Transformation|GetWorldLocation _staticmesh_2))
  ;[1 1 1] Grenade Projectile Motion
  (bind _x_y_movement (Timeline|ProjectileMotionZUp PlayFromStart)
    (:Update
      (Transformation|SetWorldLocation _staticmesh_2 (Math|Vector|MakeVector (.x _returnvalue_3) (.y _returnvalue_3) (Math|Float|Lerp StartPosZ _returnvalue _x_y_movement)) false false))
    (:Finished
      (Variables|Default|SetState "NewEnumerator4")
      (bind _x_y_movement_2 (Timeline|ProjectileMotionDown PlayFromStart)
        (:Update
          (Transformation|SetWorldLocation _staticmesh (Math|Vector|MakeVector (.x _returnvalue_2) (.y _returnvalue_2) (Math|Float|Lerp _returnvalue DesPosZ _x_y_movement_2)) false false))))))

(event EventBeginPlay
  ;[1 1 1] BeginPlay
  (Rendering|SetVisibility (Variables|Default|GetStaticMesh) false false)
  (Components|Activation|Deactivate (Variables|Default|GetExplosion))
  (Class|BPIBossAreaAttack|Deactivate(Message) (Variables|/Script/Engine.ChildActorComponent|GetChildActor (Variables|Default|GetElectrocuteArea)))
  (Class|BPITelegraph|Reset(Message) (Variables|/Script/Engine.ChildActorComponent|GetChildActor (Variables|Default|GetTelegraphCircle))))

(event EventTick
  (params (DeltaSeconds :type Float%20%28single-precision%29)))

(fn ConstructionScript)

(fn HeldatHand
  (params (SpawnPos :type Vector))
  (bind _staticmesh (Variables|Default|GetStaticMesh))
  (Transformation|SetWorldLocation _staticmesh SpawnPos false false)
  (Rendering|SetVisibility _staticmesh true false)
  (Variables|Default|SetState "NewEnumerator1"))

(fn InitGrenadeVar
  (params (ActivateTime :type Float%20%28single-precision%29))
  (Variables|Default|SetActivateTime ActivateTime))

(fn Stop
  (switch Utilities|FlowControl|Switch|SwitchonE_GrenadeState (Variables|Default|GetState)
    (:NewEnumerator2
      (switch Utilities|FlowControl|Switch|SwitchonE_GrenadeType (Variables|Default|GetGrenade%20Type)
        (:NewEnumerator0
          (Audio|Components|Audio|Stop (Variables|Default|GetQTTimeline)))
        (:NewEnumerator1
          (Audio|Components|Audio|Stop (Variables|Default|GetProjectileMotionZUp))
          (Audio|Components|Audio|Stop (Variables|Default|GetProjectileMotionXY) :!label _label))
        (:NewEnumerator2
          (Audio|Components|Audio|Stop (Variables|Default|GetDropTimeline))))
      (Class|BPITelegraph|Pause(Message) (Variables|Default|GetTelegraphCircle)))
    (:NewEnumerator4
      (Audio|Components|Audio|Stop (Variables|Default|GetProjectileMotionDown))
      (goto _label))
    (:NewEnumerator3
      (Utilities|Time|PauseTimerbyHandle (Variables|Default|GetTimer))
      (Class|BPIBossAreaAttack|Pause(Message) (Variables|Default|GetElectrocuteArea)))))

(fn Continue
  (switch Utilities|FlowControl|Switch|SwitchonE_GrenadeState (Variables|Default|GetState)
    (:NewEnumerator2
      (switch Utilities|FlowControl|Switch|SwitchonE_GrenadeType (Variables|Default|GetGrenade%20Type)
        (:NewEnumerator0
          (Audio|Components|Audio|Play (Variables|Default|GetQTTimeline)))
        (:NewEnumerator1
          (Audio|Components|Audio|Play (Variables|Default|GetProjectileMotionZUp))
          (Audio|Components|Audio|Play (Variables|Default|GetProjectileMotionXY) :!label _label))
        (:NewEnumerator2
          (Audio|Components|Audio|Play (Variables|Default|GetDropTimeline))))
      (Class|BPITelegraph|Continue(Message) (Variables|Default|GetTelegraphCircle)))
    (:NewEnumerator4
      (Audio|Components|Audio|Play (Variables|Default|GetProjectileMotionDown))
      (goto _label))
    (:NewEnumerator3
      (Utilities|Time|UnpauseTimerbyHandle (Variables|Default|GetTimer))
      (Class|BPIBossAreaAttack|Continue(Message) (Variables|Default|GetElectrocuteArea)))))