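; Orion boss character: a sword fighter with overhead swing, sweep, block, dodge, EQS quick move, strafe and jump enter/exit.
; Each action event drives montages, timelines or timers, then reports completion through dispatchers, which also signal QTE, half health and death.
; Montage notifies drive telegraphed lunges and sword traces, while well-angled hits on its block trigger a QTE.
; Pause/Continue implement time stop by freezing time dilation and the current state's timeline or timer.
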(event Custom|OverheadSwing
  (params (Target%20Actor :type Actor%20Object%20Reference) (QTE%20ver? :type Boolean))
  (bind _attackwarning_ref (Variables|Default|GetAttackWarning%20Ref))
  ;[1 1 1] Attack 1 : Overhead Swing
  (if QTE%20ver?
    (bind _notifyname (Animation|Montage|PlayMontage (Variables|Character|GetMesh) "/Game/Art/Characters/Orion/Animations/AnimMontage/AM_OverheadSwing.AM_OverheadSwing" 0.7)
      (:OnCompleted
        (Utilities|FlowControl|Delay 0.5)
        (Default|CallOnQTEAttackEnd))
      (:OnNotifyEnd
        (switch name _notifyname
          (:SwordTrace
            (Game|Damage|ApplyDamage Target%20Actor (Variables|Attack|GetQTEOverheadSwing%20Damge) 0 0)))))
    (else
      (Variables|State|SetCurrentState "NewEnumerator8")
      (bind _notifyname_2 (Animation|Montage|PlayMontage (Variables|Character|GetMesh) "/Game/Art/Characters/Orion/Animations/AnimMontage/AM_OverheadSwing.AM_OverheadSwing")
        (:then
          (Transformation|SetActorLocation _attackwarning_ref (- (Transformation|GetActorLocation) "0.000000,0.000000,87.000000") false false)
          (Class|BPITelegraph|Start(Message) _attackwarning_ref 0.7)
          (Components|Timeline|PlayfromStart (Variables|Default|GetWarningTimeline))
          (Variables|Default|SetIsWarning true))
        (:OnCompleted
          (Variables|State|SetCurrentState "NewEnumerator8")
          (CallFunction|StartTracingTarget Target%20Actor)
          (Default|CallOnActionEnd))
        (:OnNotifyBegin
          (switch name _notifyname_2
            (:SwordTrace
              (Variables|Default|SetIsWarning false)
              (Class|BPITelegraph|Reset(Message) (Variables|Default|GetAttackWarning%20Ref))
              (Default|StartMeleeTrace (Variables|Default|GetBPC_SwordTrace) (Variables|Default|GetSwordTraceTop) (Variables|Default|GetSwordTraceEnd) (Variables|Attack|GetSword%20Trace%20Radius) (Variables|Attack|GetOverhead%20Swing%20Damage) 0.001)
              (Variables|State|SetCurrentState "NewEnumerator2")
              (Components|Timeline|PlayfromStart (Variables|Default|GetAttackMoveTimeline)))
            (:LookAtTarget
              (CallFunction|StartTracingTarget Target%20Actor))))
        (:OnNotifyEnd
          (switch name _notifyname_2
            (:SwordTrace
              (Default|StopMeleeTrace (Variables|Default|GetBPC_SwordTrace)))
            (:LookAtTarget
              (CallFunction|StopTracingTarget)
              (Variables|Attack|SetAttackDestination (+ (Transformation|GetActorLocation Target%20Actor) (/ (Transformation|GetVelocity Target%20Actor) 1e+01))))))))))

(event Custom|Block
  (params (Target :type Actor%20Object%20Reference))
  ;[1 1 1] Attack 2 : Block
  (CallFunction|StopTracingTarget)
  (Variables|State|SetCurrentState "NewEnumerator3")
  (Variables|Block|SetIsBlocking true)
  (bind _asabp_orion (Utilities|Casting|CastToABP_Orion (Components|SkeletalMesh|GetAnimInstance (Variables|Character|GetMesh)))
    (:then
      (Variables|/Game/Enemies/Boss/FinalBoss/Orion/ABP_Orion.ABP_Orion_C|SetIsBlocking _asabp_orion true)
      (Utilities|Time|ClearandInvalidateTimerbyHandle (Variables|Block|GetBlockTimer))
      (bind _returnvalue (Utilities|Time|SetTimerbyEvent (delegate Custom|BlockEnd) (Variables|Block|GetBlock%20Durartion)))
      (Variables|Block|SetBlockTimer _returnvalue))
    (:CastFailed
      (Development|PrintString "ABP_Orion Cast Failed"))))

(event Custom|StopTracingTarget
  (bind _returnvalue (Transformation|GetActorRotation))
  (bind (_roll _pitch) (Math|Rotator|BreakRotator _returnvalue))
  ;[1 1 1] Rotate to focus on Target when telegraphing
  (bind _lerp_alpha (Timeline|RotateToPlayer Stop)
    (:Update
      (Transformation|SetActorRotation (Math|Rotator|Lerp(Rotator) _returnvalue (Math|Rotator|MakeRotator _roll _pitch (.yaw (Math|Rotator|FindLookatRotation (Transformation|GetActorLocation) (Transformation|GetActorLocation (stale Custom|StartTracingTarget Target))))) _lerp_alpha true)))
    (:Finished
      (CallFunction|StartTracingTarget (stale Custom|StartTracingTarget Target)))))

(event Custom|Continue
  (params (TargetActor :type Actor%20Object%20Reference))
  (bind _enterexittimeline (Variables|Default|GetEnterExitTimeline))
  (bind _waittimer (Variables|wait|GetWaitTimer))
  ;[1 1 1] Time Resume
  (if (not (Variables|State|GetIsDead))
    (Variables|Default|SetCustomTimeDilation 1.0)
    (switch Utilities|FlowControl|Switch|SwitchonE_OrionState (Variables|State|GetCurrentState)
      (:NewEnumerator0
        (Utilities|Time|UnpauseTimerbyHandle (Variables|Movement|GetStarfeTimer)))
      (:NewEnumerator10
        (Audio|Components|Audio|Play (Variables|Default|GetQuckMoveTimeline)))
      (:NewEnumerator1
        (Audio|Components|Audio|Play (Variables|Default|GetDodgeBTimeline)))
      (:NewEnumerator8
        (if (Variables|Default|GetIsWarning)
          (Audio|Components|Audio|Play (Variables|Default|GetWarningTimeline)))
        (CallFunction|StartTracingTarget TargetActor)
        (if (Utilities|Time|IsValidTimerHandle _waittimer)
          (Utilities|Time|UnpauseTimerbyHandle _waittimer)))
      (:NewEnumerator2
        (Audio|Components|Audio|Play (Variables|Default|GetAttackMoveTimeline) :!label _label))
      (:NewEnumerator3
        (Utilities|Time|UnpauseTimerbyHandle (Variables|Block|GetBlockTimer)))
      (:NewEnumerator4
        (goto _label))
      (:NewEnumerator5
        (Utilities|String|Reverse _enterexittimeline))
      (:NewEnumerator9
        (Audio|Components|Audio|Play _enterexittimeline)))))

(event Custom|EndBlockAnim
  ;[1 1 1] Attack 2 : Block
  (Variables|Block|SetIsBlocking false)
  (bind _asabp_orion (Utilities|Casting|CastToABP_Orion (Components|SkeletalMesh|GetAnimInstance (Variables|Character|GetMesh)))
    (:then
      (Variables|/Game/Enemies/Boss/FinalBoss/Orion/ABP_Orion.ABP_Orion_C|SetIsBlocking _asabp_orion false))
    (:CastFailed
      (Development|PrintString "ABP_Orion cast FAILED"))))

(event Custom|MoveBack
  (params (MoveDistance :type Float%20%28double-precision%29))
  ;[1 1 1] QTE MoveBack when player sucess
  (Variables|Movement|SetMovementOriginalPos (Transformation|GetActorLocation))
  (bind (_possible_location _usepossiblepos) (Utilities|DodgeValidation MoveDistance)
    (:True
      (bind _alpha (Timeline|Timeline PlayFromStart)
        (:Update
          (Transformation|SetActorLocation (Math|Vector|MakeVector (Math|Float|Lerp (.X (Math|Vector|BreakVector (Variables|Movement|GetMovementOriginalPos))) (.X (Math|Vector|BreakVector (select _usepossiblepos _possible_location (- (Variables|Movement|GetMovementOriginalPos) (* (Transformation|GetActorForwardVector) MoveDistance))))) _alpha) (Math|Float|Lerp (.Y (Math|Vector|BreakVector (Variables|Movement|GetMovementOriginalPos))) (.Y (Math|Vector|BreakVector (select _usepossiblepos _possible_location (- (Variables|Movement|GetMovementOriginalPos) (* (Transformation|GetActorForwardVector) MoveDistance))))) _alpha) (.z (Transformation|GetActorLocation))) false false))))
    (:False
      (Timeline|Timeline PlayFromStart))))

(event Custom|Enter
  (bind _returnvalue (Transformation|GetActorForwardVector))
  (bind _exitposition (Variables|Exit|GetExitPosition))
  (bind _returnvalue_2 (* _returnvalue -1.0))
  (bind _returnvalue_3 (+ _exitposition "0.000000,0.000000,500.000000"))
  (bind _returnvalue_4 (* _returnvalue_2 1e+03))
  (bind _returnvalue_5 (+ _returnvalue_3 _returnvalue_4))
  (bind (_x _y _z) (Math|Vector|BreakVector _returnvalue_5))
  ;[1 1 1] Enter /Exit
  (Variables|/Game/ThirdPerson/Blueprints/BPC_PlayerStats.BPC_PlayerStats_C|SetCanTakeDamage (Variables|Default|GetBPC_PlayerStats) true)
  (Variables|State|SetCurrentState "NewEnumerator5")
  (Rendering|SetVisibility (Variables|Collision|GetCapsuleComponent) true true)
  (Variables|/Script/Engine.CharacterMovementComponent|SetGravityScale (Variables|Character|GetCharacterMovement) 0.01)
  (bind (_direction _posxylerpalpha _poszlerpalpha) (Timeline|EnterExitTimeline ReverseFromEnd)
    (:Update
      (Transformation|SetActorLocation (Math|Vector|MakeVector (Math|Float|Lerp (.X (Math|Vector|BreakVector (stale Custom|Exit _output_get))) _x _posxylerpalpha) (Math|Float|Lerp (.Y (Math|Vector|BreakVector (stale Custom|Exit _output_get))) _y _posxylerpalpha) (Math|Float|Lerp (.Z (Math|Vector|BreakVector (stale Custom|Exit _output_get))) _z _poszlerpalpha)) false true))
    (:Finished
      (switch Utilities|FlowControl|Switch|SwitchonETimelineDirection _direction
        (:Forward
          (Rendering|SetVisibility (Variables|Collision|GetCapsuleComponent) false true)
          (Variables|State|SetCurrentState "NewEnumerator6"))
        (:Backward
          (Variables|State|SetCurrentState "NewEnumerator8")
          (Animation|Montage|PlayMontage (Variables|Character|GetMesh) "/Game/Art/Characters/Orion/Animations/Jump/AM_Land.AM_Land"
            (:OnCompleted
              _))))
      (Default|CallOnActionEnd))))

(event Custom|Exit
  ;[1 1 1] Enter /Exit
  (Variables|/Game/ThirdPerson/Blueprints/BPC_PlayerStats.BPC_PlayerStats_C|SetCanTakeDamage (Variables|Default|GetBPC_PlayerStats) false)
  (Variables|/Script/Engine.CharacterMovementComponent|SetGravityScale (Variables|Character|GetCharacterMovement) 0.0)
  (bind _output_get (Variables|Exit|SetExitPosition (Transformation|GetActorLocation)))
  (bind _notifyname (Animation|Montage|PlayMontage (Variables|Character|GetMesh) "/Game/Art/Characters/Orion/Animations/Jump/AM_Jump.AM_Jump")
    (:OnNotifyBegin
      (switch name _notifyname
        (:Jump
          (Variables|State|SetCurrentState "NewEnumerator9")
          (bind (_direction _posxylerpalpha _poszlerpalpha) (Timeline|EnterExitTimeline PlayFromStart)
            (:Update
              (Transformation|SetActorLocation (Math|Vector|MakeVector (Math|Float|Lerp (.X (Math|Vector|BreakVector _output_get)) (.X (Math|Vector|BreakVector (+ (+ (Variables|Exit|GetExitPosition) "0.000000,0.000000,500.000000") (* (* (Transformation|GetActorForwardVector) -1.0) 1e+03)))) _posxylerpalpha) (Math|Float|Lerp (.Y (Math|Vector|BreakVector _output_get)) (.Y (Math|Vector|BreakVector (+ (+ (Variables|Exit|GetExitPosition) "0.000000,0.000000,500.000000") (* (* (Transformation|GetActorForwardVector) -1.0) 1e+03)))) _posxylerpalpha) (Math|Float|Lerp (.Z (Math|Vector|BreakVector _output_get)) (.Z (Math|Vector|BreakVector (+ (+ (Variables|Exit|GetExitPosition) "0.000000,0.000000,500.000000") (* (* (Transformation|GetActorForwardVector) -1.0) 1e+03)))) _poszlerpalpha)) false true))
            (:Finished
              (switch Utilities|FlowControl|Switch|SwitchonETimelineDirection _direction
                (:Forward
                  (Rendering|SetVisibility (Variables|Collision|GetCapsuleComponent) false true)
                  (Variables|State|SetCurrentState "NewEnumerator6"))
                (:Backward
                  (Variables|State|SetCurrentState "NewEnumerator8")
                  (Animation|Montage|PlayMontage (Variables|Character|GetMesh) "/Game/Art/Characters/Orion/Animations/Jump/AM_Land.AM_Land"
                    (:OnCompleted
                      _))))
              (Default|CallOnActionEnd))))))))

(event Custom|Strafe
  (params (TargetActor :type Actor%20Object%20Reference))
  ;[1 1 1] Strafe
  (Variables|State|SetCurrentState "NewEnumerator0")
  (bind _returnvalue (Utilities|Time|SetTimerbyEvent (delegate Custom|Stafe%20Time) (Variables|Movement|GetStrafeTime)))
  (Variables|Movement|SetStarfeTimer _returnvalue)
  (Variables|/Script/Engine.CharacterMovementComponent|SetMaxWalkSpeed (Variables|Character|GetCharacterMovement) 1e+02)
  (AI|AIMoveTo self "0, 0, 0" TargetActor 3e+02 true
    (:OnSuccess
      (Utilities|Time|ClearandInvalidateTimerbyHandle (Variables|Movement|GetStarfeTimer))
      (Default|CallOnMovementEnd))))

(event Custom|Stafe%20Time
  ;[1 1 1] Strafe
  (Utilities|Time|ClearandInvalidateTimerbyHandle (Variables|Movement|GetStarfeTimer))
  (Default|CallOnMovementEnd))

(event Custom|BlockEnd
  ;[1 1 1] Attack 2 : Block
  (Utilities|Time|ClearandInvalidateTimerbyHandle (Variables|Block|GetBlockTimer))
  (Variables|State|SetCurrentState "NewEnumerator8")
  (CallFunction|EndBlockAnim)
  (Default|CallOnActionEnd))

(event Custom|Wait
  (params (Phase2Attack3? :type Boolean))
  ;[1 1 1] Wait Function
  (bind _returnvalue (Utilities|Time|SetTimerbyEvent (delegate Custom|WaitEnd) (Math|Float|SelectFloat (Variables|Wait|GetPhase2%20Attack%203WaitTime) (Variables|wait|GetWaitTime) Phase2Attack3?)))
  (Variables|wait|SetWaitTimer _returnvalue))

(event Custom|WaitEnd
  ;[1 1 1] Wait Function
  (Utilities|Time|ClearandInvalidateTimerbyHandle (Variables|wait|GetWaitTimer))
  (Default|CallOnWaitEnd))

(event Custom|Sweep
  (params (Target%20Actor :type Actor%20Object%20Reference))
  (bind _attackwarning_ref (Variables|Default|GetAttackWarning%20Ref))
  ;[1 1 1] Attack 3 : Sweep
  (Variables|State|SetCurrentState "NewEnumerator8")
  (bind _notifyname (Animation|Montage|PlayMontage (Variables|Character|GetMesh) "/Game/Art/Characters/Orion/Animations/AnimMontage/AM_Sweep.AM_Sweep")
    (:then
      (Transformation|SetActorLocation _attackwarning_ref (- (Transformation|GetActorLocation) "0.000000,0.000000,87.000000") false false)
      (Class|BPITelegraph|Start(Message) _attackwarning_ref 1.0)
      (Components|Timeline|PlayfromStart (Variables|Default|GetWarningTimeline))
      (Variables|Default|SetIsWarning true))
    (:OnCompleted
      (Variables|State|SetCurrentState "NewEnumerator8")
      (CallFunction|StartTracingTarget Target%20Actor)
      (Default|CallOnActionEnd))
    (:OnNotifyBegin
      (switch name _notifyname
        (:SwordTrace
          (Variables|Default|SetIsWarning false)
          (Class|BPITelegraph|Reset(Message) (Variables|Default|GetAttackWarning%20Ref))
          (Default|StartMeleeTrace (Variables|Default|GetBPC_SwordTrace) (Variables|Default|GetSwordTraceTop) (Variables|Default|GetSwordTraceEnd) (Variables|Attack|GetSword%20Trace%20Radius) (Variables|Attack|GetSweep%20Damage) 0.001)
          (Variables|State|SetCurrentState "NewEnumerator4")
          (Components|Timeline|PlayfromStart (Variables|Default|GetAttackMoveTimeline)))
        (:LookAtTarget
          (CallFunction|StartTracingTarget Target%20Actor))))
    (:OnNotifyEnd
      (switch name _notifyname
        (:SwordTrace
          (Default|StopMeleeTrace (Variables|Default|GetBPC_SwordTrace)))
        (:LookAtTarget
          (CallFunction|StopTracingTarget)
          (Variables|Attack|SetAttackDestination (+ (Transformation|GetActorLocation Target%20Actor) (/ (Transformation|GetVelocity Target%20Actor) 1e+01))))))))

(event Custom|Dodge
  (params (After%20Block%20Fail? :type Boolean) (Target :type Actor%20Object%20Reference))
  (bind _bpc_playerstats (Variables|Default|GetBPC_PlayerStats))
  (bind _movementoriginalpos (Variables|Movement|GetMovementOriginalPos))
  (bind _mesh (Variables|Default|GetMesh))
  (bind _returnvalue (Components|SkeletalMesh|GetAnimInstance _mesh))
  (bind (_x _y) (Math|Vector|BreakVector _movementoriginalpos))
  ;[1 1 1] Dodge Back
  (CallFunction|StopTracingTarget)
  ;;[1 1 1] Check Valid space to dodge
  (bind (_possible_location _usepossiblepos) (Utilities|DodgeValidation (Variables|Movement|GetDodgeDistance))
    (:True
      (bind _notifyname (Animation|Montage|PlayMontage _mesh "/Game/Art/Characters/Orion/Animations/DodgeBack/AM_DodgeBack.AM_DodgeBack")
        (:OnNotifyBegin
          (switch name _notifyname
            (:Move
              (Animation|Montage|MontageSetPlayRate _returnvalue "/Game/Art/Characters/Orion/Animations/DodgeBack/AM_DodgeBack.AM_DodgeBack" (/ 1.0 (Variables|Movement|GetDodgeDuration%28s%29)))
              (Variables|/Game/ThirdPerson/Blueprints/BPC_PlayerStats.BPC_PlayerStats_C|SetCanTakeDamage _bpc_playerstats false)
              (Variables|State|SetCurrentState "NewEnumerator1")
              (bind _alpha (Timeline|DodgeBTimeline PlayFromStart)
                (:Update
                  (Transformation|SetActorLocation (Math|Vector|MakeVector (Math|Float|Lerp _x (.X (Math|Vector|BreakVector (select _usepossiblepos _possible_location (- _movementoriginalpos (* (Transformation|GetActorForwardVector) (Variables|Movement|GetDodgeDistance)))))) _alpha) (Math|Float|Lerp _y (.Y (Math|Vector|BreakVector (select _usepossiblepos _possible_location (- _movementoriginalpos (* (Transformation|GetActorForwardVector) (Variables|Movement|GetDodgeDistance)))))) _alpha) (.z (Transformation|GetActorLocation))) false false))
                (:Finished
                  (Variables|State|SetCurrentState "NewEnumerator8")
                  (if After%20Block%20Fail?
                    (Default|CallOnActionEnd)
                    (else
                      (Default|CallOnMovementEnd))))))))
        (:OnNotifyEnd
          (switch name _notifyname
            (:Move
              (Variables|/Game/ThirdPerson/Blueprints/BPC_PlayerStats.BPC_PlayerStats_C|SetCanTakeDamage _bpc_playerstats true)
              (Animation|Montage|MontageSetPlayRate _returnvalue "/Game/Art/Characters/Orion/Animations/DodgeBack/AM_DodgeBack.AM_DodgeBack" 1.0))))))
    (:False
      (CallFunction|QuickMove Target))))

(event Custom|QuickMove
  (params (Target :type Actor%20Object%20Reference))
  ;[1 1 1] QuickMove
  (CallFunction|StopTracingTarget)
  (Variables|Movement|SetMovementOriginalPos (Transformation|GetActorLocation))
  (bind _returnvalue (AI|EQS|RunEQSQuery "/Game/Enemies/Boss/FinalBoss/Orion/EQS_OrionAttackRange.EQS_OrionAttackRange" self "RandomBest25Pct"))
  (EventDispatchers|AssignOnQueryFinishedEvent _returnvalue (delegate Custom|OnQueryFinishedEvent_Event)))

(event Custom|Pause
  (bind _waittimer (Variables|wait|GetWaitTimer))
  ;[1 1 1] Time Stop
  (if (not (Variables|State|GetIsDead))
    (Variables|Default|SetCustomTimeDilation 0.0)
    (CallFunction|StopTracingTarget)
    (switch Utilities|FlowControl|Switch|SwitchonE_OrionState (Variables|State|GetCurrentState)
      (:NewEnumerator0
        (Utilities|Time|PauseTimerbyHandle (Variables|Movement|GetStarfeTimer)))
      (:NewEnumerator10
        (Audio|Components|Audio|Stop (Variables|Default|GetQuckMoveTimeline)))
      (:NewEnumerator1
        (Audio|Components|Audio|Stop (Variables|Default|GetDodgeBTimeline)))
      (:NewEnumerator8
        (if (Variables|Default|GetIsWarning)
          (Audio|Components|Audio|Stop (Variables|Default|GetWarningTimeline)))
        (if (Utilities|Time|IsValidTimerHandle _waittimer)
          (Utilities|Time|PauseTimerbyHandle _waittimer)))
      (:NewEnumerator2
        (Audio|Components|Audio|Stop (Variables|Default|GetAttackMoveTimeline) :!label _label))
      (:NewEnumerator3
        (Utilities|Time|PauseTimerbyHandle (Variables|Block|GetBlockTimer)))
      (:NewEnumerator4
        (goto _label))
      (:NewEnumerator5
        (Audio|Components|Audio|Stop (Variables|Default|GetEnterExitTimeline) :!label _label_2))
      (:NewEnumerator9
        (goto _label_2)))))

(event Custom|OnQueryFinishedEvent_Event
  (params (QueryInstance :type Env%20Query%20Instance%20Blueprint%20Wrapper%20Object%20Reference) (QueryStatus :type EEnvQueryStatus%20Enum :default "Processing"))
  (bind _movementoriginalpos (Variables|Movement|GetMovementOriginalPos))
  (bind (_x _y _z) (Math|Vector|BreakVector _movementoriginalpos))
  ;[1 1 1] QuickMove
  (bind (_resultlocations _returnvalue) (AI|EQS|GetQueryResultsasLocations QueryInstance))
  (if _returnvalue
    (Components|Timeline|SetPlayRate (Variables|Default|GetQuckMoveTimeline) 5.0)
    (Variables|State|SetCurrentState "NewEnumerator10")
    (bind _move (Timeline|QuckMoveTimeline PlayFromStart)
      (:Update
        (Transformation|SetActorLocation (Math|Vector|MakeVector (Math|Float|Lerp _x (.X (Math|Vector|BreakVector (Utilities|Array|Get(acopy) _resultlocations))) _move) (Math|Float|Lerp _y (.Y (Math|Vector|BreakVector (Utilities|Array|Get(acopy) _resultlocations))) _move) (Math|Float|Lerp _z (.Z (Math|Vector|BreakVector (Utilities|Array|Get(acopy) _resultlocations))) _move)) false false))
      (:Finished
        (Variables|State|SetCurrentState "NewEnumerator8")
        (Default|CallOnMovementEnd)))
    (else
      (CallFunction|Dodge false (stale Custom|QuickMove Target)))))

(event Custom|StartTracingTarget
  (params (Target :type Actor%20Object%20Reference))
  (bind _returnvalue (Transformation|GetActorRotation))
  (bind (_roll _pitch) (Math|Rotator|BreakRotator _returnvalue))
  ;[1 1 1] Rotate to focus on Target when telegraphing
  (bind _lerp_alpha (Timeline|RotateToPlayer PlayFromStart)
    (:Update
      (Transformation|SetActorRotation (Math|Rotator|Lerp(Rotator) _returnvalue (Math|Rotator|MakeRotator _roll _pitch (.yaw (Math|Rotator|FindLookatRotation (Transformation|GetActorLocation) (Transformation|GetActorLocation Target)))) _lerp_alpha true)))
    (:Finished
      (CallFunction|StartTracingTarget Target))))

(event EventBeginPlay
  ;[1 1 1] BeginPlay
  (Utilities|FlowControl|Sequence
    (:then_0
      (Components|Timeline|SetPlayRate (Variables|Default|GetDodgeBTimeline) (/ 1.0 (Variables|Movement|GetDodgeDuration%28s%29))))
    (:then_1
      (Utilities|FlowControl|DelayUntilNextTick)
      (bind _foundwidgets (Widget|GetAllWidgetsOfClass "/Game/UI/Boss/WB_BossHealth_Orpheus_Orion.WB_BossHealth_Orpheus_Orion_C" true))
      (for _array_element _foundwidgets
        _)
      (bind _output_get (Variables|Default|SetHealthBar _array_element))
      (Default|UpdateHealthBar _output_get))
    (:then_2
      (bind _asbp_third_person_character (Utilities|Casting|CastToBP_ThirdPersonCharacter (Game|GetPlayerCharacter 0)))
      (Variables|Default|SetPlayerRef _asbp_third_person_character))
    (:then_3
      (bind _returnvalue (Game|SpawnActorfromClass "/Game/Enemies/Boss/Megaera/Laser/Warning/BP_WarningSquare_Forward.BP_WarningSquare_Forward_C" (Math|Transform|MakeTransform "0, 0, 0" "0, 0, 0" "1.000000,1.000000,1.000000") "Undefined" "MultiplyWithRoot" 0 false 0))
      (Variables|Default|SetAttackWarning%20Ref _returnvalue))))

(event EventTick
  (params (DeltaSeconds :type Float%20%28single-precision%29))
  (bind _bpc_playerstats (Variables|Default|GetBPC_PlayerStats))
  ;[1 1 1] Healing
  (if (Variables|/Game/ThirdPerson/Blueprints/BP_ThirdPersonCharacter.BP_ThirdPersonCharacter_C|GetInPresent (Variables|Default|GetPlayerRef))
    (if (<= (Variables|/Game/ThirdPerson/Blueprints/BPC_PlayerStats.BPC_PlayerStats_C|GetCurrentHealth _bpc_playerstats) (Variables|/Game/ThirdPerson/Blueprints/BPC_PlayerStats.BPC_PlayerStats_C|GetMaxHealth _bpc_playerstats))
      (Default|DecreaseHealth (Variables|Default|GetBPC_PlayerStats) (* (Variables|Default|GetHealthRegen) (Utilities|Time|GetWorldDeltaSeconds))))
    (else
      (Default|ResetHealthBarOrion (Variables|Default|GetHealthBar)))))

(event Game|Damage|EventAnyDamage
  (params (Damage :type Float%20%28single-precision%29) (DamageType :type Damage%20Type%20Object%20Reference) (InstigatedBy :type Controller%20Object%20Reference) (DamageCauser :type Actor%20Object%20Reference))
  (bind _returnvalue (Game|GetPlayerCharacter 0))
  (bind _bpc_playerstats (Variables|Default|GetBPC_PlayerStats))
  (bind _bpc_playerstats_2 (Variables|Default|GetBPC_PlayerStats))
  (bind _bpc_playerstats_3 (Variables|Default|GetBPC_PlayerStats))
  (bind _mesh (Variables|Character|GetMesh))
  (bind _returnvalue_2 (Components|SkeletalMesh|GetAnimInstance _mesh))
  ;[1 1 1] Take Damage & Blocking
  ;;[1 1 1] Block
  (if (Variables|Block|GetIsBlocking)
    (if (<= (Class|KismetMathLibrary|DegAcos (Math|Vector|DotProduct (Transformation|GetActorForwardVector) (Math|Vector|Normalize (- (Transformation|GetActorLocation (Game|GetPlayerCharacter 0)) (Transformation|GetActorLocation))))) (Variables|Block|GetValidBlcokAngle))
      ;;;[1 1 1] Enter QTE
      (Utilities|Time|ClearandInvalidateTimerbyHandle (Variables|Block|GetBlockTimer))
      (Default|CallOnQTE)
      (else
        ;;;[1 1 1] Block Failed
        (CallFunction|EndBlockAnim)
        (Animation|Montage|PlayMontage (Variables|Character|GetMesh) "/Game/Art/Characters/Orion/Animations/AnimMontage/AM_Block_Fail.AM_Block_Fail" 0.5
          (:OnCompleted
            (CallFunction|StartTracingTarget _returnvalue)
            (CallFunction|Dodge true _returnvalue)
            (Default|CallOnActionEnd)))))
    (elif (Variables|/Game/ThirdPerson/Blueprints/BPC_PlayerStats.BPC_PlayerStats_C|GetCanTakeDamage (Variables|Default|GetBPC_PlayerStats))
      (if (and (<= (- (Variables|/Game/ThirdPerson/Blueprints/BPC_PlayerStats.BPC_PlayerStats_C|GetCurrentHealth _bpc_playerstats_3) Damage) (/ (Variables|/Game/ThirdPerson/Blueprints/BPC_PlayerStats.BPC_PlayerStats_C|GetMaxHealth _bpc_playerstats_3) 2.0)) (not (Variables|State|GetHalfHPCheck)))
        ;;[1 1 1] Notify Director if reach half health
        (Variables|State|SetHalfHPCheck true)
        (Variables|/Game/ThirdPerson/Blueprints/BPC_PlayerStats.BPC_PlayerStats_C|SetCurrentHealth _bpc_playerstats_2 (/ (Variables|/Game/ThirdPerson/Blueprints/BPC_PlayerStats.BPC_PlayerStats_C|GetMaxHealth _bpc_playerstats_2) 2.0))
        (Default|UpdateHealthBar (Variables|Default|GetHealthBar))
        (Default|CallOnHalfHealth)
        (else
          ;;[1 1 1] Take Damage
          (bind _isplayerdead (Default|DecreaseHealth (Variables|Default|GetBPC_playerStats) Damage))
          (if _isplayerdead
            ;;[1 1 1] Dead
            (Utilities|FlowControl|DoOnce false
              (:Completed
                (Default|CallOnDeath)
                (Variables|State|SetIsDead true)
                (Animation|Montage|MontageStop _returnvalue_2 0.0 (Animation|Montage|GetCurrentActiveMontage _returnvalue_2))
                (Components|Movement|StopMovementImmediately (Variables|Character|GetCharacterMovement))
                (CallFunction|StopTracingTarget)
                (bind _asabp_orion (Utilities|Casting|CastToABP_Orion (Components|SkeletalMesh|GetAnimInstance (Variables|Character|GetMesh))))
                (Variables|/Game/Enemies/Boss/FinalBoss/Orion/ABP_Orion.ABP_Orion_C|SetIsDead _asabp_orion true)
                (Variables|State|SetCurrentState "NewEnumerator7")))
            (else
              (Variables|/Game/ThirdPerson/Blueprints/BPC_PlayerStats.BPC_PlayerStats_C|SetCanTakeDamage _bpc_playerstats false)
              (Default|UpdateHealthBar (Variables|Default|GetHealthBar))
              (Utilities|FlowControl|Delay 0.3)
              (Variables|/Game/ThirdPerson/Blueprints/BPC_PlayerStats.BPC_PlayerStats_C|SetCanTakeDamage _bpc_playerstats true))))))))

(fn ConstructionScript
  (Components|SkinnedMesh|SetLeaderPoseComponent (Variables|Default|GetSword) (Variables|Character|GetMesh) false false))

(fn BICanbeTarget?
  (return true))

(fn BIMinDistance
  (return false 0.0))

(fn BIonSelectedTarget
  (return false))

(fn BISetCustomTarget
  (params (CustomTarget :type Actor%20Object%20Reference))
  (return false))