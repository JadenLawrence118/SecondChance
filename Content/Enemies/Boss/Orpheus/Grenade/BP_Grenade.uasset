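; Orpheus boss grenade that flies to a ground target, then electrocutes the area for a set time.
; A timeline lerps the mesh on separate XY and Z curves, with duration scaled by distance, while a child-actor telegraph circle counts down at the target.
; A Held/Moving/Electrocuting/Idle state routes Pause and Continue to the active part.
; BeginPlay also auto-throws at the player's feet after a delay.
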(event Custom|TrajectoryToDestin
  (params (Start%20Loc :type Vector) (Destination :type Vector) (IsThowing :type Boolean))
  (bind _returnvalue (Math|Vector|Distance2D(Vector) Destination Start%20Loc))
  (bind (_x _y _z) (Math|Vector|BreakVector Start%20Loc))
  (bind (_x_2 _y_2 _z_2) (Math|Vector|BreakVector Destination))
  (bind _movingspeed_unit_per_sec_ (Variables|Default|GetMovingSpeed%28unit%20per%20sec%29))
  (bind _telegraphcircle (Variables|Default|GetTelegraphCircle))
  (bind _returnvalue_2 (/ _returnvalue _movingspeed_unit_per_sec_))
  (Rendering|SetVisibility (Variables|Default|GetStaticMesh) true false)
  (if IsThowing
    ;[1 1 1] The time of grende projectile motion
    (Components|Timeline|SetPlayRate (Variables|Default|GetMoveToDestination) (/ 1.0 _returnvalue_2))
    (Transformation|SetWorldLocation _telegraphcircle Destination false false)
    (Transformation|SetWorldLocation (Variables|Default|GetElectrocuteArea) Destination false false)
    (Class|BPITelegraph|Start(Message) (Variables|/Script/Engine.ChildActorComponent|GetChildActor _telegraphcircle) _returnvalue_2)
    (Variables|Default|SetState "NewEnumerator2")
    (bind (_direction _x_y_movement _z_movement) (Timeline|MoveToDestination PlayFromStart)
      (:Update
        (Transformation|SetWorldLocation (Variables|Default|GetStaticMesh) (Math|Vector|MakeVector (Math|Float|Lerp _x _x_2 _x_y_movement) (Math|Float|Lerp _y _y_2 _x_y_movement) (Math|Float|Lerp _z _z_2 _z_movement)) false false))
      (:Finished
        (Rendering|SetVisibility (Variables|Default|GetStaticMesh) false false)
        (Class|BPITelegraph|Reset(Message) (Variables|/Script/Engine.ChildActorComponent|GetChildActor (Variables|Default|GetTelegraphCircle)))
        (Class|BPIBossAreaAttack|Activate(Message) (Variables|/Script/Engine.ChildActorComponent|GetChildActor (Variables|Default|GetElectrocuteArea)))
        (Utilities|Time|SetTimerbyEvent (delegate Custom|ElectrocuteEnd) (Variables|Default|GetActivateTime))
        (Variables|Default|SetState "NewEnumerator3")))))

(event Custom|ElectrocuteEnd
  (Class|BPIBossAreaAttack|Deactivate(Message) (Variables|/Script/Engine.ChildActorComponent|GetChildActor (Variables|Default|GetElectrocuteArea)))
  (Variables|Default|SetState "NewEnumerator0"))

(event EventBeginPlay
  (Class|BPIBossAreaAttack|Deactivate(Message) (Variables|/Script/Engine.ChildActorComponent|GetChildActor (Variables|Default|GetElectrocuteArea)))
  (Class|BPITelegraph|Reset(Message) (Variables|/Script/Engine.ChildActorComponent|GetChildActor (Variables|Default|GetTelegraphCircle)))
  (Utilities|FlowControl|Delay 5.0)
  (bind _returnvalue (Actor|GetActorOfClass "/Game/ThirdPerson/Blueprints/BP_ThirdPersonCharacter.BP_ThirdPersonCharacter_C"))
  (Development|PrintString (Utilities|String|ToString(Vector) (Transformation|GetActorLocation _returnvalue)))
  (CallFunction|TrajectorytoDestin (Transformation|GetWorldLocation (Variables|Default|GetStaticMesh)) (- (Transformation|GetActorLocation _returnvalue) "0.000000,0.000000,88.000000") true))

(event Collision|EventActorBeginOverlap
  (params (OtherActor :type Actor%20Object%20Reference)))

(event EventTick
  (params (DeltaSeconds :type Float%20%28single-precision%29)))

(fn ConstructionScript)

(fn Pause
  (switch Utilities|FlowControl|Switch|SwitchonS_GrenadeState (Variables|Default|GetState)
    (:NewEnumerator1
      (Class|BPITelegraph|Pause(Message) (Variables|Default|GetTelegraphCircle)))
    (:NewEnumerator2
      (Audio|Components|Audio|Stop (Variables|Default|GetMoveToDestination)))
    (:NewEnumerator3
      (Class|BPIBossAreaAttack|Pause(Message) (Variables|Default|GetElectrocuteArea)))))

(fn Continue
  (switch Utilities|FlowControl|Switch|SwitchonS_GrenadeState (Variables|Default|GetState)
    (:NewEnumerator1
      (Class|BPITelegraph|Continue(Message) (Variables|Default|GetTelegraphCircle)))
    (:NewEnumerator2
      (Audio|Components|Audio|Play (Variables|Default|GetMoveToDestination)))
    (:NewEnumerator3
      (Class|BPIBossAreaAttack|Continue(Message) (Variables|Default|GetElectrocuteArea)))))

(fn HeldatHand
  (params (SpawnPos :type Vector))
  (bind _staticmesh (Variables|Default|GetStaticMesh))
  (Transformation|SetWorldLocation _staticmesh SpawnPos false false)
  (Rendering|SetVisibility _staticmesh true false)
  (Variables|Default|SetState "NewEnumerator1"))