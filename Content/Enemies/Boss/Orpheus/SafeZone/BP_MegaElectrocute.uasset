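; BP_MegaElectrocute is an electrocution attack for the Orpheus boss that pairs a damage area with a safe zone.
; Warning starts the damage telegraph for the warning time and activates the safe zone, then Activate clears the telegraph and turns on the damage area.
; A timer calls Reset after the active time, switching off both zones and broadcasting that the attack has ended.
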(event Custom|Activate
  (Class|BPITelegraph|Reset(Message) (Variables|Default|GetDamageZoneTelegraph))
  (Class|BPIBossAreaAttack|Activate(Message) (Variables|Default|GetDamageArea))
  (bind _returnvalue (Utilities|Time|SetTimerbyEvent (delegate Custom|Reset) (Variables|Default|GetActivateTime)))
  (Variables|Default|SetTimer _returnvalue))

(event Custom|Warning
  (params (WarningTime :type Float%20%28double-precision%29))
  (Class|BPITelegraph|Start(Message) (Variables|Default|GetDamageZoneTelegraph) WarningTime)
  (Class|BPIBossAreaAttack|Activate(Message) (Variables|Default|GetSafeZone)))

(event Custom|Reset
  (Class|BPIBossAreaAttack|Deactivate(Message) (Variables|Default|GetDamageArea))
  (Class|BPIBossAreaAttack|Deactivate(Message) (Variables|Default|GetSafeZone))
  (Utilities|Time|ClearandInvalidateTimerbyHandle (Variables|Default|GetTimer))
  (Default|CallOnAttackEnd))

(event EventBeginPlay
  (Class|BPITelegraph|Reset(Message) (Variables|Default|GetDamageZoneTelegraph))
  (Class|BPIBossAreaAttack|Deactivate(Message) (Variables|Default|GetSafeZone))
  (Class|BPIBossAreaAttack|Deactivate(Message) (Variables|Default|GetDamageArea)))

(event Collision|EventActorBeginOverlap
  (params (OtherActor :type Actor%20Object%20Reference)))

(event EventTick
  (params (DeltaSeconds :type Float%20%28single-precision%29)))

(fn ConstructionScript)