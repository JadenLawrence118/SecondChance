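; BP_PushOutCylinder is an actor in the Megaera boss folder, apparently meant to toggle a collision cylinder with the player's present/past state.
; BeginPlay caches the player character, and Tick is empty.
; Disconnected logic would watch the player's InPresent flag, enabling Cylinder collision in the present and disabling it after a short delay in the past.
; That logic never runs, and its GetActorOfClass lookups show no class.
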(event EventBeginPlay
  (bind _asbp_third_person_character (Utilities|Casting|CastToBP_ThirdPersonCharacter (Game|GetPlayerCharacter 0)))
  (Variables|Default|SetPlayerRef _asbp_third_person_character))

(event EventTick
  (params (DeltaSeconds :type Float%20%28single-precision%29)))

(fn ConstructionScript)