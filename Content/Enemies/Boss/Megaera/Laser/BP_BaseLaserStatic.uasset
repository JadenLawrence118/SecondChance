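; Base laser hazard for the Megaera boss that damages the player while its LaserShape is visible and overlapping the player's hitbox.
; Overlap events on components tagged PlayerHitBox track contact, and Tick applies damage every frame, or once per contact when ShouldDmgOnce is set.
; The construction script applies a configurable material and scale, and SetVisible toggles the shape, which also switches damage on or off.
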(event OnComponentBeginOverlap(LaserShape)
  (params (OverlappedComponent :type Primitive%20Component%20Object%20Reference) (OtherActor :type Actor%20Object%20Reference) (OtherComp :type Primitive%20Component%20Object%20Reference) (OtherBodyIndex :type Integer) (bFromSweep :type Boolean) (SweepResult :type Hit%20Result%20Structure%20%28by%20ref%29))
  (if (Components|ComponentHasTag OtherComp "PlayerHitBox")
    (Variables|Private|SetIsCollidingWithPlayer true)))

(event OnComponentEndOverlap(LaserShape)
  (params (OverlappedComponent :type Primitive%20Component%20Object%20Reference) (OtherActor :type Actor%20Object%20Reference) (OtherComp :type Primitive%20Component%20Object%20Reference) (OtherBodyIndex :type Integer))
  (if (Components|ComponentHasTag OtherComp "PlayerHitBox")
    (Variables|Private|SetIsCollidingWithPlayer false)
    (Variables|Private|SetPlayerTookDmg false)))

(event EventTick
  (params (DeltaSeconds :type Float%20%28single-precision%29))
  (if (and (Rendering|IsVisible (Variables|Default|GetLaserShape)) (Variables|Private|GetIsCollidingWithPlayer))
    (if (not (Variables|Private|GetPlayerTookDmg))
      (Game|Damage|ApplyDamage (Variables|Private|GetPlayerRef) (Variables|Customisation|GetDamage) 0 0)
      (if (Variables|Customisation|GetShouldDmgOnce)
        (Variables|Private|SetPlayerTookDmg true)))))

(event EventBeginPlay
  (bind _asbp_third_person_character (Utilities|Casting|CastToBP_ThirdPersonCharacter (Game|GetPlayerCharacter 0)))
  (Variables|Private|SetPlayerRef _asbp_third_person_character))

(fn ConstructionScript
  (bind _lasershape (Variables|Default|GetLaserShape))
  (Rendering|Material|SetMaterial _lasershape 0 (Variables|Customisation|GetMaterial))
  (Transformation|SetRelativeScale3D _lasershape (Variables|Customisation|GetScaleMultiplyer))
  (if (Variables|Customisation|GetIsStatic)
    _))

(fn SetVisible
  (params (Visible :type Boolean))
  (Rendering|SetVisibility (Variables|Default|GetLaserShape) Visible false))