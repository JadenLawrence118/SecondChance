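; Base warning indicator actor for Megaera's boss laser attack, hidden at spawn while a 2D lock-on sound starts playing.
; Start shows it, activates two Niagara warning effects and plays a Scaling timeline rate-matched to the warning time, intended to drive MainWarning's XY scale.
; Pause and Continue halt and resume timeline and effects together, while Reset only hides the actor's components.
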(event EventBeginPlay
  (Rendering|SetVisibility (Variables|Default|GetDefaultSceneRoot) false true)
  (bind _returnvalue (Audio|CreateSound2D "/Game/SoundEffects/SoundFX/nmeBossLockOnGrid_FS.nmeBossLockOnGrid_FS" 1.0 1.0 0.0 0))
  (Variables|Default|SetBHWarningSFX _returnvalue)
  (Audio|Components|Audio|Play (Variables|Default|GetBHWarningSFX) 0.0))

(event Collision|EventActorBeginOverlap
  (params (OtherActor :type Actor%20Object%20Reference)))

(event EventTick
  (params (DeltaSeconds :type Float%20%28single-precision%29)))

(event EventStart
  (params (WarningTime%28sec%29 :type Float%20%28double-precision%29))
  (bind _scaling (Variables|Default|GetScaling))
  (Rendering|SetVisibility (Variables|Default|GetDefaultSceneRoot) true true)
  (Components|Activation|Activate (Variables|Default|GetMainWarning) false)
  (Components|Timeline|SetPlayRate _scaling (/ 1.0 WarningTime%28sec%29))
  (Components|Timeline|PlayfromStart _scaling))

(event EventReset
  (Rendering|SetVisibility (Variables|Default|GetDefaultSceneRoot) false true))

(event EventContinue
  (Audio|Components|Audio|Play (Variables|Default|GetScaling))
  (Class|NiagaraComponent|SetPaused (Variables|Default|GetMainWarning) false))

(event EventPause
  (Audio|Components|Audio|Stop (Variables|Default|GetScaling))
  (Class|NiagaraComponent|SetPaused (Variables|Default|GetMainWarning) true))

(fn ConstructionScript)