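; BP_WarningSquare_Forward is a forward-stretching warning marker for the Megaera boss's laser, extending a parent warning actor.
; SetWarningLength rotates the actor from a start location toward a destination and scales its Niagara effect's X axis by their 2D distance.
; Pause, Start, Continue and Reset defer to the parent; all but Start also toggle an UpdateSetLength flag, which this graph never reads.
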(event Custom|Set%20Warning%20Length
  (params (Start%20location :type Vector) (Destination :type Vector))
  (Variables|Default|SetUpdate%20Set%20length true)
  (Transformation|SetRelativeScale3D (Variables|Default|GetNiagaraWarningBase_0) (Math|Vector|MakeVector (/ (Math|Vector|Distance2D(Vector) Destination Start%20location) 2e+02) 1.0 1.0))
  (Transformation|SetActorRotation (Math|Rotator|FindLookatRotation Start%20location Destination)))

(event EventBeginPlay
  (|CallParentFunction) ; This node is disabled and will not be called.\nDrag off pins to build functionality.
)

(event Collision|EventActorBeginOverlap
  (params (OtherActor :type Actor%20Object%20Reference))
  (|CallParentFunction OtherActor) ; This node is disabled and will not be called.\nDrag off pins to build functionality.
)

(event EventTick
  (params (DeltaSeconds :type Float%20%28single-precision%29))
  (|CallParentFunction DeltaSeconds))

(event EventPause
  (|CallParentFunction)
  (Variables|Default|SetUpdate%20Set%20length false))

(event EventStart
  (params (WarningTime%28sec%29 :type Float%20%28double-precision%29))
  (|CallParentFunction WarningTime%28sec%29))

(event EventContinue
  (|CallParentFunction)
  (Variables|Default|SetUpdate%20Set%20length true))

(event EventReset
  (|CallParentFunction)
  (Variables|Default|SetUpdate%20Set%20length false))

(fn ConstructionScript
  (|CallParentFunction))