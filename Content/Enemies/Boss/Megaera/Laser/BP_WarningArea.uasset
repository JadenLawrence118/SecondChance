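; Warning area telegraph for the laser of the Megaera boss, showing a Niagara grid that scales over a given warning time.
; Activate reveals the pivot hierarchy, starts the effect and replays the MainScaling timeline, with play rate set to the inverse of the warning time.
; The timeline drives the moving grid's X and Y scale.
; Deactivate hides it and flattens that scale, while Pause and Continue freeze and resume both timeline and effect.
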(event EventBeginPlay)

(event Collision|EventActorBeginOverlap
  (params (OtherActor :type Actor%20Object%20Reference)))

(event EventTick
  (params (DeltaSeconds :type Float%20%28single-precision%29)))

(fn ConstructionScript)

(fn Activate
  (params (Warning%20Time :type Float%20%28double-precision%29))
  (Components|Timeline|SetPlayRate (Variables|Default|GetMainScaling) (/ 1.0 Warning%20Time))
  (Components|Activation|Activate (Variables|Default|GetNiagara) false)
  (Rendering|SetVisibility (Variables|Default|GetPivot%20Point) true true)
  (Components|Timeline|PlayfromStart (Variables|Default|GetMainScaling))
  (Variables|Default|SetIsOn true))

(fn Deactivate
  (Rendering|SetVisibility (Variables|Default|GetPivot%20Point) false true)
  (Transformation|SetRelativeScale3D (Variables|Default|GetVFX_WarningGrid_Moving) "0.000000,0.000000,1.000000")
  (Variables|Default|SetIsOn false))

(fn Pause
  (Audio|Components|Audio|Stop (Variables|Default|GetMainScaling))
  (Class|NiagaraComponent|SetPaused (Variables|Default|GetNiagara) true))

(fn Continue
  (Audio|Components|Audio|Play (Variables|Default|GetMainScaling))
  (Class|NiagaraComponent|SetPaused (Variables|Default|GetNiagara) false))