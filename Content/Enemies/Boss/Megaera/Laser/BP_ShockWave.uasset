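; Expanding shockwave attack in the Megaera boss's laser set, hidden and without collision until fired.
; Fire shows the shape with query-only collision, starts Niagara and runs a timeline that scales it outward in X and Y.
; When the timeline finishes, Reset hides the shape, disables collision, zeroes its XY scale and stops the effect.
; It follows the player's time-change event, freezing via CustomTimeDilation while in the present.
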(event Custom|OnTimeChange_Event
  (params (InPresent :type Boolean))
  (if InPresent
    (Variables|Default|SetCustomTimeDilation 0.0)
    (else
      (Variables|Default|SetCustomTimeDilation 1.0))))

(event Custom|Fire
  (bind _lasershape (Variables|Default|GetLaserShape))
  (Collision|SetCollisionEnabled _lasershape "QueryOnly")
  (Rendering|SetVisibility _lasershape true false)
  (Components|Activation|Activate (Variables|Default|GetNiagara) false)
  (bind _size (Timeline|Timeline PlayFromStart)
    (:Update
      (Transformation|SetRelativeScale3D (Variables|Default|GetLaserShape) (Math|Vector|MakeVector _size _size 1.0)))
    (:Finished
      (CallFunction|Reset))))

(event EventBeginPlay
  (|CallParentFunction)
  (EventDispatchers|AssignOnTimeChange (Variables|Default|GetPlayerRef) (EventDispatchers|CreateEvent :!event Custom|OnTimeChange_Event))
  (Collision|SetCollisionEnabled (Variables|Default|GetLaserShape) "NoCollision")
  (Rendering|SetVisibility (Variables|Default|GetLaserShape) false false))

(event EventTick
  (params (DeltaSeconds :type Float%20%28single-precision%29))
  (|CallParentFunction DeltaSeconds) ; This node is disabled and will not be called.\nDrag off pins to build functionality.
)

(fn ConstructionScript)

(fn Reset
  (bind _lasershape (Variables|Default|GetLaserShape))
  (Collision|SetCollisionEnabled _lasershape "NoCollision")
  (Rendering|SetVisibility _lasershape false false)
  (Transformation|SetRelativeScale3D _lasershape (Math|Vector|MakeVector 0.0 0.0 1.0))
  (Components|Activation|Deactivate (Variables|Default|GetNiagara)))