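; BP_BulletHellLaser is a reusable laser projectile, filed under the Megaera boss, that stays hidden and collisionless until fired.
; Fire shows LaserShape, enables query-only collision and sends ProjectileMovement along the shape's up vector at LaserSpeed.
; Reset stops movement, hides the shape, disables collision and moves the actor to a given location, so one instance can be fired again.
; A scale timeline and delayed TurnOnLaser call are left unconnected.
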(event Custom|TurnOnLaser
  (Rendering|SetVisibility (Variables|Default|GetLaserShape) true false))

(event EventBeginPlay
  (|CallParentFunction)
  (Rendering|SetVisibility (Variables|Default|GetLaserShape) false false)
  (Collision|SetCollisionEnabled (Variables|Default|GetLaserShape) "NoCollision"))

(event Collision|EventActorBeginOverlap
  (params (OtherActor :type Actor%20Object%20Reference)))

(event EventTick
  (params (DeltaSeconds :type Float%20%28single-precision%29))
  (|CallParentFunction DeltaSeconds) ; This node is disabled and will not be called.\nDrag off pins to build functionality.
)

(fn ConstructionScript
  (|CallParentFunction))

(fn Fire
  (bind _lasershape (Variables|Default|GetLaserShape))
  (Rendering|SetVisibility _lasershape true false)
  (Collision|SetCollisionEnabled _lasershape "QueryOnly")
  (Variables|/Script/Engine.MovementComponent|SetVelocity (Variables|Default|GetProjectileMovement) (* (Math|Vector|GetUpVector _lasershape) (Variables|Default|GetLaserSpeed))))

(fn Reset
  (params (ResetLocation :type Vector))
  (bind _lasershape (Variables|Default|GetLaserShape))
  (Variables|/Script/Engine.MovementComponent|SetVelocity (Variables|Default|GetProjectileMovement) "0, 0, 0")
  (Collision|SetCollisionEnabled _lasershape "NoCollision")
  (Rendering|SetVisibility _lasershape false false)
  (Transformation|SetActorLocation ResetLocation false false))