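; Megaera boss bullet-hell attack that fires a laser grid in two alternating, checkerboard-style waves.
; BeginPlay spawns paired, deactivated warning and laser areas per cell and binds to the boss's start, pause and unpause events.
; Chained timers run warning then laser for each index-parity set, then clear CanUseBulletHell and signal the boss that the attack finished.
; Boss pause events freeze the timer and active areas, while Tick pauses sounds whenever the player is InPresent.
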(event Custom|Attack1
  (bind _chargingtime (Variables|Default|GetChargingTime))
  ;[1 1 1] Starts the 1 attack then calls the second one when the first is over
  (CallFunction|Turnon1Warnings _chargingtime)
  (bind _returnvalue (Utilities|Time|SetTimerbyEvent (delegate Custom|Turn%20on%201Laser) _chargingtime))
  (Variables|Default|SetTimer _returnvalue))

(event Custom|Attack2
  (bind _chargingtime (Variables|Default|GetChargingTime))
  (CallFunction|Turnon2Warnings _chargingtime)
  (bind _returnvalue (Utilities|Time|SetTimerbyEvent (delegate Custom|Laser2%20Turn%20On) _chargingtime))
  (Variables|Default|SetTimer _returnvalue))

(event Custom|Turn%20on%201Laser
  ;[1 1 1] Starts the 1 attack then calls the second one when the first is over
  (Utilities|Time|ClearandInvalidateTimerbyHandle (Variables|Default|GetTimer))
  (CallFunction|TurnOffWarning)
  (CallFunction|Turnon1Lasers)
  (bind _returnvalue (Utilities|Time|SetTimerbyEvent (delegate Custom|Laser1%20Ended) (Variables|Default|GetAttackTime)))
  (Variables|Default|SetTimer _returnvalue))

(event Custom|Laser1%20Ended
  ;[1 1 1] Starts the 1 attack then calls the second one when the first is over
  (CallFunction|TurnOffAttack)
  (Utilities|Time|ClearandInvalidateTimerbyHandle (Variables|Default|GetTimer))
  (CallFunction|Attack2))

(event Custom|Laser2%20Turn%20On
  (Utilities|Time|ClearandInvalidateTimerbyHandle (Variables|Default|GetTimer))
  (CallFunction|TurnOffWarning)
  (CallFunction|Turnon2Lasers)
  (bind _returnvalue (Utilities|Time|SetTimerbyEvent (delegate Custom|Laser2%20Ended) (Variables|Default|GetAttackTime)))
  (Variables|Default|SetTimer _returnvalue))

(event Custom|Laser2%20Ended
  (bind _owningbossactor (Variables|Default|GetOwningBossActor))
  (CallFunction|TurnOffAttack)
  (Utilities|Time|ClearandInvalidateTimerbyHandle (Variables|Default|GetTimer))
  (Variables|/Game/Enemies/Boss/Megaera/BP_Megaera.BP_Megaera_C|SetCanUseBulletHell _owningbossactor false)
  (Default|CallOnFinishAttack _owningbossactor))

(event Custom|OnPause_Event
  (Utilities|Time|PauseTimerbyHandle (Variables|Default|GetTimer))
  (if (Variables|Default|GetIsWarning)
    (for _array_element (Variables|Default|GetWarningAreas)
      (Utilities|IsValid _array_element
        (:Is%20Valid
          (Default|Pause _array_element))))
    (elif (Variables|Default|GetIsAttacking)
      (for _array_element_2 (Variables|Default|GetLaserAreas)
        (Utilities|IsValid _array_element_2
          (:Is%20Valid
            (Default|Pause _array_element_2)))))))

(event Custom|OnUnPause_Event
  (Utilities|Time|UnpauseTimerbyHandle (Variables|Default|GetTimer))
  (if (Variables|Default|GetIsWarning)
    (for _array_element (Variables|Default|GetWarningAreas)
      (Utilities|IsValid _array_element
        (:Is%20Valid
          (Default|Continue _array_element))))
    (elif (Variables|Default|GetIsAttacking)
      (for _array_element_2 (Variables|Default|GetLaserAreas)
        (Utilities|IsValid _array_element_2
          (:Is%20Valid
            (Default|Continue _array_element_2)))))))

(event Custom|OnLaserGridStart_Event
  (CallFunction|Attack1))

(event EventBeginPlay
  (Utilities|FlowControl|Sequence
    (:then_0
      (bind _returnvalue (Actor|GetActorOfClass "/Game/Enemies/Boss/Megaera/BP_Megaera.BP_Megaera_C"))
      (bind _output_get (Variables|Default|SetOwningBossActor _returnvalue))
      (CallFunction|MakeGrid)
      (EventDispatchers|AssignOnLaserGridStart _output_get (EventDispatchers|CreateEvent :!event Custom|OnLaserGridStart_Event))
      (EventDispatchers|AssignOnPause _returnvalue (EventDispatchers|CreateEvent :!event Custom|OnPause_Event))
      (EventDispatchers|AssignOnUnPause _returnvalue (EventDispatchers|CreateEvent :!event Custom|OnUnPause_Event)))
    (:then_1
      (bind _asbp_third_person_character (Utilities|Casting|CastToBP_ThirdPersonCharacter (Game|GetPlayerCharacter 0)))
      (Variables|Default|SetPlayerRef _asbp_third_person_character))))

(event Collision|EventActorBeginOverlap
  (params (OtherActor :type Actor%20Object%20Reference)))

(event EventTick
  (params (DeltaSeconds :type Float%20%28single-precision%29))
  (bind _bhgridwarningsfx (Variables|SFXVariables|GetBHGridWarningSFX))
  (bind _bhgridwarningsfx_2 (Variables|SFXVariables|GetBHGridWarningSFX))
  (bind _bhgridfiresfx (Variables|SFXVariables|GetBHGridFireSFX))
  (bind _bhgridfiresfx_2 (Variables|SFXVariables|GetBHGridFireSFX))
  (if (Variables|/Game/ThirdPerson/Blueprints/BP_ThirdPersonCharacter.BP_ThirdPersonCharacter_C|GetInPresent (Variables|Default|GetPlayerRef))
    (Utilities|FlowControl|Sequence
      (:then_0
        (Utilities|IsValid _bhgridwarningsfx
          (:Is%20Valid
            (Class|AudioComponent|SetPaused _bhgridwarningsfx true))))
      (:then_1
        (Utilities|IsValid _bhgridfiresfx_2
          (:Is%20Valid
            (Class|AudioComponent|SetPaused _bhgridfiresfx_2 true)))))
    (else
      (Utilities|FlowControl|Sequence
        (:then_0
          (Utilities|IsValid _bhgridwarningsfx_2
            (:Is%20Valid
              (Class|AudioComponent|SetPaused _bhgridwarningsfx_2 false))))
        (:then_1
          (Utilities|IsValid _bhgridfiresfx
            (:Is%20Valid
              (Class|AudioComponent|SetPaused _bhgridfiresfx false))))))))

(fn ConstructionScript)

(fn MakeGrid
  (bind _returnvalue (Transformation|GetActorLocation))
  (bind _scale (Variables|Default|GetScale))
  (bind _scale_2 (Variables|Default|GetScale))
  (bind _cellsize (Variables|Default|GetCellSize))
  ;[1 1 1] Create a grid of warning and attacking lasers and add them to an array
  (Utilities|Array|Clear (Variables|Default|GetWarningAreas))
  (Utilities|Array|Clear (Variables|Default|GetLaserAreas))
  (for _index (range 0 (- (Variables|Default|GetRows) 1))
    (for _index_2 (range 0 (- (Variables|Default|GetColumns) 1))
      (bind _returnvalue_2 (Game|SpawnActorfromClass "/Game/Enemies/Boss/Megaera/Laser/Attacks/BulletHell_P2/BP_WarningArea.BP_WarningArea_C" (Math|Transform|MakeTransform (Math|Vector|MakeVector (+ (* _index_2 _cellsize (.x _scale)) (.x _returnvalue)) (+ (* _index _cellsize (.y _scale)) (.y _returnvalue)) (.z _returnvalue)) "0, 0, 0" (Math|Vector|MakeVector (.x _scale_2) (.y _scale_2) 0.1)) "Undefined" "OverrideRootScale" self 0))
      (Default|Deactivate _returnvalue_2)
      (bind _returnvalue_3 (Utilities|Array|Add (Variables|Default|GetWarningAreas) _returnvalue_2))
      (Variables|/Game/Enemies/Boss/Megaera/Laser/Attacks/BulletHell_P2/BP_WarningArea.BP_WarningArea_C|SetArayNum _returnvalue_2 _returnvalue_3)
      (bind _returnvalue_4 (Game|SpawnActorfromClass "/Game/Enemies/Boss/Megaera/Laser/Attacks/BulletHell_P2/BP_LaserArea.BP_LaserArea_C" (Math|Transform|MakeTransform (Math|Vector|MakeVector (+ (* _index_2 _cellsize (.x _scale)) (.x _returnvalue)) (+ (* _index _cellsize (.y _scale)) (.y _returnvalue)) (.z _returnvalue)) "0, 0, 0" (Variables|Default|GetScale)) "Undefined" "OverrideRootScale" self (Variables|Default|GetAttackTime) "1.000000,1.000000,0.500000" "/Game/Enemies/Boss/Megaera/Laser/Materials/MI_Transparent.MI_Transparent" true true (Variables|Default|GetDamage) 0))
      (Default|Deactivate _returnvalue_4)
      (Utilities|Array|Add (Variables|Default|GetLaserAreas) _returnvalue_4))))

(fn TurnOffWarning
  ;[1 1 1] Turning off all the lasers if they are on
  (Variables|Default|SetIsWarning false)
  (for _array_element (Variables|Default|GetWarningAreas)
    (Utilities|IsValid _array_element
      (:Is%20Valid
        (if (Variables|/Game/Enemies/Boss/Megaera/Laser/Attacks/BulletHell_P2/BP_WarningArea.BP_WarningArea_C|GetIsOn _array_element)
          (Default|Deactivate _array_element))))))

(fn IsAlternating
  (params (X :type Integer))
  (bind _rows (Variables|Default|GetRows))
  ;[1 1 1] Checks if the index has to be activated
  (return (== (Math|Integer|%(Integer) (+ (Math|Integer|%(Integer) X _rows) (/ X _rows)) 2) 0)))

(fn Turnon1Lasers
  (Variables|Default|SetIsAttacking true)
  (for (_array_element _array_index) (Variables|Default|GetLaserAreas)
    (bind _isalternating (CallFunction|IsAlternating _array_index))
    (if _isalternating
      (Utilities|IsValid _array_element
        (:Is%20Valid
          (Default|Activate _array_element)
          (bind _returnvalue (Audio|CreateSound2D "/Game/SoundEffects/SoundFX/nmeLaserGrid_FS.nmeLaserGrid_FS" 1.0 1.0 0.0 0))
          (Variables|SFXVariables|SetBHGridFireSFX _returnvalue)
          (Audio|Components|Audio|Play (Variables|SFXVariables|GetBHGridFireSFX) 0.0))))))

(fn Turnon2Lasers
  (Variables|Default|SetIsAttacking true)
  (for (_array_element _array_index) (Variables|Default|GetLaserAreas)
    (bind _isalternating (CallFunction|IsAlternating _array_index))
    (if (not _isalternating)
      (Utilities|IsValid _array_element
        (:Is%20Valid
          (Default|Activate _array_element)
          (bind _returnvalue (Audio|CreateSound2D "/Game/SoundEffects/SoundFX/nmeLaserGrid_FS.nmeLaserGrid_FS" 1.0 1.0 0.0 0))
          (Variables|SFXVariables|SetBHGridFireSFX _returnvalue)
          (Audio|Components|Audio|Play (Variables|SFXVariables|GetBHGridFireSFX) 0.0))))))

(fn Turnon1Warnings
  (params (WarningTime :type Float%20%28double-precision%29))
  (Variables|Default|SetIsWarning true)
  (for (_array_element _array_index) (Variables|Default|GetWarningAreas)
    (bind _isalternating (CallFunction|IsAlternating _array_index))
    (if _isalternating
      (Utilities|IsValid _array_element
        (:Is%20Valid
          (Default|Activate _array_element WarningTime)
          (bind _returnvalue (Audio|CreateSound2D "/Game/SoundEffects/SoundFX/nmeBossLockOnGrid_FS.nmeBossLockOnGrid_FS" 1.0 1.0 0.0 0))
          (Variables|SFXVariables|SetBHGridWarningSFX _returnvalue)
          (Audio|Components|Audio|Play (Variables|SFXVariables|GetBHGridWarningSFX) 0.0))))))

(fn Turnon2Warnings
  (params (Warning%20Time :type Float%20%28double-precision%29))
  (Variables|Default|SetIsWarning true)
  (for (_array_element _array_index) (Variables|Default|GetWarningAreas)
    (bind _isalternating (CallFunction|IsAlternating _array_index))
    (if (not _isalternating)
      (Utilities|IsValid _array_element
        (:Is%20Valid
          (Default|Activate _array_element Warning%20Time)
          (bind _returnvalue (Audio|CreateSound2D "/Game/SoundEffects/SoundFX/nmeBossLockOnGrid_FS.nmeBossLockOnGrid_FS" 1.0 1.0 0.0 0))
          (Variables|SFXVariables|SetBHGridWarningSFX _returnvalue)
          (Audio|Components|Audio|Play (Variables|SFXVariables|GetBHGridWarningSFX) 0.0))))))

(fn TurnOffAttack
  ;[1 1 1] Turning off all the lasers if they are on
  (Variables|Default|SetIsAttacking false)
  (for _array_element (Variables|Default|GetLaserAreas)
    (Utilities|IsValid _array_element
      (:Is%20Valid
        (if (Variables|/Game/Enemies/Boss/Megaera/Laser/Attacks/BulletHell_P2/BP_LaserArea.BP_LaserArea_C|GetIsOn _array_element)
          (Default|Deactivate _array_element))))))