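; Laser wave projectile for the Megaera boss's attacks, built to be reused rather than destroyed.
; Fire places it, enables query collision, visuals and Niagara, launches it along Direction's forward vector and sets a LifeSpan timer naming Reset.
; Reset stops movement, hides the shape, disables collision and effects, and relocates it to a given location.
; The player's time-change event freezes it in the present via CustomTimeDilation and resumes it otherwise.
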(event Custom|OnTimeChange_Event
  (params (InPresent :type Boolean))
  (if InPresent
    (Variables|Default|SetCustomTimeDilation 0.0)
    (else
      (Variables|Default|SetCustomTimeDilation 1.0))))

(event EventBeginPlay
  (|CallParentFunction)
  (EventDispatchers|AssignOnTimeChange (Variables|Default|GetPlayerRef) (EventDispatchers|CreateEvent :!event Custom|OnTimeChange_Event))
  (Collision|SetCollisionEnabled (Variables|Default|GetLaserShape) "NoCollision"))

(event Collision|EventActorBeginOverlap
  (params (OtherActor :type Actor%20Object%20Reference)))

(event EventTick
  (params (DeltaSeconds :type Float%20%28single-precision%29))
  (|CallParentFunction DeltaSeconds))

(fn ConstructionScript
  (|CallParentFunction))

(fn Reset
  (params (NewLocation :type Vector))
  (bind _lasershape (Variables|Default|GetLaserShape))
  (Variables|/Script/Engine.MovementComponent|SetVelocity (Variables|Default|GetProjectileMovement) "0, 0, 0")
  (Collision|SetCollisionEnabled _lasershape "NoCollision")
  (Rendering|SetVisibility _lasershape false false)
  (Transformation|SetActorLocation NewLocation false false)
  (Components|Activation|Deactivate (Variables|Default|GetNiagara)))

(fn Fire
  (params (Fire%20Location :type Vector) (Fire%20Rotation :type Rotator))
  (bind _lasershape (Variables|Default|GetLaserShape))
  (Transformation|SetActorLocationAndRotation Fire%20Location Fire%20Rotation)
  (Collision|SetCollisionEnabled _lasershape "QueryOnly")
  (Rendering|SetVisibility _lasershape true false)
  (Components|Activation|Activate (Variables|Default|GetNiagara) false)
  (Variables|/Script/Engine.MovementComponent|SetVelocity (Variables|Default|GetProjectileMovement) (* (Math|Vector|GetForwardVector (Variables|Default|GetDirection)) (Variables|Default|GetWaveSpeed)))
  (Utilities|Time|SetTimerbyFunctionName 0 "Reset" (Variables|Default|GetLifeSpan)))