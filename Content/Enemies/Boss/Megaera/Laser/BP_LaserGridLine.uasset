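; One line of the Megaera boss laser grid, pairing two BP_BulletHellLaser child actors with a visual indicator.
; The construction script places each laser at its start marker, and BeginPlay caches the laser references after a short delay.
; Ready shows the indicator and Fire hides it and fires both lasers.
; Reset returns lasers to their markers, SetDamage sets their damage, and TimeStop freezes or resumes them through custom time dilation.
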(event EventBeginPlay
  (Utilities|FlowControl|Sequence
    (:then_0
      (Rendering|SetVisibility (Variables|Default|GetIndicator) false false))
    (:then_1
      (Utilities|FlowControl|Delay 0.2)
      (Utilities|FlowControl|Sequence
        (:then_0
          (bind _asbp_bullet_hell_laser (Utilities|Casting|CastToBP_BulletHellLaser (Variables|/Script/Engine.ChildActorComponent|GetChildActor (Variables|Default|GetLaser1)))
            (:then
              (Variables|Default|SetBP%20Bullet%20Hell%20Laser1 _asbp_bullet_hell_laser))
            (:CastFailed
              (Development|PrintString "BP_Bullet_Hell_Laser cast failed" :!label _label))))
        (:then_1
          (bind _asbp_bullet_hell_laser_2 (Utilities|Casting|CastToBP_BulletHellLaser (Variables|/Script/Engine.ChildActorComponent|GetChildActor (Variables|Default|GetLaser2)))
            (:then
              (Variables|Default|SetBP%20Bullet%20Hell%20Laser2 _asbp_bullet_hell_laser_2))
            (:CastFailed
              (goto _label))))))))

(event Collision|EventActorBeginOverlap
  (params (OtherActor :type Actor%20Object%20Reference)))

(event EventTick
  (params (DeltaSeconds :type Float%20%28single-precision%29)))

(fn ConstructionScript
  (Transformation|SetActorLocation (Variables|/Script/Engine.ChildActorComponent|GetChildActor (Variables|Default|GetLaser1)) (Transformation|GetWorldLocation (Variables|Default|GetLaser1%20StartPos)) false false)
  (Transformation|SetActorLocation (Variables|/Script/Engine.ChildActorComponent|GetChildActor (Variables|Default|GetLaser2)) (Transformation|GetWorldLocation (Variables|Default|GetLaser%202%20StartPos)) false false))

(fn Ready
  (Rendering|SetVisibility (Variables|Default|GetIndicator) true false))

(fn Fire
  (Rendering|SetVisibility (Variables|Default|GetIndicator) false false)
  (Default|Fire (Variables|Default|GetBP%20Bullet%20Hell%20Laser1))
  (Default|Fire (Variables|Default|GetBP%20Bullet%20Hell%20Laser2)))

(fn TimeStop
  (params (In%20Present :type Boolean))
  (bind _laser1 (Variables|Default|GetLaser1))
  (bind _laser2 (Variables|Default|GetLaser2))
  (bind _childactor (Variables|/Script/Engine.ChildActorComponent|GetChildActor _laser1))
  (bind _childactor_2 (Variables|/Script/Engine.ChildActorComponent|GetChildActor _laser2))
  (if In%20Present
    (Variables|/Script/Engine.Actor|SetCustomTimeDilation _childactor 0.0)
    (Variables|/Script/Engine.Actor|SetCustomTimeDilation _childactor_2 0.0)
    (else
      (Variables|/Script/Engine.Actor|SetCustomTimeDilation _childactor 1.0)
      (Variables|/Script/Engine.Actor|SetCustomTimeDilation _childactor_2 1.0))))

(fn Reset
  (bind _asbp_bullet_hell_laser (Utilities|Casting|CastToBP_BulletHellLaser (Variables|/Script/Engine.ChildActorComponent|GetChildActor (Variables|Default|GetLaser1))))
  (bind _asbp_bullet_hell_laser_2 (Utilities|Casting|CastToBP_BulletHellLaser (Variables|/Script/Engine.ChildActorComponent|GetChildActor (Variables|Default|GetLaser2))))
  (Default|Reset _asbp_bullet_hell_laser (Transformation|GetWorldLocation (Variables|Default|GetLaser1%20StartPos)))
  (Default|Reset _asbp_bullet_hell_laser_2 (Transformation|GetWorldLocation (Variables|Default|GetLaser%202%20StartPos))))

(fn SetDamage
  (params (Damage :type Float%20%28double-precision%29))
  (Utilities|FlowControl|Sequence
    (:then_0
      (bind _asbp_bullet_hell_laser (Utilities|Casting|CastToBP_BulletHellLaser (Variables|/Script/Engine.ChildActorComponent|GetChildActor (Variables|Default|GetLaser1))))
      (Variables|/Game/Enemies/Boss/Megaera/Laser/BP_BaseLaser.BP_BaseLaser_C|SetDamage _asbp_bullet_hell_laser Damage))
    (:then_1
      (bind _asbp_bullet_hell_laser_2 (Utilities|Casting|CastToBP_BulletHellLaser (Variables|/Script/Engine.ChildActorComponent|GetChildActor (Variables|Default|GetLaser2))))
      (Variables|/Game/Enemies/Boss/Megaera/Laser/BP_BaseLaser.BP_BaseLaser_C|SetDamage _asbp_bullet_hell_laser_2 Damage))))