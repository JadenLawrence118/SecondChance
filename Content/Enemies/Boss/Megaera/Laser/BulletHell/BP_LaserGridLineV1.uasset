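; BP_LaserGridLineV1 is one line of a boss bullet-hell laser grid, built around a pair of BP_BulletHellLaserV2 actors.
; BeginPlay hides the warning VFX and spawns both lasers once at start-position markers, and they are reused afterwards.
; Ready shows the warning, resets the lasers to their markers and plays a lock-on sound; Fire clears the warning and launches both.
; Time Stop freezes them through CustomTimeDilation, and Set Damage updates both.
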(event EventBeginPlay
  (bind _laser_2_startpos (Variables|Default|GetLaser%202%20StartPos))
  (bind _laser1_startpos (Variables|Default|GetLaser1%20StartPos))
  (Utilities|FlowControl|Sequence
    (:then_0
      (Rendering|SetVisibility (Variables|Default|GetWarningVFX) false false))
    (:then_1
      (bind _returnvalue (Game|SpawnActorfromClass "/Game/Enemies/Boss/Megaera/Laser/BulletHell/BP_BulletHellLaserV2.BP_BulletHellLaserV2_C" (Math|Transform|MakeTransform (Transformation|GetWorldLocation _laser1_startpos) (Transformation|GetWorldRotation _laser1_startpos) "1.000000,1.000000,1.000000") "Undefined" "MultiplyWithRoot" 0 "1.000000,1.000000,1.000000" "/Game/Enemies/Boss/Megaera/Laser/Materials/MI_Transparent.MI_Transparent" false true (Variables|Default|GetBulletDamage) 0))
      (Variables|Default|SetBP%20Bullet%20Hell%20Laser1 _returnvalue)
      (bind _returnvalue_2 (Game|SpawnActorfromClass "/Game/Enemies/Boss/Megaera/Laser/BulletHell/BP_BulletHellLaserV2.BP_BulletHellLaserV2_C" (Math|Transform|MakeTransform (Transformation|GetWorldLocation _laser_2_startpos) (Transformation|GetWorldRotation _laser_2_startpos) "1.000000,1.000000,1.000000") "Undefined" "MultiplyWithRoot" 0 "1.000000,1.000000,1.000000" "/Game/Enemies/Boss/Megaera/Laser/Materials/MI_Transparent.MI_Transparent" false true (Variables|Default|GetBulletDamage) 0))
      (Variables|Default|SetBP%20Bullet%20Hell%20Laser2 _returnvalue_2))))

(event Collision|EventActorBeginOverlap
  (params (OtherActor :type Actor%20Object%20Reference)))

(event EventTick
  (params (DeltaSeconds :type Float%20%28single-precision%29)))

(fn ConstructionScript)

(fn Ready
  (Rendering|SetVisibility (Variables|Default|GetWarningVFX) true false)
  (Components|Activation|Activate (Variables|Default|GetWarningVFX) false)
  (CallFunction|SetBulletLocation)
  (Audio|PlaySound2D "/Game/SoundEffects/SoundFX/nmeBossLockOnGrid_FS.nmeBossLockOnGrid_FS" 1.0 1.0 0.0 0 0))

(fn Fire
  (bind _warningvfx (Variables|Default|GetWarningVFX))
  (Components|Activation|Deactivate _warningvfx)
  (Rendering|SetVisibility _warningvfx false false)
  (Default|Fire (Variables|Default|GetBP%20Bullet%20Hell%20Laser1))
  (Default|Fire (Variables|Default|GetBP%20Bullet%20Hell%20Laser2)))

(fn TimeStop
  (params (In%20Present :type Boolean))
  (bind _bp_bullet_hell_laser1 (Variables|Default|GetBP%20Bullet%20Hell%20Laser1))
  (bind _bp_bullet_hell_laser2 (Variables|Default|GetBP%20Bullet%20Hell%20Laser2))
  (if In%20Present
    (Variables|/Script/Engine.Actor|SetCustomTimeDilation _bp_bullet_hell_laser1 0.0)
    (Variables|/Script/Engine.Actor|SetCustomTimeDilation _bp_bullet_hell_laser2 0.0)
    (else
      (Variables|/Script/Engine.Actor|SetCustomTimeDilation _bp_bullet_hell_laser1 1.0)
      (Variables|/Script/Engine.Actor|SetCustomTimeDilation _bp_bullet_hell_laser2 1.0))))

(fn SetBulletLocation
  (bind _laser1_startpos (Variables|Default|GetLaser1%20StartPos))
  (bind _laser_2_startpos (Variables|Default|GetLaser%202%20StartPos))
  (Default|Reset (Variables|Default|GetBP%20Bullet%20Hell%20Laser1) (Transformation|GetWorldLocation _laser1_startpos) (Transformation|GetWorldRotation _laser1_startpos))
  (Default|Reset (Variables|Default|GetBP%20Bullet%20Hell%20Laser2) (Transformation|GetWorldLocation _laser_2_startpos) (Transformation|GetWorldRotation _laser_2_startpos)))

(fn SetDamage
  (params (Damage :type Float%20%28double-precision%29))
  (Variables|/Game/Enemies/Boss/Megaera/Laser/BulletHell/BP_BulletHellLaserV2.BP_BulletHellLaserV2_C|SetDamage (Variables|Default|GetBP%20Bullet%20Hell%20Laser1) Damage)
  (Variables|/Game/Enemies/Boss/Megaera/Laser/BulletHell/BP_BulletHellLaserV2.BP_BulletHellLaserV2_C|SetDamage (Variables|Default|GetBP%20Bullet%20Hell%20Laser2) Damage))