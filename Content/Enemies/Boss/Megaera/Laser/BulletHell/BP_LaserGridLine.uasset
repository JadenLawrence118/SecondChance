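; BP_LaserGridLine is one laser line for the Megaera boss's bullet-hell laser grid, driven through Ready, Fire and Reset.
; Ready shows a warning effect with a lock-on sound; Fire swaps it for the child BP_LaserBeam2, two Niagara effects and a burst sound.
; Reset hides the beam and stops its effects.
; Time Stop pauses or resumes the effects, and Set Damage forwards damage to the child beam.
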(event EventBeginPlay
  (Rendering|SetVisibility (Variables|Default|GetWarningVFX) false false)
  (Utilities|FlowControl|Delay 0.2)
  (bind _asbp_laser_beam_2 (Utilities|Casting|CastToBP_LaserBeam2 (Variables|/Script/Engine.ChildActorComponent|GetChildActor (Variables|Default|GetChildActor))))
  (bind _output_get (Variables|Default|SetAs%20BP%20Laser%20Beam%202 _asbp_laser_beam_2))
  (Default|SetVisible _output_get false))

(event Collision|EventActorBeginOverlap
  (params (OtherActor :type Actor%20Object%20Reference)))

(event EventTick
  (params (DeltaSeconds :type Float%20%28single-precision%29)))

(fn ConstructionScript
  (Transformation|SetRelativeLocation (Variables|Default|GetBeam1) (Variables|/Script/Engine.SceneComponent|GetRelativeLocation (Variables|Default|GetLaser1%20StartPos)) false false)
  (Transformation|SetRelativeLocation (Variables|Default|GetBeam2) (Variables|/Script/Engine.SceneComponent|GetRelativeLocation (Variables|Default|GetLaser%202%20StartPos)) false false))

(fn Ready
  (Rendering|SetVisibility (Variables|Default|GetWarningVFX) true false)
  (Components|Activation|Activate (Variables|Default|GetWarningVFX) false)
  (Audio|PlaySound2D "/Game/SoundEffects/SoundFX/nmeBossLockOnGrid_FS.nmeBossLockOnGrid_FS" 1.0 1.0 0.0 0 0))

(fn Fire
  (bind _warningvfx (Variables|Default|GetWarningVFX))
  (Components|Activation|Deactivate _warningvfx)
  (Rendering|SetVisibility _warningvfx false false)
  (bind _as_bp_laser_beam_2 (Variables|Default|GetAs%20BP%20Laser%20Beam%202)
    (:then
      (Default|SetVisible _as_bp_laser_beam_2 true)
      (Components|Activation|Activate (Variables|Default|GetNiagara1) false)
      (Audio|PlaySound2D "/Game/SoundEffects/SoundFX/nmeBurstLazer_FS.nmeBurstLazer_FS" 1.0 1.0 0.0 0 0))
    (:else)))

(fn TimeStop
  (params (In%20Present :type Boolean))
  (if In%20Present
    (Class|NiagaraComponent|SetPaused (Variables|Default|GetNiagara1) true)
    (else
      (Class|NiagaraComponent|SetPaused (Variables|Default|GetNiagara1) false))))

(fn Reset
  (Components|Activation|Deactivate (Variables|Default|GetNiagara1))
  (bind _as_bp_laser_beam_2 (Variables|Default|GetAs%20BP%20Laser%20Beam%202)
    (:then
      (Default|SetVisible _as_bp_laser_beam_2 false))
    (:else)))

(fn SetDamage
  (params (Damage :type Float%20%28double-precision%29))
  (bind _asbp_laser_beam_2 (Utilities|Casting|CastToBP_LaserBeam2 (Variables|/Script/Engine.ChildActorComponent|GetChildActor (Variables|Default|GetChildActor))))
  (Variables|/Game/Enemies/Boss/Megaera/Laser/BP_BaseLaserStatic.BP_BaseLaserStatic_C|SetDamage _asbp_laser_beam_2 Damage))