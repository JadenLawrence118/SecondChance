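; Manager for the boss's laser bullet-hell attack, running its configured waves when BP_BossNew starts the attack.
; It pre-spawns a pool of BP_LaserGridLineV1 actors sized for the largest wave, with damage read per phase from DT_AttackCustoms.
; Each wave rotates the manager, spaces lasers along two perpendicular axes, then uses timers to indicate, fire and reset.
; Boss pause events freeze lasers and timer; CheckWave previews waves for developers.
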(event Custom|SecondPhase
  (bind _returnvalue (Utilities|GetDataTableRow "/Game/Enemies/Boss/Megaera/BossTryTwo/DT_AttackCustoms.DT_AttackCustoms" "2ndPhase")
    (:then
      (for _array_element (Variables|BulletHellMakerTool|GetBulletPool)
        (Default|SetDamage _array_element (.BH_Pattern1_Damage (Utilities|Struct|BreakS_MegaeraCustomVar _returnvalue)))))))

(event Custom|ResetAttackEndDoOnce
  ;[1 1 1] Loop through all the created waves
  (Utilities|FlowControl|DoOnce false) ; enters at Reset
)

(event Custom|OnPause_Event
  ;[1 1 1] Pause / UnPause when player time switch
  (for _array_element (Variables|BulletHellMakerTool|GetBulletPool)
    (Default|TimeStop _array_element true)
    (Utilities|Time|PauseTimerbyHandle (Variables|Default|GetBulletTimer))))

(event Custom|OnUnPause_Event
  ;[1 1 1] Pause / UnPause when player time switch
  (for _array_element (Variables|BulletHellMakerTool|GetBulletPool)
    (Default|TimeStop _array_element false)
    (Utilities|Time|UnpauseTimerbyHandle (Variables|Default|GetBulletTimer))))

(event Custom|OnBulletHellAttackStart_Event
  (Variables|LoopControl|SetcurrentWave 0)
  (Variables|LoopControl|SetwaveAttack true)
  (CallFunction|ResetAttackEndDoOnce)
  (CallFunction|ResetDoOnce))

(event Custom|ResetBullets
  ;[1 1 1] Loop through all the created waves
  (for _array_element (Variables|BulletHellMakerTool|GetBulletPool)
    (Default|SetBulletLocation _array_element))
  (Utilities|Time|ClearandInvalidateTimerbyHandle (Variables|Default|GetBulletTimer))
  (Variables|LoopControl|SetWaveEnded true))

(event Custom|Fire%20Bullets
  ;[1 1 1] Loop through all the created waves
  (Utilities|Time|ClearandInvalidateTimerbyHandle (Variables|Default|GetBulletTimer))
  (for _array_element (Variables|BulletHellMakerTool|GetBulletPool)
    (Default|Fire _array_element))
  (bind _returnvalue (Utilities|Time|SetTimerbyEvent (delegate Custom|ResetBullets) (Variables|BulletHellMakerTool|GetBulletLifeSpan) true))
  (Variables|Default|SetBulletTimer _returnvalue))

(event Custom|ResetDoOnce
  ;[1 1 1] Loop through all the created waves
  (Utilities|FlowControl|DoOnce false) ; enters at Reset
)

(event EventBeginPlay
  (Utilities|FlowControl|Delay 0.2)
  (Utilities|FlowControl|Sequence
    (:then_0
      (bind _returnvalue (Actor|GetActorOfClass "/Game/Enemies/Boss/Megaera/BossTryTwo/BP_BossNew.BP_BossNew_C"))
      (EventDispatchers|AssignOnBulletHellAttackStart _returnvalue (EventDispatchers|CreateEvent :!event Custom|OnBulletHellAttackStart_Event))
      (EventDispatchers|AssignOnPause _returnvalue (EventDispatchers|CreateEvent :!event Custom|OnPause_Event))
      (EventDispatchers|AssignOnUnPause _returnvalue (EventDispatchers|CreateEvent :!event Custom|OnUnPause_Event))
      (EventDispatchers|BindEventtoOnSecondPhase _returnvalue (EventDispatchers|CreateEvent :!event Custom|SecondPhase)))
    (:then_1
      (BulletHellMakerTool|SpawnBullets))))

(event Collision|EventActorBeginOverlap
  (params (OtherActor :type Actor%20Object%20Reference)))

(event EventTick
  (params (DeltaSeconds :type Float%20%28single-precision%29))
  ;[1 1 1] Loop through all the created waves
  (if (Variables|LoopControl|GetwaveAttack)
    (if (not (Variables|LoopControl|GetWaveEnded))
      (Utilities|FlowControl|DoOnce false
        (:Completed
          (CallFunction|WaveSetup (Utilities|Array|Get(acopy) (Variables|BulletHellMakerTool|GetBulletHellWaves) (Variables|LoopControl|GetcurrentWave)))
          (for _array_element (Variables|BulletHellMakerTool|GetBulletPool)
            (Default|Ready _array_element))
          (bind _returnvalue (Utilities|Time|SetTimerbyEvent (delegate Custom|Fire%20Bullets) (Variables|BulletHellMakerTool|GetIndicateTime)))
          (Variables|Default|SetBulletTimer _returnvalue)))
      (else
        (bind _result (Math|Integer|IncrementInt (Variables|LoopControl|GetcurrentWave))
          (:%20%20
            (if (>= _result (Utilities|Array|Length (Variables|BulletHellMakerTool|GetBulletHellWaves)))
              (Variables|LoopControl|SetWaveEnded false)
              (Variables|LoopControl|SetwaveAttack false)
              (else
                (CallFunction|ResetDoOnce)
                (Variables|LoopControl|SetWaveEnded false)))))))
    (else
      (Utilities|FlowControl|DoOnce false
        (:Completed
          (Default|CallOnAttackEnd))))))

(fn ConstructionScript)

(fn SetSpawnRangePos(EqualOffset)
  (params (Offset :type Float%20%28double-precision%29))
  (bind _spawn_range_y1 (Variables|Default|GetSpawn%20Range%20y1))
  (bind _spawn_range_y2 (Variables|Default|GetSpawn%20Range%20y2))
  (bind _spawn_range_x1 (Variables|Default|GetSpawn%20Range%20x1))
  (bind _spawn_range_x2 (Variables|Default|GetSpawn%20Range%20x2))
  (bind _relativelocation (Variables|/Script/Engine.SceneComponent|GetRelativeLocation _spawn_range_x2))
  (bind _relativelocation_2 (Variables|/Script/Engine.SceneComponent|GetRelativeLocation _spawn_range_y1))
  (bind _relativelocation_3 (Variables|/Script/Engine.SceneComponent|GetRelativeLocation _spawn_range_y2))
  (bind _relativelocation_4 (Variables|/Script/Engine.SceneComponent|GetRelativeLocation _spawn_range_x1))
  ;[1 1 1] Set the positions of all the Spawn range points with equal offset
  (Transformation|SetRelativeLocation _spawn_range_y1 (Math|Vector|MakeVector (+ 0.0 Offset) (.y _relativelocation_2) (.z _relativelocation_2)) false false)
  (Transformation|SetRelativeLocation _spawn_range_y2 (Math|Vector|MakeVector (- 0.0 Offset) (.y _relativelocation_3) (.z _relativelocation_3)) false false)
  (Transformation|SetRelativeLocation _spawn_range_x1 (Math|Vector|MakeVector (.x _relativelocation_4) (+ 0.0 Offset) (.z _relativelocation_4)) false false)
  (Transformation|SetRelativeLocation _spawn_range_x2 (Math|Vector|MakeVector (.x _relativelocation) (- 0.0 Offset) (.z _relativelocation)) false false))

(fn SetSpawnRangePos
  (params (Spawn%20y1%20offset :type Float%20%28double-precision%29) (Spawn%20y2%20offset :type Float%20%28double-precision%29) (Spawn%20x1%20offset :type Float%20%28double-precision%29) (Spawn%20x2%20offset :type Float%20%28double-precision%29))
  (bind _spawn_range_y1 (Variables|Default|GetSpawn%20Range%20y1))
  (bind _spawn_range_y2 (Variables|Default|GetSpawn%20Range%20y2))
  (bind _spawn_range_x1 (Variables|Default|GetSpawn%20Range%20x1))
  (bind _spawn_range_x2 (Variables|Default|GetSpawn%20Range%20x2))
  (bind _relativelocation (Variables|/Script/Engine.SceneComponent|GetRelativeLocation _spawn_range_x2))
  (bind _relativelocation_2 (Variables|/Script/Engine.SceneComponent|GetRelativeLocation _spawn_range_y1))
  (bind _relativelocation_3 (Variables|/Script/Engine.SceneComponent|GetRelativeLocation _spawn_range_y2))
  (bind _relativelocation_4 (Variables|/Script/Engine.SceneComponent|GetRelativeLocation _spawn_range_x1))
  ;[1 1 1] Set the positions of all the Spawn range points with customed offset
  (Transformation|SetRelativeLocation _spawn_range_y1 (Math|Vector|MakeVector (+ 0.0 Spawn%20y1%20offset) (.y _relativelocation_2) (.z _relativelocation_2)) false false)
  (Transformation|SetRelativeLocation _spawn_range_y2 (Math|Vector|MakeVector (- 0.0 Spawn%20y2%20offset) (.y _relativelocation_3) (.z _relativelocation_3)) false false)
  (Transformation|SetRelativeLocation _spawn_range_x1 (Math|Vector|MakeVector (.x _relativelocation_4) (+ 0.0 Spawn%20x1%20offset) (.z _relativelocation_4)) false false)
  (Transformation|SetRelativeLocation _spawn_range_x2 (Math|Vector|MakeVector (.x _relativelocation) (- 0.0 Spawn%20x2%20offset) (.z _relativelocation)) false false))

(fn BulletPosSetup
  (params (isSquareStruct :type Boolean) (Num%20of%20LaserX :type Integer) (Num%20of%20LaserY :type Integer))
  (bind _returnvalue (Transformation|GetActorRotation))
  (bind _returnvalue_2 (Math|Integer|SelectInt Num%20of%20LaserX Num%20of%20LaserY isSquareStruct))
  (bind _returnvalue_3 (- Num%20of%20LaserX 1))
  (bind _spawn_range_x1 (Variables|Default|GetSpawn%20Range%20x1))
  (bind _spawn_range_x2 (Variables|Default|GetSpawn%20Range%20x2))
  (bind _spawn_range_y1 (Variables|Default|GetSpawn%20Range%20y1))
  (bind _spawn_range_y2 (Variables|Default|GetSpawn%20Range%20y2))
  (bind _returnvalue_4 (Transformation|GetWorldLocation _spawn_range_y1))
  (bind _returnvalue_5 (Transformation|GetWorldLocation _spawn_range_y2))
  (bind _returnvalue_6 (Transformation|GetWorldLocation _spawn_range_x1))
  (bind _returnvalue_7 (Transformation|GetWorldLocation _spawn_range_x2))
  (bind _returnvalue_8 (- _returnvalue_2 1))
  (bind _returnvalue_9 (Math|Vector|MakeVector (.x _returnvalue_7) (.y _returnvalue_7) 0.0))
  (bind _returnvalue_10 (Math|Vector|MakeVector (.x _returnvalue_6) (.y _returnvalue_6) 0.0))
  (bind _returnvalue_11 (Math|Vector|MakeVector (.x _returnvalue_4) (.y _returnvalue_4) 0.0))
  (bind _returnvalue_12 (Math|Vector|MakeVector (.x _returnvalue_5) (.y _returnvalue_5) 0.0))
  ;[1 1 1] Set Position for the bullets needed on X
  (for _index (range 0 _returnvalue_3)
    (Transformation|SetActorLocationAndRotation (Utilities|Array|Get(acopy) (Variables|BulletHellMakerTool|GetBulletPool) _index) (+ (* _index (* (/ (Math|Vector|Distance2D(Vector) _returnvalue_9 _returnvalue_10) _returnvalue_3) (Math|Vector|Normalize (- _returnvalue_9 _returnvalue_10)))) (Transformation|GetWorldLocation _spawn_range_x1)) (Transformation|GetActorRotation)))
  ;[1 1 1] Set Position for the bullets needed on Y
  (for _index_2 (range Num%20of%20LaserX (+ Num%20of%20LaserX _returnvalue_8))
    (Transformation|SetActorLocationAndRotation (Utilities|Array|Get(acopy) (Variables|BulletHellMakerTool|GetBulletPool) _index_2) (+ (* (- _index_2 Num%20of%20LaserX) (* (/ (Math|Vector|Distance2D(Vector) _returnvalue_12 _returnvalue_11) _returnvalue_8) (Math|Vector|Normalize (- _returnvalue_12 _returnvalue_11)))) (Transformation|GetWorldLocation _spawn_range_y1)) (Math|Rotator|MakeRotator (.roll _returnvalue) (.pitch _returnvalue) (+ (.yaw _returnvalue) 9e+01))))
  ;[1 1 1] Reset the unused Bullets position
  (for _index_3 (range (Math|Integer|SelectInt (* Num%20of%20LaserX 2) (+ Num%20of%20LaserX Num%20of%20LaserY) isSquareStruct) (- (Utilities|Array|Length (Variables|BulletHellMakerTool|GetBulletPool)) 1))
    (Transformation|SetActorLocationAndRotation (Utilities|Array|Get(acopy) (Variables|BulletHellMakerTool|GetBulletPool) _index_3) "0.000000,0.000000,-100.000000")))

(fn WaveSetup
  (params (S_BulletHellSet :type S%20Bullet%20Hell%20Set%20Structure%20%28by%20ref%29))
  (bind (_yaw _issquarestruct _spawnequaloffset _spawny1offset _spawny2offset _spawnx1offset _spawnx2offset _numberoflaserx _numberoflasery) (Utilities|Struct|BreakS_BulletHellSet S_BulletHellSet))
  (bind _returnvalue (Transformation|GetActorRotation))
  ;[1 1 1] Set up the components needed for the wave
  (Transformation|SetActorRotation (Math|Rotator|MakeRotator (.roll _returnvalue) (.pitch _returnvalue) _yaw))
  (if _issquarestruct
    (CallFunction|SetSpawnRangePos(EqualOffset) _spawnequaloffset)
    (else
      (CallFunction|SetSpawnRangePos _spawny1offset _spawny2offset _spawnx1offset _spawnx2offset)))
  (CallFunction|BulletPosSetup _issquarestruct _numberoflaserx _numberoflasery))

(fn CheckWave
  (bind _bulletpool (Variables|BulletHellMakerTool|GetBulletPool))
  (bind _check_wave_id (Variables|WaveChecker|GetCheck%20Wave%20ID))
  (bind _bullethellwaves (Variables|BulletHellMakerTool|GetBulletHellWaves))
  (bind _output (Utilities|Array|Get(acopy) _bullethellwaves _check_wave_id))
  (bind (_yaw _issquarestruct _spawnequaloffset _spawny1offset _spawny2offset _spawnx1offset _spawnx2offset _numberoflaserx _numberoflasery) (Utilities|Struct|BreakS_BulletHellSet _output))
  ;[0.04911 1 0.6101] Preview wave in Editor - For Developer
  ;;[1 1 1] Clear the previous Pool
  (for _array_element _bulletpool
    (Actor|DestroyActor _array_element))
  (Utilities|Array|Clear _bulletpool)
  ;;[1 1 1] Spawn lasers and add to the pool
  (for _index (range 1 (Math|Integer|SelectInt (* _numberoflaserx 2) (+ _numberoflaserx _numberoflasery) _issquarestruct))
    (bind _returnvalue (Game|SpawnActorfromClass "/Game/Enemies/Boss/Megaera/Laser/BulletHell/BP_LaserGridLineV1.BP_LaserGridLineV1_C" (Math|Transform|MakeTransform "0, 0, 0" "0, 0, 0" "1.000000,1.000000,1.000000") "Undefined" "MultiplyWithRoot" self 0.0 0))
    (Utilities|Array|Add (Variables|BulletHellMakerTool|GetBulletPool) _returnvalue)
    (Transformation|AttachActorToActor self "None" "KeepWorld" "KeepWorld" "KeepWorld" true)
    (CallFunction|WaveSetup (Utilities|Array|Get(acopy) (Variables|BulletHellMakerTool|GetBulletHellWaves) (Variables|WaveChecker|GetCheck%20Wave%20ID)))))

(fn SpawnBullets
  (bind _bulletpool (Variables|BulletHellMakerTool|GetBulletPool))
  ;[1 1 1] Clear the previous Pool
  (for _array_element _bulletpool
    (Actor|DestroyActor _array_element))
  (Utilities|Array|Clear _bulletpool)
  (bind _returnvalue (Utilities|GetDataTableRow "/Game/Enemies/Boss/Megaera/BossTryTwo/DT_AttackCustoms.DT_AttackCustoms" "1stPhase")
    (:then
      (for (_array_element_2 _array_index) (Variables|BulletHellMakerTool|GetBulletHellWaves)
        ;[1 1 1] Check The wave with highest num of lasers
        (if (== _array_index 0)
          (Variables|BulletHellMakerTool|SetHighestNumOfLasers (* (.NumberofLaserX (Utilities|Struct|BreakS_BulletHellSet _array_element_2)) 2))
          (elif (> (Math|Integer|SelectInt (* (.NumberofLaserX (Utilities|Struct|BreakS_BulletHellSet _array_element_2)) 2) (+ (.NumberofLaserX (Utilities|Struct|BreakS_BulletHellSet _array_element_2)) (.NumberofLaserY (Utilities|Struct|BreakS_BulletHellSet _array_element_2))) (.isSquareStruct (Utilities|Struct|BreakS_BulletHellSet _array_element_2))) (Variables|BulletHellMakerTool|GetHighestNumOfLasers))
            (Variables|BulletHellMakerTool|SetHighestNumOfLasers (Math|Integer|SelectInt (* (.NumberofLaserX (Utilities|Struct|BreakS_BulletHellSet _array_element_2)) 2) (+ (.NumberofLaserX (Utilities|Struct|BreakS_BulletHellSet _array_element_2)) (.NumberofLaserY (Utilities|Struct|BreakS_BulletHellSet _array_element_2))) (.isSquareStruct (Utilities|Struct|BreakS_BulletHellSet _array_element_2)))))))
      ;[1 1 1] Spawn lasers and add to the pool
      (for _index (range 1 (Variables|BulletHellMakerTool|GetHighestNumOfLasers))
        (bind _returnvalue_2 (Game|SpawnActorfromClass "/Game/Enemies/Boss/Megaera/Laser/BulletHell/BP_LaserGridLineV1.BP_LaserGridLineV1_C" (Math|Transform|MakeTransform "0.000000,0.000000,-100.000000" "0, 0, 0" "1.000000,1.000000,1.000000") "Undefined" "MultiplyWithRoot" self 0.0 0))
        (Default|SetDamage _returnvalue_2 (.BH_Pattern1_Damage (Utilities|Struct|BreakS_MegaeraCustomVar _returnvalue)))
        (Utilities|Array|Add (Variables|BulletHellMakerTool|GetBulletPool) _returnvalue_2)
        (Transformation|AttachActorToActor _returnvalue_2 self "None" "KeepWorld" "KeepWorld" "KeepWorld" true)))))

(fn ClearScene
  (bind _bulletpool (Variables|BulletHellMakerTool|GetBulletPool))
  ;[1 1 1] Clear all the bullets actor in the scene
  (for _array_element _bulletpool
    (Actor|DestroyActor _array_element))
  (Utilities|Array|Clear _bulletpool))