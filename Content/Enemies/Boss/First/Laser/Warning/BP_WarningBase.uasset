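; BP_WarningBase is a base warning indicator for the first boss's laser attack, hidden until triggered.
; StartWarning shows it, activates its main and base Niagara effects, and plays the Scaling timeline at a rate inverse to the warning time.
; The timeline drives MainWarning's X and Y scale.
; Pause and Continue halt and resume both timeline and effects, while Reset only hides the indicator.
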(event EventBeginPlay
  (Rendering|SetVisibility (Variables|Default|GetDefaultSceneRoot) false true))

(event Collision|EventActorBeginOverlap
  (params (OtherActor :type Actor%20Object%20Reference)))

(event EventTick
  (params (DeltaSeconds :type Float%20%28single-precision%29)))

(fn ConstructionScript)

(fn StartWarning
  (params (WarningTIme :type Float%20%28double-precision%29))
  (bind _scaling (Variables|Default|GetScaling))
  (Rendering|SetVisibility (Variables|Default|GetDefaultSceneRoot) true true)
  (Components|Activation|Activate (Variables|Default|GetMainWarning) false)
  (Components|Timeline|SetPlayRate _scaling (/ 1.0 WarningTIme))
  (Components|Timeline|PlayfromStart _scaling))

(fn Pause
  (Audio|Components|Audio|Stop (Variables|Default|GetScaling))
  (Class|NiagaraComponent|SetPaused (Variables|Default|GetMainWarning) true))

(fn Continue
  (Audio|Components|Audio|Play (Variables|Default|GetScaling))
  (Class|NiagaraComponent|SetPaused (Variables|Default|GetMainWarning) false))

(fn Reset
  (Rendering|SetVisibility (Variables|Default|GetDefaultSceneRoot) false true))