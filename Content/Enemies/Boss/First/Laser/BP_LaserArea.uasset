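; Laser area actor for the first boss's attack, wrapping a Niagara laser effect that can be switched on, off or paused.
; On BeginPlay it passes AttackDuration to the effect's Lifetime parameter after running the parent logic.
; Activate and Deactivate toggle root visibility with children, the Niagara system and the IsOn flag together.
; Pause and Continue only freeze and resume the Niagara simulation.
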(event EventBeginPlay
  (|CallParentFunction)
  (Niagara|SetNiagaraVariable(Float) (Variables|Default|GetNiagara) "Lifetime" (Variables|Default|GetAttackDuration)))

(event Collision|EventActorBeginOverlap
  (params (OtherActor :type Actor%20Object%20Reference)))

(event EventTick
  (params (DeltaSeconds :type Float%20%28single-precision%29))
  (|CallParentFunction DeltaSeconds) ; This node is disabled and will not be called.\nDrag off pins to build functionality.
)

(fn ConstructionScript
  (|CallParentFunction))

(fn Activate
  (Rendering|SetVisibility (Variables|Default|GetDefaultSceneRoot) true true)
  (Components|Activation|Activate (Variables|Default|GetNiagara) false)
  (Variables|Default|SetIsOn true))

(fn Deactivate
  (Rendering|SetVisibility (Variables|Default|GetDefaultSceneRoot) false true)
  (Components|Activation|Deactivate (Variables|Default|GetNiagara))
  (Variables|Default|SetIsOn false))

(fn Pause
  (Class|NiagaraComponent|SetPaused (Variables|Default|GetNiagara) true))

(fn Continue
  (Class|NiagaraComponent|SetPaused (Variables|Default|GetNiagara) false))