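; BP_LaserGridLine is one line of a boss laser grid, made of two BP_BulletHellLaser child actors and an indicator.
; The construction script places each laser at its start position component, and Reset sends them back there.
; The indicator starts hidden, Ready shows it as a telegraph, and Fire hides it and fires both lasers.
; TimeStop freezes or resumes both lasers through their custom time dilation.
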(event EventBeginPlay
  (Rendering|SetVisibility (Variables|Default|GetIndicator) false false))

(event Collision|EventActorBeginOverlap
  (params (OtherActor :type Actor%20Object%20Reference)))

(event EventTick
  (params (DeltaSeconds :type Float%20%28single-precision%29)))

(fn ConstructionScript
  (Transformation|SetActorLocation (Variables|/Script/Engine.ChildActorComponent|GetChildActor (Variables|Default|GetLaser1)) (Transformation|GetWorldLocation (Variables|Default|GetLaser1%20StartPos)) false false)
  (Transformation|SetActorLocation (Variables|/Script/Engine.ChildActorComponent|GetChildActor (Variables|Default|GetLaser2)) (Transformation|GetWorldLocation (Variables|Default|GetLaser%202%20StartPos)) false false))

(fn Ready
  (Rendering|SetVisibility (Variables|Default|GetIndicator) true false))

(fn Fire
  (Rendering|SetVisibility (Variables|Default|GetIndicator) false false)
  (bind _asbp_bullet_hell_laser (Utilities|Casting|CastToBP_BulletHellLaser (Variables|/Script/Engine.ChildActorComponent|GetChildActor (Variables|Default|GetLaser1))))
  (bind _asbp_bullet_hell_laser_2 (Utilities|Casting|CastToBP_BulletHellLaser (Variables|/Script/Engine.ChildActorComponent|GetChildActor (Variables|Default|GetLaser2))))
  (Default|Fire _asbp_bullet_hell_laser)
  (Default|Fire _asbp_bullet_hell_laser_2))

(fn TimeStop
  (params (In%20Present :type Boolean))
  (bind _laser1 (Variables|Default|GetLaser1))
  (bind _laser2 (Variables|Default|GetLaser2))
  (bind _childactor (Variables|/Script/Engine.ChildActorComponent|GetChildActor _laser1))
  (bind _childactor_2 (Variables|/Script/Engine.ChildActorComponent|GetChildActor _laser2))
  (if In%20Present
    (Variables|/Script/Engine.Actor|SetCustomTimeDilation _childactor 0.0)
    (Variables|/Script/Engine.Actor|SetCustomTimeDilation _childactor_2 0.0)
    (else
      (Variables|/Script/Engine.Actor|SetCustomTimeDilation _childactor 1.0)
      (Variables|/Script/Engine.Actor|SetCustomTimeDilation _childactor_2 1.0))))

(fn Reset
  (bind _asbp_bullet_hell_laser (Utilities|Casting|CastToBP_BulletHellLaser (Variables|/Script/Engine.ChildActorComponent|GetChildActor (Variables|Default|GetLaser1))))
  (bind _asbp_bullet_hell_laser_2 (Utilities|Casting|CastToBP_BulletHellLaser (Variables|/Script/Engine.ChildActorComponent|GetChildActor (Variables|Default|GetLaser2))))
  (Default|Reset _asbp_bullet_hell_laser (Transformation|GetWorldLocation (Variables|Default|GetLaser1%20StartPos)))
  (Default|Reset _asbp_bullet_hell_laser_2 (Transformation|GetWorldLocation (Variables|Default|GetLaser%202%20StartPos))))