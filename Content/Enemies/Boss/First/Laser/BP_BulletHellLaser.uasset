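; BP_BulletHellLaser is a laser actor for the first boss, named for a bullet-hell attack.
; Two seconds after BeginPlay it calls TurnOnLaser, which makes the LaserShape component visible and plays a timeline from the start.
; The timeline's Size track drives the shape's relative Z scale, animating the beam along that axis while X and Y stay fixed.
; The graph itself has no damage or overlap logic.
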(event Custom|TurnOnLaser
  (Rendering|SetVisibility (Variables|Default|GetLaserShape) true false)
  (bind _size (Timeline|Timeline PlayFromStart)
    (:Update
      (Transformation|SetRelativeScale3D (Variables|Default|GetLaserShape) (Math|Vector|MakeVector 1.0 1.0 _size)))))

(event EventBeginPlay
  (|CallParentFunction)
  (Utilities|FlowControl|Delay 2.0)
  (CallFunction|TurnonLaser))

(event Collision|EventActorBeginOverlap
  (params (OtherActor :type Actor%20Object%20Reference)))

(event EventTick
  (params (DeltaSeconds :type Float%20%28single-precision%29))
  (|CallParentFunction DeltaSeconds) ; This node is disabled and will not be called.\nDrag off pins to build functionality.
)

(fn ConstructionScript
  (|CallParentFunction))