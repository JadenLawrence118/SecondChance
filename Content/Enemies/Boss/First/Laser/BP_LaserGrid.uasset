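; Boss laser grid attack that covers an area with warning and damaging laser tiles in a checkerboard pattern.
; MakeGrid spawns paired warning and laser actors at BeginPlay, and IsAlternating splits them by index parity.
; BP_BossNew's OnLaserGridStart triggers two timer-chained waves, each warning then firing one half of the pattern.
; The timer follows the boss's pause events, and the last wave clears CanUseBulletHell and fires OnFinishAttack.
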(event Custom|Attack1
  (bind _chargingtime (Variables|Default|GetChargingTime))
  ;[1 1 1] Starts the 1 attack then calls the second one when the first is over
  (CallFunction|Turnon1Warnings _chargingtime)
  (bind _returnvalue (Utilities|Time|SetTimerbyEvent (delegate Custom|Turn%20on%201Laser) _chargingtime))
  (Variables|Default|SetTimer _returnvalue))

(event Custom|Attack2
  (bind _chargingtime (Variables|Default|GetChargingTime))
  (CallFunction|Turnon2Warnings _chargingtime)
  (bind _returnvalue (Utilities|Time|SetTimerbyEvent (delegate Custom|Laser2%20Turn%20On) _chargingtime))
  (Variables|Default|SetTimer _returnvalue))

(event Custom|Turn%20on%201Laser
  ;[1 1 1] Starts the 1 attack then calls the second one when the first is over
  (Utilities|Time|ClearandInvalidateTimerbyHandle (Variables|Default|GetTimer))
  (CallFunction|Turnon1Lasers)
  (bind _returnvalue (Utilities|Time|SetTimerbyEvent (delegate Custom|Laser1%20Ended) (Variables|Default|GetAttackTime)))
  (Variables|Default|SetTimer _returnvalue))

(event Custom|Laser1%20Ended
  ;[1 1 1] Starts the 1 attack then calls the second one when the first is over
  (CallFunction|TurnOffAll)
  (Utilities|Time|ClearandInvalidateTimerbyHandle (Variables|Default|GetTimer))
  (CallFunction|Attack2))

(event Custom|Laser2%20Turn%20On
  (Utilities|Time|ClearandInvalidateTimerbyHandle (Variables|Default|GetTimer))
  (CallFunction|Turnon2Lasers)
  (bind _returnvalue (Utilities|Time|SetTimerbyEvent (delegate Custom|Laser2%20Ended) (Variables|Default|GetAttackTime)))
  (Variables|Default|SetTimer _returnvalue))

(event Custom|Laser2%20Ended
  (bind _owningbossactor (Variables|Default|GetOwningBossActor))
  (CallFunction|TurnOffAll)
  (Utilities|Time|ClearandInvalidateTimerbyHandle (Variables|Default|GetTimer))
  (Variables|/Game/Enemies/Boss/First/BossTryTwo/BP_BossNew.BP_BossNew_C|SetCanUseBulletHell _owningbossactor false)
  (Default|CallOnFinishAttack _owningbossactor))

(event Custom|OnPause_Event
  (Utilities|Time|PauseTimerbyHandle (Variables|Default|GetTimer)))

(event Custom|OnUnPause_Event
  (Utilities|Time|UnpauseTimerbyHandle (Variables|Default|GetTimer)))

(event Custom|OnLaserGridStart_Event
  (CallFunction|Attack1))

(event EventBeginPlay
  (bind _returnvalue (Actor|GetActorOfClass "/Game/Enemies/Boss/First/BossTryTwo/BP_BossNew.BP_BossNew_C"))
  (bind _output_get (Variables|Default|SetOwningBossActor _returnvalue))
  (EventDispatchers|AssignOnLaserGridStart _output_get (EventDispatchers|CreateEvent :!event Custom|OnLaserGridStart_Event))
  (EventDispatchers|AssignOnPause _returnvalue (EventDispatchers|CreateEvent :!event Custom|OnPause_Event))
  (EventDispatchers|AssignOnUnPause _returnvalue (EventDispatchers|CreateEvent :!event Custom|OnUnPause_Event))
  (CallFunction|MakeGrid))

(event Collision|EventActorBeginOverlap
  (params (OtherActor :type Actor%20Object%20Reference)))

(fn ConstructionScript)

(fn MakeGrid
  (bind _returnvalue (Transformation|GetActorLocation))
  (bind _scale (Variables|Default|GetScale))
  (bind _scale_2 (Variables|Default|GetScale))
  (bind _cellsize (Variables|Default|GetCellSize))
  ;[1 1 1] Create a grid of warning and attacking lasers and add them to an array
  (for _index (range 0 (- (Variables|Default|GetRows) 1))
    (for _index_2 (range 0 (- (Variables|Default|GetColumns) 1))
      (bind _returnvalue_2 (Game|SpawnActorfromClass "/Game/Enemies/Boss/First/Laser/BP_WarningArea.BP_WarningArea_C" (Math|Transform|MakeTransform (Math|Vector|MakeVector (+ (* _index_2 _cellsize (.x _scale)) (.x _returnvalue)) (+ (* _index _cellsize (.y _scale)) (.y _returnvalue)) (.z _returnvalue)) "0, 0, 0" (Math|Vector|MakeVector (.x _scale_2) (.y _scale_2) 0.1)) "Undefined" "OverrideRootScale" self 0))
      (Default|Deactivate _returnvalue_2)
      (bind _returnvalue_3 (Utilities|Array|Add (Variables|Default|GetWarningAreas) _returnvalue_2))
      (Variables|/Game/Enemies/Boss/First/Laser/BP_WarningArea.BP_WarningArea_C|SetArayNum _returnvalue_2 _returnvalue_3)
      (bind _returnvalue_4 (Game|SpawnActorfromClass "/Game/Enemies/Boss/First/Laser/BP_LaserArea.BP_LaserArea_C" (Math|Transform|MakeTransform (Math|Vector|MakeVector (+ (* _index_2 _cellsize (.x _scale)) (.x _returnvalue)) (+ (* _index _cellsize (.y _scale)) (.y _returnvalue)) (.z _returnvalue)) "0, 0, 0" "1.000000,1.000000,1.000000") "Undefined" "OverrideRootScale" self (Variables|Default|GetScale) "/Game/Enemies/Boss/First/Laser/Materials/M_BaseLaserTransLucent.M_BaseLaserTransLucent" true true (Variables|Default|GetDamage) 0))
      (Default|Deactivate _returnvalue_4)
      (Utilities|Array|Add (Variables|Default|GetLaserAreas) _returnvalue_4))))

(fn TurnOffAll
  ;[1 1 1] Turning off all the lasers if they are on
  (for _array_element (Variables|Default|GetWarningAreas)
    (Utilities|IsValid _array_element
      (:Is%20Valid
        (if (Variables|/Game/Enemies/Boss/First/Laser/BP_WarningArea.BP_WarningArea_C|GetIsOn _array_element)
          (Default|Deactivate _array_element)))))
  (for _array_element_2 (Variables|Default|GetLaserAreas)
    (Utilities|IsValid _array_element_2
      (:Is%20Valid
        (if (Variables|/Game/Enemies/Boss/First/Laser/BP_LaserArea.BP_LaserArea_C|GetIsOn _array_element_2)
          (Default|Deactivate _array_element_2))))))

(fn Turnon1Warnings
  (params (WarningTime :type Float%20%28double-precision%29))
  (for (_array_element _array_index) (Variables|Default|GetWarningAreas)
    (bind _isalternating (CallFunction|IsAlternating _array_index))
    (if _isalternating
      (Utilities|IsValid _array_element
        (:Is%20Valid
          (Default|Activate _array_element WarningTime))))))

(fn IsAlternating
  (params (X :type Integer))
  (bind _rows (Variables|Default|GetRows))
  ;[1 1 1] Checks if the index has to be activated
  (return (== (Math|Integer|%(Integer) (+ (Math|Integer|%(Integer) X _rows) (/ X _rows)) 2) 0)))

(fn Turnon1Lasers
  (for (_array_element _array_index) (Variables|Default|GetLaserAreas)
    (bind _isalternating (CallFunction|IsAlternating _array_index))
    (if _isalternating
      (Utilities|IsValid _array_element
        (:Is%20Valid
          (Default|Activate _array_element)
          (Development|PrintString (Utilities|String|ToString(Integer) _array_index)))))))

(fn Turnon2Lasers
  (for (_array_element _array_index) (Variables|Default|GetLaserAreas)
    (bind _isalternating (CallFunction|IsAlternating _array_index))
    (if (not _isalternating)
      (Utilities|IsValid _array_element
        (:Is%20Valid
          (Default|Activate _array_element)
          (Development|PrintString "Hello"))))))

(fn Turnon2Warnings
  (params (Warning%20Time :type Float%20%28double-precision%29))
  (for (_array_element _array_index) (Variables|Default|GetWarningAreas)
    (bind _isalternating (CallFunction|IsAlternating _array_index))
    (if (not _isalternating)
      (Utilities|IsValid _array_element
        (:Is%20Valid
          (Default|Activate _array_element Warning%20Time))))))