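; Base first-boss Blueprint that handles the player's hits on the boss and the resulting game win.
; BeginPlay caches the third-person player character, which damage events launch along its control-rotation forward vector, scaled by Knockback.
; Damage goes through the BPCPlayerStats component's DecreaseHealth, whose true result calls GameWin on the player.
; Otherwise CanBeDamaged switches off for the Iframes delay, ignoring hits during that window.
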(event EventBeginPlay
  (|CallParentFunction)
  (bind _asbp_third_person_character (Utilities|Casting|CastToBP_ThirdPersonCharacter (Game|GetPlayerCharacter 0)))
  (Variables|Default|SetPlayerRef _asbp_third_person_character))

(event Collision|EventActorBeginOverlap
  (params (OtherActor :type Actor%20Object%20Reference))
  (|CallParentFunction OtherActor) ; This node is disabled and will not be called.\nDrag off pins to build functionality.
)

(event EventTick
  (params (DeltaSeconds :type Float%20%28single-precision%29))
  (|CallParentFunction DeltaSeconds) ; This node is disabled and will not be called.\nDrag off pins to build functionality.
)

(event Game|Damage|EventAnyDamage
  (params (Damage :type Float%20%28single-precision%29) (DamageType :type Damage%20Type%20Object%20Reference) (InstigatedBy :type Controller%20Object%20Reference) (DamageCauser :type Actor%20Object%20Reference))
  (bind _playerref (Variables|Default|GetPlayerRef))
  ;[1 1 1] Player Hits the boss
  (if (Variables|Default|GetCanBeDamaged)
    (Character|LaunchCharacter _playerref (* (Math|Vector|GetForwardVector (Pawn|GetControlRotation _playerref :!class /Script/Engine.Pawn)) (Variables|Default|GetKnockback)) false false)
    (bind _isplayerdead (Default|DecreaseHealth (Variables|Default|GetBPC_PlayerStats) Damage))
    (if _isplayerdead
      (bind _asbp_third_person_character (Utilities|Casting|CastToBP_ThirdPersonCharacter (Game|GetPlayerCharacter 0)))
      (Default|GameWin _asbp_third_person_character)
      (else
        (Variables|Default|SetCanBeDamaged false)
        (Utilities|FlowControl|Delay (Variables|Default|Geti-frames))
        (Variables|Default|SetCanBeDamaged true)))))

(fn ConstructionScript
  (|CallParentFunction))