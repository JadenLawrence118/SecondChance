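; Flying first boss with a health bar widget and laser and shockwave attacks, tied to the player's present/past time state.
; Tick enables cylinder collision and applies health regen only in the present, and keeps the spinning beam's yaw matched to a mesh socket.
; Callable functions handle interpolated aiming, spinning, laser visibility, wave spawning and reset, with no attack sequencing here.
; Shockwaves also deal heavy damage to a nearby player.
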(event EventBeginPlay
  (|CallParentFunction)
  (bind _returnvalue (UserInterface|CreateWidget "/Game/UI/Boss/WB_BossHealth.WB_BossHealth_C"))
  (UserInterface|Viewport|AddtoViewport _returnvalue 0)
  (A1|AimingLaserOff)
  (A1|ChargeLaserFireOff)
  (SpinningLaser|SpinningLaserOff)
  (bind _asbp_third_person_character (Utilities|Casting|CastToBP_ThirdPersonCharacter (Game|GetPlayerCharacter 0)))
  (Variables|Default|SetPlayerRef_0 _asbp_third_person_character))

(event EventTick
  (params (DeltaSeconds :type Float%20%28single-precision%29))
  (bind _playerref_0 (Variables|Default|GetPlayerRef_0))
  (bind _bpc_playerstats (Variables|Default|GetBPC_PlayerStats))
  (bind _cylinder (Variables|Default|GetCylinder))
  (bind _inpresent (Variables|/Game/ThirdPerson/Blueprints/BP_ThirdPersonCharacter.BP_ThirdPersonCharacter_C|GetInPresent _playerref_0))
  (if (!= (Variables|Default|GetPresent/Past) _inpresent)
    (bind _output_get (Variables|Default|SetPresent/Past _inpresent))
    (if _output_get
      (Collision|SetCollisionEnabled _cylinder "QueryAndPhysics")
      (else
        (Collision|SetCollisionEnabled _cylinder "NoCollision"))))
  ;[1 1 1] Spins the laser when it is on with the msh
  (if (Variables|Default|GetIsSpinLaserOn)
    (Transformation|SetWorldRotation (Variables|Default|GetBP_LaserBeam) (Math|Rotator|MakeRotator 0.0 0.0 (.yaw (Transformation|GetSocketRotation (Variables|Character|GetMesh) "BottomSocket"))) false false))
  ;[1 1 1] Increase boss health
  (if (Variables|/Game/ThirdPerson/Blueprints/BP_ThirdPersonCharacter.BP_ThirdPersonCharacter_C|GetInPresent (Variables|Default|GetPlayerRef_0))
    (if (<= (Variables|/Game/ThirdPerson/Blueprints/BPC_PlayerStats.BPC_PlayerStats_C|GetCurrentHealth _bpc_playerstats) (Variables|/Game/ThirdPerson/Blueprints/BPC_PlayerStats.BPC_PlayerStats_C|GetMaxHealth _bpc_playerstats))
      (Default|DecreaseHealth (Variables|Default|GetBPC_PlayerStats) (* (Variables|Default|GetHealthRegen) (Utilities|Time|GetWorldDeltaSeconds))))))

(fn ConstructionScript
  (|CallParentFunction))

(fn RotatetoMesh
  (params (TargetRotation :type Vector))
  (bind _returnvalue (Utilities|Time|GetWorldDeltaSeconds))
  (bind _lookspeed (Variables|Default|GetLookSpeed))
  (bind _aimrotationoffset (LocalVariables|GetAimRotationOffset))
  (bind _mesh (Variables|Character|GetMesh))
  (bind _returnvalue_2 (Transformation|GetWorldLocation _mesh))
  (bind _returnvalue_3 (Transformation|GetWorldRotation _mesh))
  (bind _returnvalue_4 (- TargetRotation (Math|Vector|MakeVector 0.0 0.0 _aimrotationoffset)))
  (bind _returnvalue_5 (Math|Rotator|FindLookatRotation _returnvalue_2 _returnvalue_4))
  (bind _returnvalue_6 (Math|Interpolation|RInterpTo _returnvalue_3 _returnvalue_5 _returnvalue _lookspeed))
  (Transformation|SetWorldRotation (Variables|Character|GetMesh) (Math|Rotator|MakeRotator 0.0 (.pitch _returnvalue_6) (.yaw _returnvalue_6)) false false)
  (if true
    _))

(fn ResetRotation
  (Transformation|SetRelativeRotation (Variables|Character|GetMesh) (Math|Interpolation|RInterpTo (Variables|/Script/Engine.SceneComponent|GetRelativeRotation (Variables|Character|GetMesh)) "0, 0, 0" (Utilities|Time|GetWorldDeltaSeconds) 3.0) false false)
  (return (Utilities|Operators|EqualEqual :A (Variables|/Script/Engine.SceneComponent|GetRelativeRotation (Variables|Character|GetMesh)))))

(fn AimingLaseron
  (bind _aiminglaser (Variables|Default|GetAimingLaser))
  (Rendering|SetVisibility _aiminglaser true false)
  (Niagara|SetNiagaraVariable(LinearColor) _aiminglaser "BeamColor" (Math|Color|MakeColor 0.0 1.0 0.0)))

(fn AimingLaserOff
  (Rendering|SetVisibility (Variables|Default|GetAimingLaser) false false))

(fn ChargeLaserFireon
  (Rendering|SetVisibility (Variables|Default|GetChargedLaser) true true))

(fn ChargeLaserFireOff
  (Rendering|SetVisibility (Variables|Default|GetChargedLaser) false true))

(fn RotateAround
  (Transformation|AddLocalRotation (Variables|Character|GetMesh) (Math|Rotator|MakeRotator 0.0 0.0 (* (Variables|Default|GetRotationSpeed) (Utilities|Time|GetWorldDeltaSeconds))) false false))

(fn SpinningLaseron
  (Rendering|SetVisibility (Variables|Default|GetBP_LaserBeam) true true)
  (Variables|Default|SetIsSpinLaserOn true))

(fn SpinningLaserOff
  (Rendering|SetVisibility (Variables|Default|GetBP_LaserBeam) false true)
  (Variables|Default|SetIsSpinLaserOn false))

(fn SpiningLaserFlip
  (if (Variables|Default|GetIsSpinLaserOn)
    (SpinningLaser|SpinningLaserOff)
    (else
      (SpinningLaser|SpinningLaseron))))

(fn FireLaserWave
  (bind _mesh (Variables|Character|GetMesh))
  (Game|SpawnActorfromClass "/Game/Enemies/Boss/First/Laser/BP_LaserWave.BP_LaserWave_C" (Math|Transform|MakeTransform (.location (Transformation|GetSocketTransform _mesh "WaveSocket" "RTS_World")) (Transformation|GetWorldRotation _mesh) "1.000000,1.000000,1.000000") "Undefined" "MultiplyWithRoot" 0 0.0 3e+03 "0.900000,2.000000,2.000000" "/Game/Enemies/Boss/First/Laser/Materials/MI_BaseLaser_Green.MI_BaseLaser_Green" false true 5.0 0 "/Game/Enemies/Boss/First/Laser/Materials/M_BaseLaser.M_BaseLaser"))

(fn FadeAimingLaser
  (Niagara|SetNiagaraVariable(LinearColor) (Variables|Default|GetAimingLaser) "BeamColor" (Math|Color|MakeColor 1.0 0.0 0.0)))

(fn SpawnShockWave
  (bind _mesh (Variables|Character|GetMesh))
  (bind _returnvalue (Transformation|GetWorldLocation _mesh))
  (Game|SpawnActorfromClass "/Game/Enemies/Boss/First/Laser/BP_Shockwave.BP_ShockWave_C" (Math|Transform|MakeTransform (Math|Vector|MakeVector (.x _returnvalue) (.y _returnvalue) (- (.z (Transformation|GetWorldLocation (Variables|Default|GetBP_LaserBeam))) 1e+01)) "0, 0, 0" "1.000000,1.000000,1.000000") "Undefined" "MultiplyWithRoot" 0 "1.000000,1.000000,1.000000" "/Game/Enemies/Boss/First/Laser/Materials/MI_BaseLaser_Green.MI_BaseLaser_Green" true true (Variables|Default|GetShockwaveDamage) 0 "/Game/Enemies/Boss/First/Laser/Materials/M_BaseLaser.M_BaseLaser")
  (ShockWave|CheckifPlayerUnder))

(fn CheckifPlayerUnder
  (if (<= (Transformation|GetDistanceTo (Game|Player|GetPlayerPawn 0) self) 5e+02)
    (Default|DecreaseHealth (Variables|/Game/ThirdPerson/Blueprints/BP_ThirdPersonCharacter.BP_ThirdPersonCharacter_C|GetBPC_PlayerStats (Variables|Default|GetPlayerRef_0)) 5e+03)))

(fn ResetBaseComps
  (Transformation|SetWorldRotation (Variables|Character|GetMesh) "0, 0, 0" false false)
  (A1|ChargeLaserFireOff)
  (A1|AimingLaserOff)
  (SpinningLaser|SpinningLaserOff))