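; Boss enemy with health bar, knockback on hit and charge laser, laser wave, spinning laser, slam shockwave and flying bullet-hell attacks.
; A StateTree runs attacks, which report completion through CallOnFinishAttack.
; Player time switches pause attacks in the present via timers, time dilation or StateTree stops, while health regenerates, and resume them in the past.
; BeginPlay pre-spawns pooled waves and a reusable shockwave; montage notifies time the slam's damage trace.
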(event Custom|OnTimeChange_Event
  (params (InPresent :type Boolean))
  (bind _returnvalue (Transformation|GetActorLocation))
  (bind _returnvalue_2 (Game|GetPlayerCharacter 0))
  (bind _returnvalue_3 (Transformation|GetActorLocation))
  (bind _returnvalue_4 (Game|GetPlayerCharacter 0))
  (bind _returnvalue_5 (Transformation|GetActorLocation _returnvalue_2))
  (bind _returnvalue_6 (Transformation|GetActorLocation _returnvalue_4))
  (bind _returnvalue_7 (- (.z _returnvalue) 2e+02))
  (bind _returnvalue_8 (Math|Vector|MakeVector (.x _returnvalue) (.y _returnvalue) _returnvalue_7))
  ;[0 0.2405 1] If the player switch time, pause/unpause the attack
  (if InPresent
    (Default|CallOnPause)
    ;;[1 1 1] Player Switch to Present
    ;;;[1 1 1] Pause the attack when player in present
    (if (Variables|BulletHell|GetInBulletHellAttack)
      (if (or (Variables|BulletHell|GetBHMovingUp) (Variables|BulletHell|GetBHMovingDown))
        (Variables|Default|SetCustomTimeDilation 0.0))
      (else
        (switch int (Variables|Default|GetCurrentAttackID)
          (:0
            ;;;;[1 1 1] Charge Laser
            (Utilities|Time|PauseTimerbyHandle (Variables|ChargeLaser|GetFireTimer)))
          (:1
            ;;;;[1 1 1] Laser Wave
            (AI|ClearFocus (AI|GetAIController self))
            (AI|Logic|StopLogic (Variables|Default|GetStateTree) ""))
          (:2
            ;;;;[1 1 1] Spinning Laser & Shockwave
            (Variables|Default|SetCustomTimeDilation 0.0 :!label _label))
          (:3
            (goto _label)))))
    (else
      (Default|CallOnUnPause)
      (if (Variables|BulletHell|GetInBulletHellAttack)
        ;;[1 1 1] Player Switch to Past
        (if (or (Variables|BulletHell|GetBHMovingUp) (Variables|BulletHell|GetBHMovingDown))
          (Variables|Default|SetCustomTimeDilation 1.0))
        (else
          (Utilities|FlowControl|Sequence
            (:then_0
              ;;;[1 1 1] Start the state tree when first counter
              (Utilities|FlowControl|DoOnce false
                (:Completed
                  (AI|Logic|StartLogic (Variables|Default|GetStateTree)))))
            (:then_1
              ;;;[1 1 1] Continue the attack when player back
              (switch int (Variables|Default|GetCurrentAttackID)
                (:0
                  ;;;;[1 1 1] Charge Laser
                  (Utilities|Time|UnpauseTimerbyHandle (Variables|ChargeLaser|GetFireTimer)))
                (:1
                  ;;;;[1 1 1] Laser Wave
                  (Class|BrainComponent|RestartLogic (Variables|Default|GetStateTree)))
                (:2
                  ;;;;[1 1 1] Spinning Laser & Shockwave
                  (Variables|Default|SetCustomTimeDilation 1.0 :!label _label_2))
                (:3
                  (goto _label_2))))
            (:then_2
              ;;;[1 1 1] Check if player is inside the boss when time switch
              (Utilities|FlowControl|Delay 0.1)
              (bind _outhit (Collision|SphereTraceByChannel _returnvalue_8 _returnvalue_8 2e+02 "TraceTypeQuery4" false 0 "ForDuration"))
              (if (== (.HitActor (Collision|BreakHitResult _outhit)) _returnvalue_2)
                ;;;;[1 1 1] Teleport
                (Transformation|SetActorLocation _returnvalue_4 (Math|Interpolation|VInterpTo _returnvalue_6 (+ _returnvalue_6 (* (Math|Vector|Normalize (- (Math|Vector|MakeVector (.x _returnvalue_5) (.y _returnvalue_5) 0.0) (Math|Vector|MakeVector (.x _returnvalue_3) (.y _returnvalue_3) 0.0))) 3e+02)) (Utilities|Time|GetWorldDeltaSeconds) 3e+01) false false)))))))))

(event Custom|StartChargeLaser
  (params (TargetFocus :type Actor%20Object%20Reference))
  ;[1 0 0.09432] Attacks
  ;;[1 1 1] Charge Laser
  (Variables|ChargeLaser|SetAttackDone false)
  (LaserControllers|AimLaseron)
  (Variables|ChargeLaser|SetShouldRotate true)
  (AI|SetFocus (AI|GetAIController self) TargetFocus)
  (bind _returnvalue (Utilities|Time|SetTimerbyFunctionName 0 "StopMovement" (Variables|ChargeLaser|GetChargeLaserDuration)))
  (Variables|ChargeLaser|SetFireTimer _returnvalue))

(event Custom|BH_Pattern2
  (Default|CallOnLaserGridStart))

(event Custom|ContinueMoveUp
  (bind _returnvalue (Transformation|GetActorLocation))
  (bind _z_pos_ (Timeline|MoveUp Play)
    (:Update
      (Transformation|SetActorLocation (Math|Vector|MakeVector (.x _returnvalue) (.y _returnvalue) (+ (Variables|BulletHell|GetBossInitalZPos) _z_pos_)) false false))
    (:Finished
      (Variables|BulletHell|SetBHMovingUp false)
      (Default|CallOnBulletHellAttackStart))))

(event Custom|StopMoveUP
  (bind _returnvalue (Transformation|GetActorLocation))
  (bind _z_pos_ (Timeline|MoveUp Stop)
    (:Update
      (Transformation|SetActorLocation (Math|Vector|MakeVector (.x _returnvalue) (.y _returnvalue) (+ (Variables|BulletHell|GetBossInitalZPos) _z_pos_)) false false))
    (:Finished
      (Variables|BulletHell|SetBHMovingUp false)
      (Default|CallOnBulletHellAttackStart))))

(event Custom|Continue%20MoveDown
  (bind _returnvalue (Transformation|GetActorLocation))
  (bind _z_pos_ (Timeline|Timeline Play)
    (:Update
      (Transformation|SetActorLocation (Math|Vector|MakeVector (.x _returnvalue) (.y _returnvalue) (- (Variables|BulletHell|GetBossInitalZPos) _z_pos_)) false false)
      (CallFunction|BodyTrace))
    (:Finished
      (Variables|BulletHell|SetBHMovingDown false)
      (Pawn|Components|CharacterMovement|SetMovementMode (Variables|Character|GetCharacterMovement) "MOVE_Walking" 0)
      (Variables|BulletHell|SetInBulletHellAttack false)
      (Variables|Default|SetInSecondPhase true)
      (AI|ClearFocus (AI|GetAIController self))
      (Default|CallOnFinishAttack))))

(event Custom|Stop%20MoveDown
  (bind _returnvalue (Transformation|GetActorLocation))
  (bind _z_pos_ (Timeline|Timeline Stop)
    (:Update
      (Transformation|SetActorLocation (Math|Vector|MakeVector (.x _returnvalue) (.y _returnvalue) (- (Variables|BulletHell|GetBossInitalZPos) _z_pos_)) false false)
      (CallFunction|BodyTrace))
    (:Finished
      (Variables|BulletHell|SetBHMovingDown false)
      (Pawn|Components|CharacterMovement|SetMovementMode (Variables|Character|GetCharacterMovement) "MOVE_Walking" 0)
      (Variables|BulletHell|SetInBulletHellAttack false)
      (Variables|Default|SetInSecondPhase true)
      (AI|ClearFocus (AI|GetAIController self))
      (Default|CallOnFinishAttack))))

(event Custom|BH%20MoveDown
  (bind _returnvalue (Transformation|GetActorLocation))
  (Variables|BulletHell|SetBossInitalZPos (.z (Transformation|GetActorLocation)))
  (Variables|BulletHell|SetBHMovingDown true)
  (bind _z_pos_ (Timeline|Timeline PlayFromStart)
    (:Update
      (Transformation|SetActorLocation (Math|Vector|MakeVector (.x _returnvalue) (.y _returnvalue) (- (Variables|BulletHell|GetBossInitalZPos) _z_pos_)) false false)
      (CallFunction|BodyTrace))
    (:Finished
      (Variables|BulletHell|SetBHMovingDown false)
      (Pawn|Components|CharacterMovement|SetMovementMode (Variables|Character|GetCharacterMovement) "MOVE_Walking" 0)
      (Variables|BulletHell|SetInBulletHellAttack false)
      (Variables|Default|SetInSecondPhase true)
      (AI|ClearFocus (AI|GetAIController self))
      (Default|CallOnFinishAttack))))

(event Custom|InChargeLaser
  (params (TargetLocation :type Vector))
  ;[1 0 0.09432] Attacks
  ;;[1 1 1] Charge Laser
  (Utilities|FlowControl|Sequence
    (:then_0
      (if (Variables|ChargeLaser|GetShouldRotate)
        (Rotation|RotateEyeMesh TargetLocation)
        (elif (Variables|ChargeLaser|GetAttackDone)
          (bind _isrotresetdone (Rotation|ResetEyeMeshRotation))
          (LaserControllers|ChargedLaserOff)
          (if _isrotresetdone
            (Math|Integer|IncrementInt (Variables|Default|GetCurrentAttackID)
              (:%20%20
                (Utilities|Time|ClearandInvalidateTimerbyHandle (Variables|ChargeLaser|GetFireTimer))
                (Default|CallOnFinishAttack))))
          (else
            (Utilities|FlowControl|Delay 2.0)
            (Variables|ChargeLaser|SetAttackDone true)))))
    (:then_1
      (if (<= (Utilities|Time|GetTimerRemainingTimebyHandle (Variables|ChargeLaser|GetFireTimer)) 1.0)
        (LaserControllers|SetBeamColor true)))))

(event Custom|Shockwave
  ;[1 0 0.09432] Attacks
  ;;[1 1 1] Shockwave
  ;;;[1 1 1] Animation
  (bind _notifyname (Animation|Montage|PlayMontage (Variables|Character|GetMesh) "/Game/Enemies/Boss/First/Assets/AM_Boss_SlamDown.AM_Boss_SlamDown" 0.7)
    (:OnCompleted
      (Math|Integer|IncrementInt (Variables|Default|GetCurrentAttackID)
        (:%20%20
          (Default|CallOnFinishAttack))))
    (:OnNotifyBegin
      (switch name _notifyname
        (:BodySlam
          (CallFunction|StartBodyTrace))
        (:ShockWave
          (Default|Fire (Variables|Shockwave|GetShockWaveBP)))))
    (:OnNotifyEnd
      (switch name _notifyname
        (:BodySlam
          (CallFunction|StopBodyTrace))))))

(event Custom|BodyTrace
  (bind _returnvalue (Transformation|GetActorLocation))
  (bind _returnvalue_2 (- (.z _returnvalue) 2e+02))
  (bind _returnvalue_3 (Math|Vector|MakeVector (.x _returnvalue) (.y _returnvalue) _returnvalue_2))
  ;[1 0 0.09432] Attacks
  ;;[1 1 1] Shockwave
  ;;;[1 1 1] Trace to check if player is under during shockwave
  (bind _outhit (Collision|SphereTraceByChannel _returnvalue_3 _returnvalue_3 3e+02 "TraceTypeQuery4" false 0 "None"))
  (if (== (.HitActor (Collision|BreakHitResult _outhit)) (Game|GetPlayerCharacter 0))
    (Utilities|FlowControl|DoOnce false
      (:Completed
        (Default|DecreaseHealth (Variables|/Game/ThirdPerson/Blueprints/BP_ThirdPersonCharacter.BP_ThirdPersonCharacter_C|GetBPC_PlayerStats (Variables|Default|GetPlayerRef)) 5e+03)))))

(event Custom|SpinningLaser
  ;[1 0 0.09432] Attacks
  ;;[1 1 1] Spinning Laser
  (Animation|Montage|PlayMontage (Variables|Character|GetMesh) "/Game/Enemies/Boss/First/Assets/AM_BossSpin.AM_BossSpin"
    (:OnCompleted
      (Math|Integer|IncrementInt (Variables|Default|GetCurrentAttackID)
        (:%20%20
          (Default|CallOnFinishAttack))))))

(event Custom|StopBodyTrace
  ;[1 0 0.09432] Attacks
  ;;[1 1 1] Shockwave
  ;;;[1 1 1] Trace to check if player is under during shockwave
  (Utilities|Time|ClearandInvalidateTimerbyHandle (Variables|Shockwave|GetBodyTraceTimer))
  (Utilities|FlowControl|DoOnce false) ; enters at Reset
)

(event Custom|StartBodyTrace
  ;[1 0 0.09432] Attacks
  ;;[1 1 1] Shockwave
  ;;;[1 1 1] Trace to check if player is under during shockwave
  (bind _returnvalue (Utilities|Time|SetTimerbyEvent (delegate Custom|BodyTrace) 0.01 true))
  (Variables|Shockwave|SetBodyTraceTimer _returnvalue))

(event Custom|BH_Pattern1
  (bind _returnvalue (Transformation|GetActorLocation))
  (AI|SetFocus (AI|GetAIController self) (Variables|Default|GetPlayerRef))
  (Variables|BulletHell|SetInBulletHellAttack true)
  (Pawn|Components|CharacterMovement|SetMovementMode (Variables|Character|GetCharacterMovement) "MOVE_Flying" 0)
  (Variables|BulletHell|SetBossInitalZPos (.z (Transformation|GetActorLocation)))
  (Variables|BulletHell|SetBHMovingUp true)
  (bind _z_pos_ (Timeline|MoveUp PlayFromStart)
    (:Update
      (Transformation|SetActorLocation (Math|Vector|MakeVector (.x _returnvalue) (.y _returnvalue) (+ (Variables|BulletHell|GetBossInitalZPos) _z_pos_)) false false))
    (:Finished
      (Variables|BulletHell|SetBHMovingUp false)
      (Default|CallOnBulletHellAttackStart))))

(event Custom|OnBH1AttackEnd_Event
  (Default|CallOnFinishAttack))

(event EventBeginPlay
  (bind _mesh (Variables|Character|GetMesh))
  (bind _mesh_2 (Variables|Character|GetMesh))
  (bind _returnvalue (Transformation|GetWorldLocation _mesh_2))
  (Utilities|FlowControl|Sequence
    (:then_0
      ;[1 1 1] Sets up health bar
      (bind _returnvalue_2 (UserInterface|CreateWidget "/Game/UI/Boss/WB_BossBar_Monika.WB_BossBar_Monika_C"))
      (UserInterface|Viewport|AddtoViewport _returnvalue_2 0)
      (Variables|Components|SetHealthBar _returnvalue_2))
    (:then_1
      ;[1 1 1] Sets up player ref for timeline checks
      (bind _asbp_third_person_character (Utilities|Casting|CastToBP_ThirdPersonCharacter (Game|GetPlayerCharacter 0)))
      (Variables|Default|SetPlayerRef _asbp_third_person_character)
      ;[1 1 1] Event binding to check whether player swicth time
      (EventDispatchers|AssignOnTimeChange _asbp_third_person_character (EventDispatchers|CreateEvent :!event Custom|OnTimeChange_Event)))
    (:then_2
      ;[1 1 1] creating object pool for laser wave
      (for _index (range 1 (Variables|LaserWave|GetNumLaserWaves))
        (bind _returnvalue_3 (Game|SpawnActorfromClass "/Game/Enemies/Boss/First/Laser/BP_LaserWave.BP_LaserWave_C" (Math|Transform|MakeTransform (.location (Transformation|GetSocketTransform _mesh "WaveSocket" "RTS_World")) (Transformation|GetWorldRotation _mesh) "1.000000,1.000000,1.000000") "Undefined" "MultiplyWithRoot" self (Variables|LaserWave|GetWaveLifeSpan) (Variables|LaserWave|GetWave%20Speed) "0.900000,2.000000,2.000000" "/Game/Enemies/Boss/First/Laser/Materials/M_BaseLaser.M_BaseLaser" false true (Variables|LaserWave|GetLaserWaveDamage) 0))
        (Utilities|Array|Add (Variables|LaserWave|GetLaserWavePool) _returnvalue_3)))
    (:then_3
      ;[1 1 1] Create Shockwave
      (bind _returnvalue_4 (Game|SpawnActorfromClass "/Game/Enemies/Boss/First/Laser/BP_Shockwave.BP_ShockWave_C" (Math|Transform|MakeTransform (Math|Vector|MakeVector (.x _returnvalue) (.y _returnvalue) (- (.z (Transformation|GetWorldLocation (Variables|Default|GetBP_LaserBeam))) 1e+01)) "0, 0, 0" "1.000000,1.000000,1.000000") "Undefined" "MultiplyWithRoot" self "1.000000,1.000000,1.000000" "/Game/Enemies/Boss/First/Laser/Materials/M_BaseLaser.M_BaseLaser" true true (Variables|Shockwave|GetShockwaveDamage) 0))
      (Variables|Shockwave|SetShockWaveBP _returnvalue_4))
    (:then_4
      (bind _returnvalue_5 (Actor|GetActorOfClass "/Game/Enemies/Boss/First/Laser/BulletHell/BP_BulletHellManager.BP_BulletHellManager_C"))
      (EventDispatchers|AssignOnAttackEnd _returnvalue_5 (delegate Custom|OnBH1AttackEnd_Event)))))

(event EventTick
  (params (DeltaSeconds :type Float%20%28single-precision%29))
  (bind _bpc_playerstats (Variables|Default|GetBPC_PlayerStats))
  (if (Variables|Rotation|GetIsSpininngLaserOn)
    (Transformation|SetWorldRotation (Variables|Default|GetSpiningLaser) (Math|Rotator|MakeRotator 0.0 0.0 (.yaw (Transformation|GetSocketRotation (Variables|Character|GetMesh) "BottomSocket"))) false false))
  ;[1 1 1] Increase boss health
  (if (Variables|/Game/ThirdPerson/Blueprints/BP_ThirdPersonCharacter.BP_ThirdPersonCharacter_C|GetInPresent (Variables|Default|GetPlayerRef))
    (if (<= (Variables|/Game/ThirdPerson/Blueprints/BPC_PlayerStats.BPC_PlayerStats_C|GetCurrentHealth _bpc_playerstats) (Variables|/Game/ThirdPerson/Blueprints/BPC_PlayerStats.BPC_PlayerStats_C|GetMaxHealth _bpc_playerstats))
      (Default|DecreaseHealth (Variables|Default|GetBPC_PlayerStats) (* (Variables|Health|GetHealthRegen) (Utilities|Time|GetWorldDeltaSeconds)))
      (Default|UpdateHealthBar (Variables|Components|GetHealthBar)))))

(event Game|Damage|EventAnyDamage
  (params (Damage :type Float%20%28single-precision%29) (DamageType :type Damage%20Type%20Object%20Reference) (InstigatedBy :type Controller%20Object%20Reference) (DamageCauser :type Actor%20Object%20Reference))
  (bind _returnvalue (Transformation|GetActorLocation))
  (bind _returnvalue_2 (Game|GetPlayerCharacter 0))
  (bind _bpc_playerstats (Variables|Default|GetBPC_PlayerStats))
  (bind _bpc_playerstats_2 (Variables|Default|GetBPC_PlayerStats))
  (bind _returnvalue_3 (Transformation|GetActorLocation _returnvalue_2))
  ;[1 1 1] Take damage from player
  (if (Variables|/Game/ThirdPerson/Blueprints/BPC_PlayerStats.BPC_PlayerStats_C|GetCanTakeDamage (Variables|Default|GetBPC_PlayerStats))
    (Utilities|FlowControl|Sequence
      (:then_0
        (Default|CallOnDamaged)
        (Character|LaunchCharacter _returnvalue_2 (* (Math|Vector|Normalize (- (Math|Vector|MakeVector (.x _returnvalue_3) (.y _returnvalue_3) 0.0) (Math|Vector|MakeVector (.x _returnvalue) (.y _returnvalue) 0.0))) (Variables|Default|GetKnockback%20Launch)) true false)
        (Default|DecreaseHealth _bpc_playerstats_2 Damage)
        (Variables|/Game/ThirdPerson/Blueprints/BPC_PlayerStats.BPC_PlayerStats_C|SetCanTakeDamage _bpc_playerstats_2 false)
        (Utilities|FlowControl|Delay 0.4)
        (Variables|/Game/ThirdPerson/Blueprints/BPC_PlayerStats.BPC_PlayerStats_C|SetCanTakeDamage _bpc_playerstats_2 true)
        (Default|UpdateHealthBar (Variables|Components|GetHealthBar)))
      (:then_1
        ;[1 1 1] Can Do Bullet Hell once more if near death
        (if (<= (/ (Variables|/Game/ThirdPerson/Blueprints/BPC_PlayerStats.BPC_PlayerStats_C|GetCurrentHealth _bpc_playerstats) (Variables|/Game/ThirdPerson/Blueprints/BPC_PlayerStats.BPC_PlayerStats_C|GetMaxHealth _bpc_playerstats)) (Variables|Health|GetHealth_NearDeath%28Percent%29))
          (Utilities|FlowControl|DoOnce false
            (:Completed
              (Variables|BulletHell|SetCanUseBulletHell true))))))))

(fn ConstructionScript
  ;[1 1 1] Hides all attached lasers on start
  (LaserControllers|AimLaserOff)
  (LaserControllers|SpinningLaserOff)
  (LaserControllers|ChargedLaserOff))

(fn RotateEyeMesh
  (params (TargetLocation :type Vector))
  (bind _mesh (Variables|Character|GetMesh))
  (bind _returnvalue (Transformation|GetWorldRotation _mesh))
  ;[1 1 1] Rotate the eye on y axis towards the player
  (Transformation|SetWorldRotation (Variables|Character|GetMesh) (Math|Rotator|MakeRotator (.roll _returnvalue) (.pitch (Math|Interpolation|RInterpTo (Transformation|GetWorldRotation _mesh) (Math|Rotator|FindLookatRotation (Transformation|GetWorldLocation _mesh) (- TargetLocation (Math|Vector|MakeVector 0.0 0.0 (Variables|Rotation|GetAimRotationOffset)))) (Utilities|Time|GetWorldDeltaSeconds) (Variables|Rotation|GetLookSpeed))) (.yaw _returnvalue)) false false))

(fn ResetEyeMeshRotation
  (bind _mesh (Variables|Character|GetMesh))
  (bind _relativerotation (Variables|/Script/Engine.SceneComponent|GetRelativeRotation _mesh))
  ;[1 1 1] Resets the eye rotation compared to the capsule
  (Transformation|SetRelativeRotation (Variables|Character|GetMesh) (Math|Interpolation|RInterpTo _relativerotation "0, 0, 0" (Utilities|Time|GetWorldDeltaSeconds) (Variables|Rotation|GetLookSpeed)) false false)
  ;[1 1 1] Checks if the eye mesh has returned to the original rotation
  (if (Utilities|Operators|EqualEqual :A _relativerotation :ErrorTolerance 0.1)
    (Variables|Rotation|SetIsRotResetDone true))
  (return (Variables|Rotation|GetIsRotResetDone)))

(fn AimLaseron
  ;[1 1 1] Turns on visual effect for aiming
  (Rendering|SetVisibility (Variables|Default|GetAimingLaser) true false)
  (LaserControllers|SetBeamColor false))

(fn AimLaserOff
  ;[1 1 1] Turns aiming visual effect off.
  (Rendering|SetVisibility (Variables|Default|GetAimingLaser) false false))

(fn SpinningLaseron
  (Rendering|SetVisibility (Variables|Default|GetSpiningLaser) true true)
  (Variables|Rotation|SetIsSpininngLaserOn true))

(fn SpinningLaserOff
  (Rendering|SetVisibility (Variables|Default|GetSpiningLaser) false true)
  (Variables|Rotation|SetIsSpininngLaserOn false))

(fn ChargedLaseron
  ;[1 1 1] Turns on damaging laser
  (Rendering|SetVisibility (Variables|Default|GetChargedLaser) true true))

(fn ChargedLaserOff
  (Rendering|SetVisibility (Variables|Default|GetChargedLaser) false true))

(fn SpawnShockWave
  (bind _mesh (Variables|Character|GetMesh))
  (bind _returnvalue (Transformation|GetWorldLocation _mesh))
  (Game|SpawnActorfromClass "/Game/Enemies/Boss/First/Laser/BP_Shockwave.BP_ShockWave_C" (Math|Transform|MakeTransform (Math|Vector|MakeVector (.x _returnvalue) (.y _returnvalue) (- (.z (Transformation|GetWorldLocation (Variables|Default|GetBP_LaserBeam))) 1e+01)) "0, 0, 0" "1.000000,1.000000,1.000000") "Undefined" "MultiplyWithRoot" 0 "1.000000,1.000000,1.000000" "/Game/Enemies/Boss/First/Laser/Materials/M_BaseLaser.M_BaseLaser" true true (Variables|Shockwave|GetShockwaveDamage) 0)
  (ShockWave|CheckifPlayerUnder))

(fn CheckifPlayerUnder
  (if (<= (Transformation|GetDistanceTo (Game|Player|GetPlayerPawn 0) self) 5e+02)
    (Default|DecreaseHealth (Variables|/Game/ThirdPerson/Blueprints/BP_ThirdPersonCharacter.BP_ThirdPersonCharacter_C|GetBPC_PlayerStats (Variables|Default|GetPlayerRef)) 5e+03)))

(fn SpinningLaserFlip
  (if (Variables|Rotation|GetIsSpininngLaserOn)
    (LaserControllers|SpinningLaserOff)
    (else
      (LaserControllers|SpinningLaseron))))

(fn SetBeamColor
  (params (Red :type Boolean))
  (bind _aiminglaser (Variables|Default|GetAimingLaser))
  (if Red
    (Niagara|SetNiagaraVariable(LinearColor) _aiminglaser "BeamColor" (Math|Color|MakeColor 1.0 0.0 0.0))
    (else
      (Niagara|SetNiagaraVariable(LinearColor) _aiminglaser "BeamColor" (Math|Color|MakeColor 0.0 1.0 0.0)))))

(fn StopMovement
  (Variables|ChargeLaser|SetShouldRotate false)
  (AI|ClearFocus (AI|GetAIController self))
  (LaserControllers|AimLaserOff)
  (LaserControllers|ChargedLaseron))