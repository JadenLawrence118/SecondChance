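; Orion boss character with overhead swing, sweep, timed block and backward dodge actions.
; Montage notifies toggle BPCSwordTrace melee traces, target-facing rotation on Tick and dodge movement in Flying mode.
; The overhead swing predicts the target's position from its velocity and lunges there on a timeline.
; Blocking drives ABP_Orion and damages the player back when a yaw check passes; swings and block signal attack end on completion.
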(event Custom|OverheadSwing
  (params (Target%20Actor :type Actor%20Object%20Reference))
  (bind _returnvalue (Transformation|GetActorLocation))
  (bind (_x _y _z) (Math|Vector|BreakVector _returnvalue))
  ;[1 1 1] Attack 1 : Overhead Swing
  (Variables|Default|SetTarget%20Actor Target%20Actor)
  (bind _notifyname (Animation|Montage|PlayMontage (Variables|Character|GetMesh) "/Game/Art/Characters/Orion/Animations/AM_OverheadSwing.AM_OverheadSwing")
    (:OnCompleted
      (Default|CallOnAttackEnd))
    (:OnNotifyBegin
      (switch name _notifyname
        (:SwordTrace
          (Default|StartMeleeTrace (Variables|Default|GetBPC_SwordTrace) (Variables|Default|GetSwordTraceTop) (Variables|Default|GetSwordTraceEnd) (Variables|Default|GetSword%20Trace%20Radius) 1e+01 0.001)
          (bind _x_y_movement (Timeline|MoveToPlayer PlayFromStart)
            (:Update
              (Transformation|SetActorLocation (Math|Vector|MakeVector (Math|Float|Lerp _x (.X (Math|Vector|BreakVector (- (Variables|Default|GetAttackDestination) (* (Math|Vector|Normalize (- (Variables|Default|GetAttackDestination) _returnvalue)) 5e+01)))) _x_y_movement) (Math|Float|Lerp _y (.Y (Math|Vector|BreakVector (- (Variables|Default|GetAttackDestination) (* (Math|Vector|Normalize (- (Variables|Default|GetAttackDestination) _returnvalue)) 5e+01)))) _x_y_movement) _z) false false))))
        (:LookAtTarget
          (Variables|Default|SetIsTracingTarget true))))
    (:OnNotifyEnd
      (switch name _notifyname
        (:SwordTrace
          (Default|StopMeleeTrace (Variables|Default|GetBPC_SwordTrace)))
        (:LookAtTarget
          (Variables|Default|SetIsTracingTarget false)
          (Variables|Default|SetAttackDestination (+ (Transformation|GetActorLocation (Variables|Default|GetTarget%20Actor)) (/ (Transformation|GetVelocity (Variables|Default|GetTarget%20Actor)) 1e+01))))))))

(event Custom|Block
  ;[1 1 1] Attack 2 : Block
  (Variables|Default|SetIsBlocking true)
  (bind _asabp_orion (Utilities|Casting|CastToABP_Orion (Components|SkeletalMesh|GetAnimInstance (Variables|Character|GetMesh))))
  (Variables|/Game/Enemies/Boss/Orion/ABP_Orion.ABP_Orion_C|SetIsBlocking _asabp_orion true)
  (bind _returnvalue (Utilities|Time|SetTimerbyEvent (delegate Custom|BlockEnd) (Variables|Default|GetBlock%20Durartion)))
  (Variables|Default|SetTimer _returnvalue))

(event Custom|BlockEnd
  ;[1 1 1] Attack 2 : Block
  (Variables|Default|SetIsBlocking false)
  (bind _asabp_orion (Utilities|Casting|CastToABP_Orion (Components|SkeletalMesh|GetAnimInstance (Variables|Character|GetMesh))))
  (Variables|/Game/Enemies/Boss/Orion/ABP_Orion.ABP_Orion_C|SetIsBlocking _asabp_orion false)
  (Default|CallOnAttackEnd))

(event Custom|Sweep
  (params (Target%20Actor :type Actor%20Object%20Reference))
  ;[1 1 1] Attack 3 : Sweep
  (Variables|Default|SetTarget%20Actor Target%20Actor)
  (bind _notifyname (Animation|Montage|PlayMontage (Variables|Character|GetMesh) "/Game/Art/Characters/Orion/Animations/AM_Sweep.AM_Sweep")
    (:OnCompleted
      (Default|CallOnAttackEnd))
    (:OnNotifyBegin
      (switch name _notifyname
        (:SwordTrace
          (Default|StartMeleeTrace (Variables|Default|GetBPC_SwordTrace) (Variables|Default|GetSwordTraceTop) (Variables|Default|GetSwordTraceEnd) (Variables|Default|GetSword%20Trace%20Radius) 1e+01 0.001))
        (:LookAtTarget
          (Variables|Default|SetIsTracingTarget true))))
    (:OnNotifyEnd
      (switch name _notifyname
        (:SwordTrace
          (Default|StopMeleeTrace (Variables|Default|GetBPC_SwordTrace)))
        (:LookAtTarget
          (Variables|Default|SetIsTracingTarget false))))))

(event Custom|Dodge
  (bind _charactermovement (Variables|Character|GetCharacterMovement))
  (bind _capsulecomponent (Variables|Default|GetCapsuleComponent))
  ;[1 1 1] Attack 2: Dodge Back
  (bind _notifyname (Animation|Montage|PlayMontage (Variables|Default|GetMesh) 0)
    (:OnNotifyBegin
      (switch name _notifyname
        (:Move
          (Variables|/Script/Engine.MovementComponent|SetVelocity _charactermovement "0, 0, 0")
          (Pawn|Components|CharacterMovement|SetMovementMode _charactermovement "MOVE_Flying" 0)
          (Components|MoveComponentTo _capsulecomponent (- (Transformation|GetWorldLocation _capsulecomponent) (* (Math|Vector|GetForwardVector _capsulecomponent) (Variables|Default|GetDodgeDistance))) (Variables|/Script/Engine.SceneComponent|GetRelativeRotation _capsulecomponent) false false 0.2 false))
        (:Jump
          (Variables|/Script/Engine.MovementComponent|SetVelocity (Variables|Character|GetCharacterMovement) "0.000000,0.000000,50.000000"))))
    (:OnNotifyEnd
      (switch name _notifyname
        (:Move
          (Pawn|Components|CharacterMovement|SetMovementMode (Variables|Character|GetCharacterMovement) "MOVE_Walking" 0))))))

(event Custom|test
  ;[0.09321 1 0.9702] Function for testing
  (Variables|Default|SetTarget%20Actor (Game|GetPlayerCharacter 0)))

(event EventBeginPlay)

(event Collision|EventActorBeginOverlap
  (params (OtherActor :type Actor%20Object%20Reference)))

(event EventTick
  (params (DeltaSeconds :type Float%20%28single-precision%29))
  ;[1 1 1] Rotate to focus on Target when telegraphing
  (if (Variables|Default|GetIsTracingTarget)
    (Variables|Default|SetRotationLerp (Math|Float|Clamp(Float) (+ (Variables|Default|GetRotationLerp) 0.01)))
    (Transformation|SetActorRotation (Math|Rotator|Lerp(Rotator) (Transformation|GetActorRotation) (Math|Rotator|FindLookatRotation (Transformation|GetActorLocation) (Transformation|GetActorLocation (Variables|Default|GetTarget%20Actor))) (Variables|Default|GetRotationLerp)))))

(event Game|Damage|EventAnyDamage
  (params (Damage :type Float%20%28single-precision%29) (DamageType :type Damage%20Type%20Object%20Reference) (InstigatedBy :type Controller%20Object%20Reference) (DamageCauser :type Actor%20Object%20Reference))
  ;[1 1 1] Attack 2 : Block
  (if (and (Variables|Default|GetIsBlocking) (<= (Math|Float|Absolute(Float) (.yaw (Math|Rotator|FindLookatRotation (Transformation|GetActorLocation) (Transformation|GetActorLocation (Game|GetPlayerCharacter 0))))) (Variables|Default|GetValidBlcokAngle)))
    (Game|Damage|ApplyDamage (Game|GetPlayerCharacter 0) 5.0 0 0)))

(fn ConstructionScript
  (Components|SkinnedMesh|SetLeaderPoseComponent (Variables|Default|GetSword) (Variables|Character|GetMesh) false false))