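; Enemy spawner that delivers reinforcement waves of a configurable enemy type via a dropship once few enough remain.
; BeginPlay counts existing enemies, finds the enemy counter and collects the BP_SpawnerPos actors targeting this spawner.
; SpawnEnemies checks the threshold, shows the dropship with sound and starts a timer that spawns enemies at the spawner's transform.
; After each wave it sets the counter aggressive, hides the dropship, cycles to the next position and yaws 90 degrees.
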(event Custom|SpawnEnemies
  ;[1 1 1] Set the enemy type you want to spawn in EnemyType, the number of enemies to spawn in NumberToSpawn, and the number of that type of enemy left in the world that triggers a respawn in NumberLeftWhenSpawn
  (if (not (Variables|Default|GetisSpawning))
    (if (<= (Variables|Default|GetEnemiesLeft) (+ (Variables|Default|GetNumberLeftWhenSpawn) 1))
      (Rendering|SetVisibility (Variables|Default|GetSM_Dropship) true false)
      (Audio|PlaySound2D "/Game/SoundEffects/SoundFX/nmeDropShip_FS.nmeDropShip_FS" 1.0 1.0 0.0 0 0)
      (bind _returnvalue (Utilities|Time|SetTimerbyEvent (delegate Custom|Spawn) (Variables|Default|GetSpawnDelay) (Variables|Default|GetEventLooping))))))

(event Custom|Spawn
  (bind _returnvalue (Transformation|GetActorRotation))
  ;[1 1 1] Set the enemy type you want to spawn in EnemyType, the number of enemies to spawn in NumberToSpawn, and the number of that type of enemy left in the world that triggers a respawn in NumberLeftWhenSpawn
  (Variables|Default|SetisSpawning true)
  (Game|SpawnActorfromClass (Variables|Default|GetEnemyType) (Transformation|GetActorTransform) "Undefined" "MultiplyWithRoot" 0 0)
  (bind _result (Math|Integer|IncrementInt (Variables|Default|GetSpawnIndex))
    (:%20%20
      (if (not (< _result (Variables|Default|GetNumberToSpawn)))
        (Utilities|Time|ClearandInvalidateTimerbyHandle (stale Custom|SpawnEnemies _returnvalue))
        (Variables|Default|SetSpawnIndex 0)
        (Default|SetAggressive (Variables|Default|GetEnemyCounter))
        ;;[1 1 1] Rotational spawning
        (Variables|Default|SetisSpawning false)
        (Rendering|SetVisibility (Variables|Default|GetSM_Dropship) false false)
        (if (>= (Variables|Default|GetcurrentPosIndex) (- (Utilities|Array|Length (Variables|Default|GetSpawnPositions)) 1))
          (Variables|Default|SetcurrentPosIndex 0)
          (else
            (Math|Integer|IncrementInt (Variables|Default|GetcurrentPosIndex)
              (:%20%20
                _))))
        (Transformation|SetActorLocation (Transformation|GetActorLocation (Utilities|Array|Get(acopy) (Variables|Default|GetSpawnPositions) (Variables|Default|GetcurrentPosIndex))) false false)
        (Transformation|SetActorRotation (Math|Rotator|MakeRotator (.roll _returnvalue) (.pitch _returnvalue) (+ (.yaw _returnvalue) 9e+01)))))))

(event EventBeginPlay
  (bind _outactors (Actor|GetAllActorsOfClass (Variables|Default|GetEnemyType)))
  (Variables|Default|SetEnemiesLeft (Utilities|Array|Length _outactors))
  (bind _returnvalue (Actor|GetActorOfClass "/Game/Enemies/Spawner/BP_EnemyCounter.BP_EnemyCounter_C"))
  (Variables|Default|SetEnemyCounter _returnvalue)
  (bind _outactors_2 (Actor|GetAllActorsOfClass "/Game/Enemies/Spawner/BP_SpawnerPos.BP_SpawnerPos_C"))
  (for _array_element _outactors_2
    (if (== (Variables|/Game/Enemies/Spawner/BP_SpawnerPos.BP_SpawnerPos_C|GetTargetSpawner _array_element) self)
      (Utilities|Array|Add (Variables|Default|GetSpawnPositions) _array_element)))
  (Transformation|SetActorLocation (Transformation|GetActorLocation (Utilities|Array|Get(acopy) (Variables|Default|GetSpawnPositions) (Variables|Default|GetcurrentPosIndex))) false false))

(fn ConstructionScript)