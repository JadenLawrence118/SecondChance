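; Damageable dummy enemy that gets knocked back when hit and can act as a boss whose death wins the game.
; Hits launch it along the player's forward vector, harder for slam attacks, then reduce health through BPCPlayerStats, with a brief invulnerability window.
; On death it enables mesh physics and calls IncreaseTime on the player, then triggers GameWin if boss or destroys itself.
; Tick turns the health bar toward the camera.
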(event EventTick
  (params (DeltaSeconds :type Float%20%28single-precision%29))
  ;[1 1 1] Event Tick - currently makes tyhe enemy healthbar always look at the player
  (Transformation|SetWorldRotation (Variables|Default|GetHealthBarWidget) (Math|Rotator|FindLookatRotation (Transformation|GetWorldLocation (Variables|Default|GetHealthBarWidget)) (Transformation|GetWorldLocation (Variables|/Script/Engine.PlayerCameraManager|GetTransformComponent (Game|GetPlayerCameraManager 0)))) false false))

(event Game|Damage|EventAnyDamage
  (params (Damage :type Float%20%28single-precision%29) (DamageType :type Damage%20Type%20Object%20Reference) (InstigatedBy :type Controller%20Object%20Reference) (DamageCauser :type Actor%20Object%20Reference))
  ;[1 1 1] Event AnyDamage - When the dummy is hit it checks if it can take damage. If true the dummy is knocked back and takes damage. If health<0 the dummy dies and gets detroyed
  (if (Variables|Default|GetCanTakeDamage)
    (if (Variables|Default|GetIsSlamAttack)
      (Variables|Default|SetCanTakeDamage false)
      (bind _asbp_third_person_character (Utilities|Casting|CastToBP_ThirdPersonCharacter (Game|GetPlayerCharacter 0)))
      (Character|LaunchCharacter (* (Math|Vector|GetForwardVector (Transformation|GetActorRotation _asbp_third_person_character)) 2e+03) false false)
      (bind _isplayerdead (Default|DecreaseHealth (Variables|Default|GetBPC_playerStats) Damage))
      (if _isplayerdead
        (Collision|SetCollisionObjectType (Variables|Character|GetMesh) "ECC_PhysicsBody" :!label _label)
        (Physics|SetSimulatePhysics (Variables|Character|GetMesh) true)
        (Default|IncreaseTime (Variables|Default|GetPlayerBP))
        (if (Variables|Default|GetIsBoss)
          (Development|PrintString "boss")
          (Utilities|FlowControl|Delay 0.5)
          (Default|GameWin (Variables|Default|GetPlayerBP))
          (else
            (Development|PrintString "not boss")
            (Actor|DestroyActor)))
        (else
          (Utilities|FlowControl|Delay 0.2 :!label _label_2)
          (Variables|Default|SetCanTakeDamage true)))
      (else
        (Variables|Default|SetCanTakeDamage false)
        (bind _asbp_third_person_character_2 (Utilities|Casting|CastToBP_ThirdPersonCharacter (Game|GetPlayerCharacter 0)))
        (Character|LaunchCharacter (* (Math|Vector|GetForwardVector (Transformation|GetActorRotation _asbp_third_person_character_2)) 7.5e+02) false false)
        (bind _isplayerdead_2 (Default|DecreaseHealth (Variables|Default|GetBPC_playerStats) Damage))
        (if _isplayerdead_2
          (goto _label)
          (else
            (goto _label_2)))))))

(event EventBeginPlay
  ;[1 1 1] Begin Play - Gets the dummys health widget
  (bind _aswb_dummy_health (Utilities|Casting|CastToWB_DummyHealth (UserInterface|GetWidget (Variables|Default|GetHealthBarWidget))))
  (Variables|Default|SetEnemyHealthWidget _aswb_dummy_health)
  (bind _asbp_third_person_character (Utilities|Casting|CastToBP_ThirdPersonCharacter (Game|GetPlayerCharacter 0)))
  (Variables|Default|SetPlayerBP _asbp_third_person_character))

(fn ConstructionScript)