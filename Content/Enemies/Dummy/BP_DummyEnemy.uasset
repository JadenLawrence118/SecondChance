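; Training dummy enemy that runs the combat tutorial, creating a WB_Tutorial widget and walking the player through Combo 1, Combo 2, Slam, Surge and a final Fracture prompt.
; AnyDamage identifies the attack by checking which montage plays on the player's mesh, then plays dummy hit animations and widget success feedback.
; Active-stage flags and delayed prompt events sequence the stages, swapping button images and indexed name and description text.
; Fracture has no hit check and hides after a timer.
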(event Custom|Combo1Prompt
  ;[0.1456 0.2916 1] Set Up Combo 1 Prompt
  (Widget|SetVisibility (Variables|/Game/UI/Tutorial/WB_Tutorial.WB_Tutorial_C|GetLightPromptImage_3 (Variables|Default|GetTutorialUI)) "Collapsed")
  (Utilities|FlowControl|Delay 1.5)
  (CallFunction|DisplayNewInputs)
  (Variables|Default|SetCombo1EventActive true))

(event Custom|Combo2Prompt
  (bind _tutorialui (Variables|Default|GetTutorialUI))
  ;[0.7528 1 0.4937] Set Up Combo 2 Prompt
  (Appearance|SetBrushfromTexture (Variables|/Game/UI/Tutorial/WB_Tutorial.WB_Tutorial_C|GetLightPromptImage_1 _tutorialui) "/Game/UI/ButtonPrompts/waitstar.waitstar" false)
  (Widget|SetVisibility (Variables|/Game/UI/Tutorial/WB_Tutorial.WB_Tutorial_C|GetLightPromptImage_3 _tutorialui) "Visible")
  (Utilities|FlowControl|Delay 1.5)
  (CallFunction|DisplayNewInputs)
  (Variables|Default|SetCombo2EventActive true))

(event Custom|FracturePrompt
  (bind _tutorialui (Variables|Default|GetTutorialUI))
  (Widget|SetVisibility (Variables|/Game/UI/Tutorial/WB_Tutorial.WB_Tutorial_C|GetLightPromptImage_3 _tutorialui) "Collapsed")
  (Widget|SetVisibility (Variables|/Game/UI/Tutorial/WB_Tutorial.WB_Tutorial_C|GetLightPromptImage_2 _tutorialui) "Collapsed")
  (Widget|SetVisibility (Variables|/Game/UI/Tutorial/WB_Tutorial.WB_Tutorial_C|GetLightPromptImage_1 _tutorialui) "Collapsed")
  (Widget|SetVisibility (Variables|/Game/UI/Tutorial/WB_Tutorial.WB_Tutorial_C|GetLightPromptImage _tutorialui) "Collapsed")
  (Utilities|FlowControl|Delay 1.5)
  (CallFunction|DisplayNewInputs)
  (Utilities|FlowControl|Delay 7.0)
  (UserInterface|Animation|PlayAnimation _tutorialui (Variables|/Game/UI/Tutorial/WB_Tutorial.WB_Tutorial_C|GetHideInputs _tutorialui) 0.0 1 "Forward" 1.0 false))

(event Custom|SlamPrompt
  (bind _tutorialui (Variables|Default|GetTutorialUI))
  ;[1 0.4933 0.7452] Set Up Slam Prompt
  (Widget|SetVisibility (Variables|/Game/UI/Tutorial/WB_Tutorial.WB_Tutorial_C|GetLightPromptImage_1 _tutorialui) "Collapsed")
  (Widget|SetVisibility (Variables|/Game/UI/Tutorial/WB_Tutorial.WB_Tutorial_C|GetLightPromptImage_2 _tutorialui) "Collapsed")
  (Widget|SetVisibility (Variables|/Game/UI/Tutorial/WB_Tutorial.WB_Tutorial_C|GetLightPromptImage_3 _tutorialui) "Collapsed")
  (Appearance|SetBrushfromTexture (Variables|/Game/UI/Tutorial/WB_Tutorial.WB_Tutorial_C|GetLightPromptImage _tutorialui) "/Game/UI/ButtonPrompts/button_xbox_digital_y_8.button_xbox_digital_y_8" false)
  (Utilities|FlowControl|Delay 1.5)
  (CallFunction|DisplayNewInputs)
  (Variables|Default|SetSlamEventActive true))

(event Custom|SurgePrompt
  (bind _tutorialui (Variables|Default|GetTutorialUI))
  (bind _lightpromptimage_1 (Variables|/Game/UI/Tutorial/WB_Tutorial.WB_Tutorial_C|GetLightPromptImage_1 _tutorialui))
  ;[1 0.8804 0.3413] Set Up Surge Prompt
  (Widget|SetVisibility _lightpromptimage_1 "Visible")
  (Appearance|SetBrushfromTexture (Variables|/Game/UI/Tutorial/WB_Tutorial.WB_Tutorial_C|GetLightPromptImage _tutorialui) "/Game/UI/ButtonPrompts/button_xboxone_digital_analog_click_dark_4.button_xboxone_digital_analog_click_dark_4" false)
  (Appearance|SetBrushfromTexture _lightpromptimage_1 "/Game/UI/ButtonPrompts/button_xbox_digital_y_8.button_xbox_digital_y_8" false)
  (Utilities|FlowControl|Delay 1.5)
  (CallFunction|DisplayNewInputs)
  (Variables|Default|SetSurgeEventActive true))

(event EventBeginPlay
  (|CallParentFunction)
  ;[1 1 1] Create Tutorial UI
  (bind _returnvalue (UserInterface|CreateWidget "/Game/UI/Tutorial/WB_Tutorial.WB_Tutorial_C"))
  (bind _output_get (Variables|Default|SetTutorialUI _returnvalue))
  (UserInterface|Viewport|AddtoViewport _output_get 0)
  (CallFunction|Combo1Prompt)
  (Variables|Default|SetCurrentTextIndex 0))

(event Collision|EventActorBeginOverlap
  (params (OtherActor :type Actor%20Object%20Reference)))

(event EventTick
  (params (DeltaSeconds :type Float%20%28single-precision%29))
  (|CallParentFunction DeltaSeconds) ; This node is disabled and will not be called.\nDrag off pins to build functionality.
)

(event Game|Damage|EventAnyDamage
  (params (Damage :type Float%20%28single-precision%29) (DamageType :type Damage%20Type%20Object%20Reference) (InstigatedBy :type Controller%20Object%20Reference) (DamageCauser :type Actor%20Object%20Reference))
  (bind _tutorialui (Variables|Default|GetTutorialUI))
  (bind _tutorialui_2 (Variables|Default|GetTutorialUI))
  (bind _tutorialui_3 (Variables|Default|GetTutorialUI))
  (bind _tutorialui_4 (Variables|Default|GetTutorialUI))
  (bind _tutorialui_5 (Variables|Default|GetTutorialUI))
  (bind _tutorialui_6 (Variables|Default|GetTutorialUI))
  (bind _tutorialui_7 (Variables|Default|GetTutorialUI))
  (bind _tutorialui_8 (Variables|Default|GetTutorialUI))
  ;[0.2885 0.2885 0.2885] Check Through Events On Hit
  (if (Variables|Default|GetCanTakeDamage)
    (Variables|Default|SetCanTakeDamage false)
    (if (Variables|Default|GetCombo1EventActive)
      ;[0.04615 0.3466 1] Combo 1 Checks
      (bind _isplaying (CallFunction|CheckAnimInstance "/Game/ThirdPerson/Animations/NewCombo1/Combo1A_Montage.Combo1A_Montage"))
      (if _isplaying
        (UserInterface|Animation|PlayAnimation _tutorialui (Variables|/Game/UI/Tutorial/WB_Tutorial.WB_Tutorial_C|GetSuccessfullyPressed1 _tutorialui) 0.0 1 "Forward" 1.0 false)
        (Components|Animation|PlayAnimation (Variables|Character|GetMesh) "/Game/Art/Environment/TutorialArea/Animation/AS_TrainingDummyRight.AS_TrainingDummyRight" false)
        (Utilities|FlowControl|Delay 0.2)
        (Variables|Default|SetCanTakeDamage true)
        (else
          (bind _isplaying_2 (CallFunction|CheckAnimInstance "/Game/ThirdPerson/Animations/NewCombo1/Combo1B_Montage.Combo1B_Montage"))
          (if _isplaying_2
            (UserInterface|Animation|PlayAnimation _tutorialui_2 (Variables|/Game/UI/Tutorial/WB_Tutorial.WB_Tutorial_C|GetSuccessfullyPressed2 _tutorialui_2) 0.0 1 "Forward" 1.0 false)
            (Components|Animation|PlayAnimation (Variables|Character|GetMesh) "/Game/Art/Environment/TutorialArea/Animation/AS_TrainingDummyLeft.AS_TrainingDummyLeft" false)
            (Utilities|FlowControl|Delay 0.4)
            (Variables|Default|SetCanTakeDamage true)
            (else
              (bind _isplaying_3 (CallFunction|CheckAnimInstance "/Game/ThirdPerson/Animations/NewCombo1/Combo1C_Montage.Combo1C_Montage"))
              (if _isplaying_3
                (UserInterface|Animation|PlayAnimation _tutorialui_6 (Variables|/Game/UI/Tutorial/WB_Tutorial.WB_Tutorial_C|GetSuccessfullyPressed3 _tutorialui_6) 0.0 1 "Forward" 1.0 false)
                (Components|Animation|PlayAnimation (Variables|Character|GetMesh) "/Game/Art/Environment/TutorialArea/Animation/AS_TrainingDummyRight.AS_TrainingDummyRight" false)
                (UserInterface|Animation|PlayAnimation _tutorialui_6 (Variables|/Game/UI/Tutorial/WB_Tutorial.WB_Tutorial_C|GetInputDone _tutorialui_6) 0.0 1 "Forward" 1.0 false)
                (Utilities|FlowControl|Delay 0.4)
                (UserInterface|Animation|PlayAnimation _tutorialui_6 (Variables|/Game/UI/Tutorial/WB_Tutorial.WB_Tutorial_C|GetHideInputs _tutorialui_6) 0.0 1 "Forward" 1.0 false)
                (Variables|Default|SetCanTakeDamage true)
                (Variables|Default|SetCombo1EventActive false)
                (Utilities|FlowControl|Delay 0.4)
                (CallFunction|Combo2Prompt))))))
      (elif (Variables|Default|GetCombo2EventActive)
        ;[0.61 1 0.6367] Combo 2 Checks
        (bind _isplaying_4 (CallFunction|CheckAnimInstance "/Game/ThirdPerson/Animations/NewCombo1/Combo1A_Montage.Combo1A_Montage"))
        (if _isplaying_4
          (UserInterface|Animation|PlayAnimation _tutorialui_3 (Variables|/Game/UI/Tutorial/WB_Tutorial.WB_Tutorial_C|GetSuccessfullyPressed1 _tutorialui_3) 0.0 1 "Forward" 1.0 false)
          (Components|Animation|PlayAnimation (Variables|Character|GetMesh) "/Game/Art/Environment/TutorialArea/Animation/AS_TrainingDummyRight.AS_TrainingDummyRight" false)
          (Utilities|FlowControl|Delay 0.2)
          (Variables|Default|SetCanTakeDamage true)
          (else
            (bind _isplaying_5 (CallFunction|CheckAnimInstance "/Game/Art/Characters/Kaia/Animations/Combo2/Combo2B1_Montage.Combo2B1_Montage"))
            (if _isplaying_5
              (UserInterface|Animation|PlayAnimation _tutorialui_5 (Variables|/Game/UI/Tutorial/WB_Tutorial.WB_Tutorial_C|GetSuccessfullyPressed2 _tutorialui_5) 0.0 1 "Forward" 1.0 false)
              (UserInterface|Animation|PlayAnimation _tutorialui_5 (Variables|/Game/UI/Tutorial/WB_Tutorial.WB_Tutorial_C|GetSuccessfullyPressed3 _tutorialui_5) 0.0 1 "Forward" 1.0 false)
              (Components|Animation|PlayAnimation (Variables|Character|GetMesh) "/Game/Art/Environment/TutorialArea/Animation/AS_TrainingDummyBack.AS_TrainingDummyBack" false)
              (Utilities|FlowControl|Delay 0.4)
              (Variables|Default|SetCanTakeDamage true)
              (else
                (bind _isplaying_6 (CallFunction|CheckAnimInstance "/Game/Art/Characters/Kaia/Animations/Combo2/Combo2C1_Montage.Combo2C1_Montage"))
                (if _isplaying_6
                  (UserInterface|Animation|PlayAnimation _tutorialui_7 (Variables|/Game/UI/Tutorial/WB_Tutorial.WB_Tutorial_C|GetSuccessfullyPressed4 _tutorialui_7) 0.0 1 "Forward" 1.0 false)
                  (Components|Animation|PlayAnimation (Variables|Character|GetMesh) "/Game/Art/Environment/TutorialArea/Animation/AS_TrainingDummyBack.AS_TrainingDummyBack" false)
                  (UserInterface|Animation|PlayAnimation _tutorialui_7 (Variables|/Game/UI/Tutorial/WB_Tutorial.WB_Tutorial_C|GetInputDone _tutorialui_7) 0.0 1 "Forward" 1.0 false)
                  (Utilities|FlowControl|Delay 0.4)
                  (UserInterface|Animation|PlayAnimation _tutorialui_7 (Variables|/Game/UI/Tutorial/WB_Tutorial.WB_Tutorial_C|GetHideInputs _tutorialui_7) 0.0 1 "Forward" 1.0 false)
                  (Variables|Default|SetCanTakeDamage true)
                  (Variables|Default|SetCombo2EventActive false)
                  (Utilities|FlowControl|Delay 0.4)
                  (CallFunction|SlamPrompt))))))
        (elif (Variables|Default|GetSlamEventActive)
          ;[1 0.5505 0.9243] Slam Check
          (bind _isplaying_7 (CallFunction|CheckAnimInstance "/Game/Art/Characters/Kaia/Animations/Slam/Slam_3Attack_Montage.Slam_3Attack_Montage"))
          (if _isplaying_7
            (UserInterface|Animation|PlayAnimation _tutorialui_8 (Variables|/Game/UI/Tutorial/WB_Tutorial.WB_Tutorial_C|GetSuccessfullyPressed1 _tutorialui_8) 0.0 1 "Forward" 1.0 false)
            (Components|Animation|PlayAnimation (Variables|Character|GetMesh) "/Game/Art/Environment/TutorialArea/Animation/AS_TrainingDummyBack.AS_TrainingDummyBack" false)
            (UserInterface|Animation|PlayAnimation _tutorialui_8 (Variables|/Game/UI/Tutorial/WB_Tutorial.WB_Tutorial_C|GetInputDone _tutorialui_8) 0.0 1 "Forward" 1.0 false)
            (Utilities|FlowControl|Delay 0.4)
            (UserInterface|Animation|PlayAnimation _tutorialui_8 (Variables|/Game/UI/Tutorial/WB_Tutorial.WB_Tutorial_C|GetHideInputs _tutorialui_8) 0.0 1 "Forward" 1.0 false)
            (Variables|Default|SetCanTakeDamage true)
            (Variables|Default|SetSlamEventActive false)
            (Utilities|FlowControl|Delay 0.4)
            (CallFunction|SurgePrompt))
          (elif (Variables|Default|GetSurgeEventActive)
            ;[0.9872 1 0.4807] Surge Check
            (bind _isplaying_8 (CallFunction|CheckAnimInstance "/Game/Art/Characters/Kaia/Animations/Surge/Surge_2Hold_Montage.Surge_2Hold_Montage"))
            (if _isplaying_8
              (UserInterface|Animation|PlayAnimation _tutorialui_4 (Variables|/Game/UI/Tutorial/WB_Tutorial.WB_Tutorial_C|GetSuccessfullyPressed1 _tutorialui_4) 0.0 1 "Forward" 1.0 false)
              (UserInterface|Animation|PlayAnimation _tutorialui_4 (Variables|/Game/UI/Tutorial/WB_Tutorial.WB_Tutorial_C|GetSuccessfullyPressed2 _tutorialui_4) 0.0 1 "Forward" 1.0 false)
              (Components|Animation|PlayAnimation (Variables|Character|GetMesh) "/Game/Art/Environment/TutorialArea/Animation/AS_TrainingDummyBack.AS_TrainingDummyBack" false)
              (UserInterface|Animation|PlayAnimation _tutorialui_4 (Variables|/Game/UI/Tutorial/WB_Tutorial.WB_Tutorial_C|GetInputDone _tutorialui_4) 0.0 1 "Forward" 1.0 false)
              (Utilities|FlowControl|Delay 0.4)
              (UserInterface|Animation|PlayAnimation _tutorialui_4 (Variables|/Game/UI/Tutorial/WB_Tutorial.WB_Tutorial_C|GetHideInputs _tutorialui_4) 0.0 1 "Forward" 1.0 false)
              (Variables|Default|SetCanTakeDamage true)
              (Variables|Default|SetSurgeEventActive false)
              (Utilities|FlowControl|Delay 0.4)
              (CallFunction|FracturePrompt))
            (else
              (Utilities|FlowControl|Delay 0.2)
              (Variables|Default|SetCanTakeDamage true))))))
    (else
      (Variables|Default|SetCanTakeDamage true))))

(fn ConstructionScript
  (|CallParentFunction))

(fn CheckAnimInstance
  (params (Montage :type Anim%20Montage%20Object%20Reference))
  (bind _asbp_third_person_character (Utilities|Casting|CastToBP_ThirdPersonCharacter (Game|GetPlayerCharacter 0)))
  (return (Animation|Montage|MontageIsPlaying (Components|SkeletalMesh|GetAnimInstance (Variables|/Script/Engine.Character|GetMesh _asbp_third_person_character)) Montage)))

(fn DisplayNewInputs
  (bind _tutorialui (Variables|Default|GetTutorialUI))
  (Rendering|Components|TextRender|SetText (Variables|/Game/UI/Tutorial/WB_Tutorial.WB_Tutorial_C|GetAttackDescriptionText _tutorialui) (Utilities|Text|ToText(String) (Utilities|Array|Get(acopy) (Variables|Default|GetAttackDescText) (Variables|Default|GetCurrentTextIndex))))
  (Rendering|Components|TextRender|SetText (Variables|/Game/UI/Tutorial/WB_Tutorial.WB_Tutorial_C|GetAttackNameText _tutorialui) (Utilities|Text|ToText(String) (Utilities|Array|Get(acopy) (Variables|Default|GetAttackNameText) (Variables|Default|GetCurrentTextIndex))))
  (UserInterface|Animation|PlayAnimation _tutorialui (Variables|/Game/UI/Tutorial/WB_Tutorial.WB_Tutorial_C|GetDisplayInputs _tutorialui) 0.0 1 "Forward" 1.0 false)
  (Math|Integer|IncrementInt (Variables|Default|GetCurrentTextIndex)))