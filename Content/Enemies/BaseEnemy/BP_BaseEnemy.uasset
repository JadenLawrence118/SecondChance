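; Base enemy character with a camera-facing health bar, walk/sprint speeds, and interface functions for AI range and player targeting.
; Damage can stun it, pausing AI behind an indicator, and knocks it along the player's facing, harder for slams, with a brief hit cooldown.
; When BPCPlayerStats reports death, it heals the player, updates the enemy counter, returns attack tokens, then ragdolls away before being destroyed.
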(event Custom|Event%20Stun
  ;[1 1 1] Stuns the enemy by set a bool to true which stops the behaviour tree from reaching the controlling nodes. Also makes a blue box appear above the enemy's head to indicate that they are stunned
  (Rendering|SetVisibility (Variables|Default|GetStunIndicator) true false)
  (Variables|Default|SetAIActive false)
  (Utilities|FlowControl|Delay (Variables|Default|GetStunDuration))
  (Variables|Default|SetAIActive true)
  (Rendering|SetVisibility (Variables|Default|GetStunIndicator) false false))

(event Custom|SetWalking
  (params (Walking :type Boolean))
  ;[1 1 1] Toggles the enemy between walking and running. Movement speeds are variable and instance-editable
  (if Walking
    ;[1 1 1] Event AnyDamage - When the dummy is hit it checks if it can take damage. If true the dummy is knocked back and takes damage. If health<0 the dummy dies and gets detroyed
    (Variables|/Script/Engine.CharacterMovementComponent|SetMaxWalkSpeed (Variables|Character|GetCharacterMovement) (Variables|Default|GetWalkSpeed))
    (else
      (Variables|/Script/Engine.CharacterMovementComponent|SetMaxWalkSpeed (Variables|Character|GetCharacterMovement) (Variables|Default|GetSprintSpeed)))))

(event EventTick
  (params (DeltaSeconds :type Float%20%28single-precision%29))
  ;[1 1 1] Event Tick -  makes the enemy healthbar always look at the player
  (if (Variables|Default|GetAlive?)
    (Transformation|SetWorldRotation (Variables|Default|GetHealthBarWidget) (Math|Rotator|FindLookatRotation (Transformation|GetWorldLocation (Variables|Default|GetHealthBarWidget)) (Transformation|GetWorldLocation (Variables|/Script/Engine.PlayerCameraManager|GetTransformComponent (Game|GetPlayerCameraManager 0)))) false false)))

(event Game|Damage|EventAnyDamage
  (params (Damage :type Float%20%28single-precision%29) (DamageType :type Damage%20Type%20Object%20Reference) (InstigatedBy :type Controller%20Object%20Reference) (DamageCauser :type Actor%20Object%20Reference))
  (bind _playerbp (Variables|Default|GetPlayerBP))
  (bind _mesh (Variables|Character|GetMesh))
  (bind _mesh_2 (Variables|Character|GetMesh))
  (bind _returnvalue (Transformation|GetActorLocation _playerbp))
  (bind _returnvalue_2 (Transformation|GetWorldLocation _mesh))
  (bind _returnvalue_3 (Math|Rotator|FindLookatRotation _returnvalue_2 _returnvalue))
  (bind _returnvalue_4 (* _returnvalue_3 -1e+04))
  (bind (_x _y) (Math|Vector|BreakVector _returnvalue_4))
  ;[1 1 1] Event AnyDamage - When the dummy is hit it checks if it can take damage. If true the dummy is knocked back and takes damage. If health<0 the dummy dies and gets detroyed
  (if (Variables|Default|GetCanTakeDamage)
    (if (Variables|Default|GetUnstunnable)
      _
      (else
        (CallFunction|EventStun)))
    (if (Variables|Default|GetIsSlamAttack)
      (Variables|Default|SetCanTakeDamage false)
      (bind _asbp_third_person_character (Utilities|Casting|CastToBP_ThirdPersonCharacter (Game|GetPlayerCharacter 0)))
      (Character|LaunchCharacter (* (Math|Vector|GetForwardVector (Transformation|GetActorRotation _asbp_third_person_character)) 2e+03) false false)
      (bind _isplayerdead (Default|DecreaseHealth (Variables|Default|GetBPC_playerStats) Damage))
      (if _isplayerdead
        (Collision|SetCollisionObjectType (Variables|Character|GetMesh) "ECC_PhysicsBody" :!label _label)
        (Physics|SetSimulatePhysics (Variables|Character|GetMesh) true)
        (Default|IncreaseHealthonKill (Variables|Default|GetPlayerBP))
        (Default|CountEnemies (Variables|Default|GetEnemyCounter))
        (Rendering|SetVisibility (Variables|Default|GetStunIndicator) false false)
        (Variables|Default|SetAlive? false)
        (Class|BPITokenSystem|ReturnAttackToken(Message) (Game|Player|GetPlayerPawn 0) (Variables|Default|GetTokensHeld) (Variables|Default|GetAttackCooldown))
        ;[1 1 1] ragdoll
        (Components|DestroyComponent (Variables|Default|GetBPC_PlayerStats))
        (Components|DestroyComponent (Variables|Default|GetHealthBarWidget))
        (Class|BPIHitReaction|HasAttackHit(Message) (Variables|Default|GetPlayerBP) (Transformation|GetActorLocation))
        (Physics|SetSimulatePhysics _mesh_2 true)
        (Collision|SetCollisionEnabled _mesh_2 "QueryAndPhysics")
        (Physics|AddImpulse _mesh_2 (Math|Vector|MakeVector _x _y 2e+03) "None" true)
        (Class|Pawn|DetachfromControllerPendingDestroy)
        (Collision|SetActorEnableCollision false)
        (Utilities|FlowControl|Delay 5.0)
        (Actor|DestroyActor)
        (else
          (Utilities|FlowControl|Delay 0.2 :!label _label_2)
          (Variables|Default|SetCanTakeDamage true)))
      (else
        (Variables|Default|SetCanTakeDamage false)
        (bind _asbp_third_person_character_2 (Utilities|Casting|CastToBP_ThirdPersonCharacter (Game|GetPlayerCharacter 0)))
        (Character|LaunchCharacter (* (Math|Vector|GetForwardVector (Transformation|GetActorRotation _asbp_third_person_character_2)) 7.5e+02) false false)
        (bind _isplayerdead_2 (Default|DecreaseHealth (Variables|Default|GetBPC_playerStats) Damage))
        (if _isplayerdead_2
          (goto _label)
          (else
            (goto _label_2)))))))

(event EventBeginPlay
  ;[1 1 1] Begin Play - Gets the enemy's health widget
  (Variables|Default|SetAlive? true)
  (bind _aswb_dummy_health (Utilities|Casting|CastToWB_DummyHealth (UserInterface|GetWidget (Variables|Default|GetHealthBarWidget))))
  (Variables|Default|SetEnemyHealthWidget _aswb_dummy_health)
  (bind _asbp_third_person_character (Utilities|Casting|CastToBP_ThirdPersonCharacter (Game|GetPlayerCharacter 0)))
  (Variables|Default|SetPlayerBP _asbp_third_person_character)
  (bind _outactors (Actor|GetAllActorsOfClass "/Game/Enemies/Spawner/BP_EnemyCounter.BP_EnemyCounter_C"))
  (Variables|Default|SetEnemyCounter (Utilities|Array|Get(acopy) _outactors)))

(fn ConstructionScript)

(fn GetIdealRange
  (return 1.5e+02 3.5e+02))

(fn BICanbeTarget?
  (return true))

(fn BIMinDistance
  (return false 0.0))

(fn BIonSelectedTarget
  (return false))

(fn BISetCustomTarget
  (params (CustomTarget :type Actor%20Object%20Reference))
  (return false))