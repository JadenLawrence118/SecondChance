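; Charger enemy Blueprint whose attack is a straight-line charge along its LookDirection component.
; Attack ends the EnemyCounter timer, flags the enemy as attacking and uses AIMoveTo toward a point DistanceToCharge ahead, spawning a TestCube there, apparently as a debug marker.
; On success or failure alike, it signals attack end, returns its held attack tokens to the target with a cooldown delay and clears Unstunnable.
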(event Custom|Attack
  (params (AttackTarget :type Actor%20Object%20Reference))
  (bind _lookdirection (Variables|Default|GetLookDirection))
  (bind _distancetocharge (Variables|Default|GetDistanceToCharge))
  (bind _returnvalue (Transformation|GetWorldLocation _lookdirection))
  (bind _returnvalue_2 (Math|Vector|GetForwardVector _lookdirection))
  (bind _returnvalue_3 (* _returnvalue_2 _distancetocharge))
  (bind _returnvalue_4 (+ _returnvalue _returnvalue_3))
  (Default|EndTimer (Variables|Default|GetEnemyCounter))
  (Variables|Default|SetIsAttacking true)
  (AI|AIMoveTo self _returnvalue_4 0 5.0 false
    (:then
      (Game|SpawnActorfromClass "/Game/Enemies/TestCube.TestCube_C" (Math|Transform|MakeTransform _returnvalue_4 "0, 0, 0" "1.000000,1.000000,1.000000") "Undefined" "MultiplyWithRoot" 0 0))
    (:OnSuccess
      (Default|CallOnAttackEnd :!label _label)
      (Variables|Default|SetIsAttacking false)
      (Class|BPITokenSystem|ReturnAttackToken(Message) AttackTarget (Variables|Default|GetTokensHeld) (Variables|Default|GetAttackCooldown))
      (Variables|Default|SetTokensHeld 0)
      (Variables|Default|SetUnstunnable false))
    (:OnFail
      (goto _label))))

(event EventBeginPlay
  (|CallParentFunction) ; This node is disabled and will not be called.\nDrag off pins to build functionality.
)

(event Collision|EventActorBeginOverlap
  (params (OtherActor :type Actor%20Object%20Reference)))

(event EventTick
  (params (DeltaSeconds :type Float%20%28single-precision%29))
  (|CallParentFunction DeltaSeconds) ; This node is disabled and will not be called.\nDrag off pins to build functionality.
)

(fn ConstructionScript
  (|CallParentFunction))