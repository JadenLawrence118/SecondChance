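; Melee enemy character Blueprint that lunges forward with an attack montage to damage the player.
; Attack launches it along its facing and sets IsAttacking, so an overlap with the player deals damage only once per swing.
; When the montage completes or is interrupted, it clears attack state and returns held attack tokens to the target with a cooldown delay.
; On death, detected after parent damage handling, it hides and disables AttackBox.
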(event Custom|Attack
  (params (Attack%20Target :type Actor%20Object%20Reference))
  ;[1 1 1] Attack - Launches the enemy towards the player and plays the attack animation. Also sets IsAttacking to true at the start of the animation, and false at the end so that damage is only inflicted on the player during the animation. Also at the end returns the attack tokens it took after a short delay. Taking attack tokens is done in the behaviour tree
  (Variables|Default|SetIsAttacking true)
  (Character|LaunchCharacter (* (Math|Vector|GetForwardVector (Transformation|GetActorRotation)) (Variables|Default|GetLaunchDistance)) false false)
  (Animation|Montage|PlayMontage (Variables|Character|GetMesh) "/Game/Enemies/MeleeEnemy/Animations/AM_Attack.AM_Attack"
    (:OnCompleted
      _)
    (:OnInterrupted
      _))
  (Default|CallOnAttackEnd)
  (Variables|Default|SetIsAttacking false)
  (Class|BPITokenSystem|ReturnAttackToken(Message) Attack%20Target (Variables|Default|GetTokensHeld) (Variables|Default|GetAttackCooldown))
  (Variables|Default|SetTokensHeld 0)
  (Variables|Default|SetUnstunnable false))

(event Collision|EventActorBeginOverlap
  (params (OtherActor :type Actor%20Object%20Reference))
  (bind _returnvalue (Game|GetPlayerCharacter 0))
  ;[1 1 1] Collision - Checks if the enemy is doing its attack animation. If it is and is also colliding with the player, deals damage to the player. Otherwise does nothing
  (if (Variables|Default|GetIsAttacking)
    (if (== OtherActor _returnvalue)
      (Game|Damage|ApplyDamage _returnvalue (Variables|Default|GetBaseDamage) 0 0)
      (Variables|Default|SetIsAttacking false))))

(event Game|Damage|EventAnyDamage
  (params (Damage :type Float%20%28single-precision%29) (DamageType :type Damage%20Type%20Object%20Reference) (InstigatedBy :type Controller%20Object%20Reference) (DamageCauser :type Actor%20Object%20Reference))
  (bind _attackbox (Variables|Default|GetAttackBox))
  (|CallParentFunction Damage 0 0 0)
  (if (not (Variables|Default|GetAlive?))
    (Rendering|SetVisibility _attackbox false false)
    (Collision|SetCollisionEnabled _attackbox "NoCollision")))

(event EventTick
  (params (DeltaSeconds :type Float%20%28single-precision%29))
  (|CallParentFunction DeltaSeconds) ; This node is disabled and will not be called.\nDrag off pins to build functionality.
)

(event EventBeginPlay
  (|CallParentFunction) ; This node is disabled and will not be called.\nDrag off pins to build functionality.
)

(fn ConstructionScript
  (|CallParentFunction))

(fn NewFunction
  (return false))