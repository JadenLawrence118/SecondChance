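; Explosive enemy that turns into a visible bomb when damaged and blows up, hurting the player and other actors by separate amounts.
; Every hit stuns it unless unstunnable and launches it by a fixed knockback along the player's facing.
; Once hit, striking ExplodeOnHit actors or overlapping non-player actors detonates it, as does death.
; A timer-driven material flash countdown also ends in the sphere-trace explosion, and Tick returns held attack tokens.
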(event Custom|Explode
  (bind _returnvalue (Transformation|GetActorLocation))
  (Utilities|FlowControl|Sequence
    (:then_0
      (bind _outhits (Collision|MultiSphereTraceByChannel _returnvalue _returnvalue (Variables|Default|GetExplosionRadius) "TraceTypeQuery1" false 0 "ForDuration"))
      (for _array_element _outhits
        (if (Actor|ActorHasTag "damageable")
          (if (== (.HitActor (Collision|BreakHitResult _array_element)) (Game|GetPlayerCharacter 0))
            (Game|Damage|ApplyDamage (.HitActor (Collision|BreakHitResult _array_element)) (Variables|Default|GetDamageToPlayer) 0 0)
            (else
              (Game|Damage|ApplyDamage (.HitActor (Collision|BreakHitResult _array_element)) (Variables|Default|GetDamageToEnemies) 0 0))))))
    (:then_1
      (Actor|DestroyActor))))

(event Custom|StartExplosion
  (Utilities|Time|SetTimerbyEvent (delegate Custom|Flash) (Variables|Default|GetFlashSpeed)))

(event Custom|Flash
  (Utilities|FlowControl|Sequence
    (:then_0
      (if (Variables|Default|GetflashOn)
        (Rendering|Material|SetVectorParameterValue :self (Variables|Default|GetDynamicMaterial) :ParameterName "Colour" :!class /Script/Engine.MaterialInstanceDynamic)
        (Variables|Default|SetflashOn false)
        (else
          (Rendering|Material|SetVectorParameterValue (Variables|Default|GetDynamicMaterial) "Colour" (Variables|Default|GetFlashColour) :!class /Script/Engine.MaterialInstanceDynamic)
          (Variables|Default|SetflashOn true))))
    (:then_1
      (Math|Integer|IncrementInt (Variables|Default|GetflashCount)
        (:%20%20
          (if (< (Variables|Default|GetflashCount) (Variables|Default|GetNoToFlash))
            (CallFunction|StartExplosion)
            (else
              (CallFunction|Explode))))))))

(event EventBeginPlay
  (|CallParentFunction) ; This node is disabled and will not be called.\nDrag off pins to build functionality.
)

(event Collision|EventActorBeginOverlap
  (params (OtherActor :type Actor%20Object%20Reference))
  (if (!= OtherActor (Game|GetPlayerCharacter 0))
    (if (Variables|Default|GethasBeenHit)
      (CallFunction|Explode))))

(event Game|Damage|EventAnyDamage
  (params (Damage :type Float%20%28single-precision%29) (DamageType :type Damage%20Type%20Object%20Reference) (InstigatedBy :type Controller%20Object%20Reference) (DamageCauser :type Actor%20Object%20Reference))
  (bind _bpc_playerstats (Variables|Default|GetBPC_PlayerStats))
  ;[1 1 1] Damage script is the same as BaseEnemy but has removed the knockback changing based on the type of attack. Instead, all attacks knock this enemy back the same amount
  (if (Variables|Default|GetCanTakeDamage)
    (Variables|Default|SethasBeenHit true)
    (Rendering|SetVisibility (Variables|Character|GetMesh) false false)
    (Rendering|SetVisibility (Variables|Default|GetBomb) true false)
    (if (Variables|Default|GetUnstunnable)
      _
      (else
        (CallFunction|EventStun)))
    (Variables|Default|SetCanTakeDamage false)
    (bind _asbp_third_person_character (Utilities|Casting|CastToBP_ThirdPersonCharacter (Game|GetPlayerCharacter 0)))
    (Character|LaunchCharacter (* (Math|Vector|GetForwardVector (Transformation|GetActorRotation _asbp_third_person_character)) (Variables|Default|GetKnockback)) false false)
    (bind _isplayerdead (Default|DecreaseHealth (Variables|Default|GetBPC_playerStats) Damage))
    (if _isplayerdead
      (CallFunction|Death)
      (else
        (Progress|SetPercent (Variables|/Game/UI/Dummy/WB_DummyHealth.WB_DummyHealth_C|GetHealthBar (Variables|Default|GetEnemyHealthWidget)) (/ (Variables|/Game/ThirdPerson/Blueprints/BPC_PlayerStats.BPC_PlayerStats_C|GetCurrentHealth _bpc_playerstats) (Variables|/Game/ThirdPerson/Blueprints/BPC_PlayerStats.BPC_PlayerStats_C|GetMaxHealth _bpc_playerstats)))
        (Utilities|FlowControl|Delay 0.2)
        (Variables|Default|SetCanTakeDamage true)))))

(event EventDeath
  (Utilities|FlowControl|DelayUntilNextTick)
  (CallFunction|Explode))

(event EventTick
  (params (DeltaSeconds :type Float%20%28single-precision%29))
  (|CallParentFunction DeltaSeconds)
  (if (> (Variables|Default|GetTokensHeld) 0)
    (Class|BPITokenSystem|ReturnAttackToken(Message) (Game|Player|GetPlayerPawn 0) (Variables|Default|GetTokensHeld) 0.0)))

(event EventEventStun
  (Animation|PlayAnimMontage "/Game/Enemies/MeleeEnemy/Animations/AM_Stun.AM_Stun" 1.0 "None")
  (Variables|Default|SetAIActive false))

(event Collision|EventHit
  (params (MyComp :type Primitive%20Component%20Object%20Reference) (Other :type Actor%20Object%20Reference) (OtherComp :type Primitive%20Component%20Object%20Reference) (bSelfMoved :type Boolean) (HitLocation :type Vector :default "0, 0, 0") (HitNormal :type Vector :default "0, 0, 0") (NormalImpulse :type Vector :default "0, 0, 0") (Hit :type Hit%20Result%20Structure%20%28by%20ref%29))
  (if (Actor|ActorHasTag Other "ExplodeOnHit")
    (if (Variables|Default|GethasBeenHit)
      (CallFunction|Explode))))

(fn ConstructionScript
  (|CallParentFunction)
  (bind _returnvalue (Rendering|Material|CreateDynamicMaterialInstance (Variables|Character|GetMesh) 0 "/Game/Enemies/ExplosiveEnemy/Horde3Material.Horde3Material" "None" :!class /Script/Engine.PrimitiveComponent))
  (Variables|Default|SetDynamicMaterial _returnvalue))