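; Ranged enemy that attacks by playing an attack montage and firing a projectile from its ProjectileSpawner transform.
; The Attack event spawns the projectile as soon as the montage starts, rather than on a notify.
; Montage completion or interruption fires OnAttackEnd, clears the attacking and unstunnable flags, and returns held attack tokens to the target with a cooldown delay.
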(event Custom|Attack
  (params (AttackTarget :type Actor%20Object%20Reference))
  (Variables|Default|SetIsAttacking true)
  (Animation|Montage|PlayMontage (Variables|Character|GetMesh) "/Game/Enemies/MeleeEnemy/Animations/AM_Attack.AM_Attack"
    (:then
      (Game|SpawnActorfromClass "/Game/Enemies/RangedEnemy/BP_Projectile.BP_Projectile_C" (Transformation|GetWorldTransform (Variables|Default|GetProjectileSpawner)) "AlwaysSpawn" "MultiplyWithRoot" 0 0))
    (:OnCompleted
      (Default|CallOnAttackEnd :!label _label)
      (Variables|Default|SetIsAttacking false)
      (Class|BPITokenSystem|ReturnAttackToken(Message) AttackTarget (Variables|Default|GetTokensHeld) (Variables|Default|GetAttackCooldown))
      (Variables|Default|SetTokensHeld 0)
      (Variables|Default|SetUnstunnable false))
    (:OnInterrupted
      (goto _label))))

(event EventBeginPlay
  (|CallParentFunction) ; This node is disabled and will not be called.\nDrag off pins to build functionality.
)

(event Collision|EventActorBeginOverlap
  (params (OtherActor :type Actor%20Object%20Reference)))

(event EventTick
  (params (DeltaSeconds :type Float%20%28single-precision%29))
  (|CallParentFunction DeltaSeconds) ; This node is disabled and will not be called.\nDrag off pins to build functionality.
)

(fn ConstructionScript
  (|CallParentFunction))