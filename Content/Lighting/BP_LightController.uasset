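; Light controller that swaps a level's lighting between past and present time periods.
; BeginPlay caches both lights' intensities, then zeroes the inactive one according to StartPast, leaving post-process visibility untouched.
; SwitchLights flips InPast, restores the active light, zeroes the other and toggles both post-process objects' visibility.
; That visibility runs opposite to the names: PostProcessPresent shows in the past, PostProcessPast in the present.
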(event Custom|SwitchLights
  (bind _output_get (Variables|Default|SetInPast (not (Variables|Default|GetInPast))))
  (if _output_get
    (Rendering|Components|Light|SetIntensity (Variables|/Script/Engine.Light|GetLightComponent (Variables|Default|GetPastLight)) (Variables|Default|GetPastIntensity))
    (Rendering|Components|Light|SetIntensity (Variables|/Script/Engine.Light|GetLightComponent (Variables|Default|GetPresentLight)) 0.0)
    (Rendering|SetVisibility (Variables|Default|GetPostProcessPast) false false)
    (Rendering|SetVisibility (Variables|Default|GetPostProcessPresent) true false)
    (else
      (Rendering|Components|Light|SetIntensity (Variables|/Script/Engine.Light|GetLightComponent (Variables|Default|GetPresentLight)) (Variables|Default|GetPresentIntensity))
      (Rendering|Components|Light|SetIntensity (Variables|/Script/Engine.Light|GetLightComponent (Variables|Default|GetPastLight)) 0.0)
      (Rendering|SetVisibility (Variables|Default|GetPostProcessPast) true false)
      (Rendering|SetVisibility (Variables|Default|GetPostProcessPresent) false false))))

(event EventBeginPlay
  (Variables|Default|SetPastIntensity (Variables|/Script/Engine.LightComponentBase|GetIntensity (Variables|/Script/Engine.Light|GetLightComponent (Variables|Default|GetPastLight))))
  (Variables|Default|SetPresentIntensity (Variables|/Script/Engine.LightComponentBase|GetIntensity (Variables|/Script/Engine.Light|GetLightComponent (Variables|Default|GetPresentLight))))
  (if (Variables|Default|GetStartPast)
    (Rendering|Components|Light|SetIntensity (Variables|/Script/Engine.Light|GetLightComponent (Variables|Default|GetPastLight)) (Variables|Default|GetPastIntensity))
    (Rendering|Components|Light|SetIntensity (Variables|/Script/Engine.Light|GetLightComponent (Variables|Default|GetPresentLight)) 0.0)
    (Variables|Default|SetInPast true)
    (else
      (Rendering|Components|Light|SetIntensity (Variables|/Script/Engine.Light|GetLightComponent (Variables|Default|GetPresentLight)) (Variables|Default|GetPresentIntensity))
      (Rendering|Components|Light|SetIntensity (Variables|/Script/Engine.Light|GetLightComponent (Variables|Default|GetPastLight)) 0.0)
      (Variables|Default|SetInPast false))))

(fn ConstructionScript)